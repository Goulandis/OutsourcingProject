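; Config actor for a flight simulator that applies settings from Saved/Config/Config.ini to other game objects.
; OpenConfigFile builds the file path under the project directory for the config getters.
; Separate load functions push values into the character (camera, zoom thresholds), plane manager and WebSocket actor; the graph calls none itself.
; PlaneManager HeightOffset reads the PlaneScaleZ key, and the character loader's completion log is unconnected.
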(event EventBeginPlay)

(event Collision|EventActorBeginOverlap
  (params (OtherActor :type Actor%20Object%20Reference)))

(event EventTick
  (params (DeltaSeconds :type Float%20%28single-precision%29)))

(fn ConstructionScript)

(fn LoadCharacterConfig
  (bind _flightsimulatorcharacter (CallFunction|GetFlightSimulatorCharacter))
  (bind _filepath (Variables|Default|GetFilePath))
  (bind _section (LocalVariables|GetSection))
  (bind _value (Class|CommonFunLib|GetConfigBool _section "Autobiography" _filepath))
  (Variables|/Game/GamePlay/FlightSimulatorCharacter.FlightSimulatorCharacter_C|SetAutobiography _flightsimulatorcharacter _value)
  (bind _value_2 (Class|CommonFunLib|GetConfigFloat _section "RotateSpeed" _filepath))
  (Variables|/Game/GamePlay/FlightSimulatorCharacter.FlightSimulatorCharacter_C|SetRotateSpeed _flightsimulatorcharacter _value_2)
  (bind _value_3 (Class|CommonFunLib|GetConfigFloat _section "WheelSpeed" _filepath))
  (Variables|/Game/GamePlay/FlightSimulatorCharacter.FlightSimulatorCharacter_C|SetWheelSpeed _flightsimulatorcharacter _value_3)
  (bind _value_4 (Class|CommonFunLib|GetConfigFloat _section "MaxZoom" _filepath))
  (Variables|/Game/GamePlay/FlightSimulatorCharacter.FlightSimulatorCharacter_C|SetMaxZoom _flightsimulatorcharacter _value_4)
  (bind _value_5 (Class|CommonFunLib|GetConfigFloat _section "MinZoom" _filepath))
  (Variables|/Game/GamePlay/FlightSimulatorCharacter.FlightSimulatorCharacter_C|SetMinZoom _flightsimulatorcharacter _value_5)
  (bind _value_6 (Class|CommonFunLib|GetConfigFloat _section "CityLoadZoom" _filepath))
  (Variables|/Game/GamePlay/FlightSimulatorCharacter.FlightSimulatorCharacter_C|SetCityLoadZoom _flightsimulatorcharacter _value_6)
  (bind _value_7 (Class|CommonFunLib|GetConfigFloat _section "CapitalLoadZoom" _filepath))
  (Variables|/Game/GamePlay/FlightSimulatorCharacter.FlightSimulatorCharacter_C|SetCapitalLoadZoom _flightsimulatorcharacter _value_7)
  (bind _value_8 (Class|CommonFunLib|GetConfigFloat _section "CountryLoadZoom" _filepath))
  (Variables|/Game/GamePlay/FlightSimulatorCharacter.FlightSimulatorCharacter_C|SetCountryLoadZoom _flightsimulatorcharacter _value_8)
  (bind _value_9 (Class|CommonFunLib|GetConfigFloat _section "ContinentLoadZoom" _filepath))
  (Variables|/Game/GamePlay/FlightSimulatorCharacter.FlightSimulatorCharacter_C|SetContinentLoadZoom _flightsimulatorcharacter _value_9))

(fn LoadPlaneManagerConfig
  (bind _planemanger (CallFunction|GetPlaneManager))
  (bind _section (LocalVariables|GetSection))
  (bind _filepath (Variables|Default|GetFilePath))
  (bind _value (Class|CommonFunLib|GetConfigFloat _section "PlaneScaleX" _filepath))
  (bind _value_2 (Class|CommonFunLib|GetConfigFloat _section "PlaneScaleY" _filepath))
  (bind _value_3 (Class|CommonFunLib|GetConfigFloat _section "PlaneScaleZ" _filepath))
  (Variables|/Game/Blueprint/PlaneManager.PlaneManager_C|SetPlaneScale _planemanger (Math|Vector|MakeVector _value _value_2 _value_3))
  (bind _value_4 (Class|CommonFunLib|GetConfigFloat _section "PlaneScaleZ" _filepath))
  (Variables|/Game/Blueprint/PlaneManager.PlaneManager_C|SetHeightOffset _planemanger _value_4)
  (bind _value_5 (Class|CommonFunLib|GetConfigFloat _section "RecivedDataMaxTime" _filepath))
  (Variables|/Game/Blueprint/PlaneManager.PlaneManager_C|SetRecivedDataMaxTime _planemanger _value_5)
  (CallFunction|DebugLog "LoadPlaneManager" "PlaneManager config load compeled"))

(fn LoadWebSocketConfig
  (bind _websocketactor (CallFunction|GetWebSocketActor))
  (bind _section (LocalVariables|GetSection))
  (bind _filepath (Variables|Default|GetFilePath))
  (bind _value (Class|CommonFunLib|GetConfigString _section "ServerURL" _filepath))
  (Variables|/Script/FlightSimulator.FSWebSocket|SetServerURL _websocketactor _value)
  (bind _value_2 (Class|CommonFunLib|GetConfigString _section "ServerProtocol" _filepath))
  (Variables|/Script/FlightSimulator.FSWebSocket|SetServerProtocol _websocketactor _value_2)
  (bind _value_3 (Class|CommonFunLib|GetConfigFloat _section "ReceivedDataInterval" _filepath))
  (Variables|/Game/WebSocket/FSWebSocketBP.FSWebSocketBP_C|SetReceivedDataInterval _websocketactor _value_3)
  (CallFunction|DebugLog "LoadWebSocketConfig" "WebSocket config load compeled"))

(fn OpenConfigFile
  (bind _returnvalue (Class|KismetSystemLibrary|GetProjectDirectory))
  (bind _returnvalue_2 (Utilities|String|Append _returnvalue "Saved/Config/Config.ini"))
  (Variables|Default|SetFilePath _returnvalue_2)
  (CallFunction|DebugLog "ConfigActorConstruction" (Utilities|String|Append "Config file path " _returnvalue_2)))