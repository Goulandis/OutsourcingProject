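; Manager actor that spawns and moves planes on an Earth globe from route data and tracks the current plane.
; AddPlane spawns or updates planes by ID, merges in game-instance plane info, and places flight targets via WGS84-to-Cartesian conversion.
; Tick eases each plane toward its target with VInterpTo in Earth-relative space.
; A looping timer picks plane 1 as default; SwitchPlane cycles the current plane by ID.
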(event Custom|InitCurrentPlane
  (bind (_plane _found) (CallFunction|FindPlanebyId 1))
  (if _found
    (Variables|Default|SetCurrentPlane _plane)
    (Utilities|Time|ClearandInvalidateTimerbyHandle (stale EventBeginPlay _returnvalue))
    (Default|CallOnFindDefaultCurrentPlane (CallFunction|GetFSGameInstance))))

(event EventBeginPlay
  (bind _returnvalue (Utilities|Time|SetTimerbyEvent (delegate Custom|InitCurrentPlane) 1.0 true)))

(event EventTick
  (params (DeltaSeconds :type Float%20%28single-precision%29))
  (CallFunction|PlanesFlytoTarget DeltaSeconds))

(fn ConstructionScript)

(fn AddPlane
  (params (RouteData :type Route%20Data%20Structure))
  (bind _fullroutedata (CallFunction|MakeFullRouteData RouteData))
  (bind (_plane _found) (CallFunction|FindPlanebyId (.pnaleid RouteData)))
  (LocalVariables|SetPlane _plane)
  (if _found
    (Default|AddRouteDatas (LocalVariables|GetPlane) _fullroutedata)
    (else
      (bind _returnvalue (Game|SpawnActorfromClass "/Game/GamePlay/Plane.Plane_C" (Math|Transform|MakeTransform "0, 0, 0" (Variables|Default|GetPlaneRotation) (Variables|Default|GetPlaneScale)) "Undefined" 0 (.pnaleid RouteData) 0))
      (CallFunction|DebugLog "AddPlane" (Utilities|String|Append "Createed a plane with id " (Utilities|String|ToString(Integer) (.pnaleid RouteData))))
      (Variables|/Game/GamePlay/Plane.Plane_C|SetId _returnvalue (.pnaleid RouteData))
      (Transformation|AttachComponentToComponent _returnvalue (Variables|/Game/EarthSimulator/Blueprints/MainBP/MasterOrb.MasterOrb_C|GetScale%20/%20Rotation (CallFunction|GetEarth)) "None" "KeepRelative" "KeepRelative" "KeepRelative" true)
      (bind _returnvalue_2 (Class|CommonFunLib|WGS84toCartesian (.longitude RouteData) (.latitude RouteData) (+ (Variables|Default|GetHeightOffset) (.height RouteData))))
      (Transformation|SetActorLocation _returnvalue _returnvalue_2 false false)
      (Utilities|Array|Add (Variables|Default|GetPlanes) _returnvalue)
      (Default|AddRouteDatas _returnvalue _fullroutedata)))
  (CallFunction|UpdateTargetPosition _fullroutedata))

(fn FindPlanebyId
  (params (PlaneId :type Integer))
  (bind _planes (Variables|Default|GetPlanes))
  (if (> (Utilities|Array|Length (Variables|Default|GetPlanes)) 0)
    (LocalVariables|SetIsExist false)
    (bind (_array_element _array_index) (Utilities|Array|ForEachLoopwithBreak _planes :!label _label)
      (:LoopBody
        (if (== (Variables|/Game/GamePlay/Plane.Plane_C|GetId _array_element) PlaneId)
          (LocalVariables|SetIndex _array_index)
          (LocalVariables|SetIsExist true)
          (goto _label Break)))
      (:Completed
        (return (Utilities|Array|Get(acopy) _planes (LocalVariables|GetIndex)) (LocalVariables|GetIsExist))))))

(fn PlanesFlytoTarget
  (params (DeltaSeconds :type Float%20%28single-precision%29))
  (for _array_element (Variables|Default|GetPlanes)
    (Utilities|IsValid _array_element
      (:Is%20Valid
        (Utilities|IsValid (Variables|/Game/GamePlay/Plane.Plane_C|GetFlightTarget _array_element)
          (:Is%20Valid
            (Transformation|SetRelativeLocation (Variables|/Script/Engine.Actor|GetRootComponent _array_element) (Math|Interpolation|VInterpTo (Variables|/Script/Engine.SceneComponent|GetRelativeLocation (Variables|/Script/Engine.Actor|GetRootComponent _array_element)) (Variables|/Script/Engine.SceneComponent|GetRelativeLocation (Variables|/Script/Engine.Actor|GetRootComponent (Variables|/Game/GamePlay/Plane.Plane_C|GetFlightTarget _array_element))) DeltaSeconds (Variables|/Game/GamePlay/Plane.Plane_C|GetFlySpeed _array_element)) false false)))))))

(fn UpdateTargetPosition
  (params (Target :type Route%20Data%20Structure))
  (bind _heightoffset (Variables|Default|GetHeightOffset))
  (bind _returnvalue (+ (.height Target) _heightoffset))
  (bind (_plane _found) (CallFunction|FindPlanebyId (.pnaleid Target)))
  (LocalVariables|SetPlane _plane)
  (if _found
    (Utilities|IsValid (Variables|/Game/GamePlay/Plane.Plane_C|GetFlightTarget (LocalVariables|GetPlane))
      (:Is%20Valid
        (bind _returnvalue_2 (Class|CommonFunLib|WGS84toCartesian (.longitude Target) (.latitude Target) _returnvalue))
        (Transformation|SetActorLocation (Variables|/Game/GamePlay/Plane.Plane_C|GetFlightTarget (LocalVariables|GetPlane)) _returnvalue_2 false false))
      (:Is%20Not%20Valid
        (bind _returnvalue_3 (Game|SpawnActorfromClass "/Game/Blueprint/FlightTarget.FlightTarget_C" (Math|Transform|MakeTransform "0, 0, 0" "0, 0, 0" "1,1,1") "Undefined" 0 (.pnaleid Target) 0))
        (Transformation|AttachComponentToComponent _returnvalue_3 (Variables|/Game/EarthSimulator/Blueprints/MainBP/MasterOrb.MasterOrb_C|GetScale%20/%20Rotation (CallFunction|GetEarth)) "None" "KeepRelative" "KeepRelative" "KeepRelative" true)
        (bind _returnvalue_4 (Class|CommonFunLib|WGS84toCartesian (.longitude Target) (.latitude Target) _returnvalue))
        (Transformation|SetActorLocation _returnvalue_3 _returnvalue_4 false false)
        (Variables|/Game/GamePlay/Plane.Plane_C|SetFlightTarget (LocalVariables|GetPlane) _returnvalue_3)))
    (else
      (CallFunction|DebugLog "UpdateTargetPosition" (Utilities|String|Append "Plane is not exist that id is " (Utilities|String|ToString(Integer) (.pnaleid Target)))))))

(fn MakeFullRouteData
  (params (RouteData :type Route%20Data%20Structure))
  (for _array_element (Variables|/Game/GamePlay/FSGameInstance.FSGameInstance_C|GetPlaneInfos (CallFunction|GetFSGameInstance))
    (if (== (.pnaleid RouteData) (.PnaleId (Utilities|Struct|BreakRouteData _array_element)))
      (return (Utilities|Struct|MakeRouteData (.longitude RouteData) (.latitude RouteData) (.height RouteData) (.pnaleid RouteData) (.directionangle RouteData) (.pitchangle RouteData) (.PlaneType (Utilities|Struct|BreakRouteData _array_element)) (.PlaneLength (Utilities|Struct|BreakRouteData _array_element)) (.PlaneHeight (Utilities|Struct|BreakRouteData _array_element)) (.WingSpan (Utilities|Struct|BreakRouteData _array_element)) (.EmptyWeight (Utilities|Struct|BreakRouteData _array_element))))))
  (CallFunction|DebugLog "MakeFullRouteData" (Utilities|String|Append "There is no plane with id equal to  " (Utilities|String|ToString(Integer) (.pnaleid RouteData)) " in PlaneInfo")))

(fn GetCurrentPlane
  (bind _currentplane (Variables|Default|GetCurrentPlane))
  (Utilities|IsValid _currentplane
    (:Is%20Valid
      (return _currentplane))
    (:Is%20Not%20Valid
      (CallFunction|DebugLog "GetCurrentPlane" "CurrentPlane is not valid"))))

(fn SwitchPlane
  (params (SwitchPlameType :type SwitchPlaneType%20Enum :default "NewEnumerator0"))
  (bind _currentplane (CallFunction|GetCurrentPlane))
  (bind _planes (Variables|Default|GetPlanes))
  (bind _returnvalue (Utilities|Array|Length _planes))
  (bind _id (Variables|/Game/GamePlay/Plane.Plane_C|GetId _currentplane))
  (bind _returnvalue_2 (- _id 1))
  (bind _returnvalue_3 (+ _id 1))
  (Utilities|IsValid _currentplane
    (:Is%20Valid
      (switch Utilities|FlowControl|Switch|SwitchonSwitchPlaneType SwitchPlameType
        (:NewEnumerator0
          (if (> _returnvalue _returnvalue_3)
            (bind (_plane _found) (CallFunction|FindPlanebyId _returnvalue_3))
            (if _found
              (Variables|Default|SetCurrentPlane _plane))
            (else
              (bind (_plane_2 _found_2) (CallFunction|FindPlanebyId))
              (if _found_2
                (Variables|Default|SetCurrentPlane _plane_2)))))
        (:NewEnumerator1
          (if (> _returnvalue_2 0)
            (bind (_plane_3 _found_3) (CallFunction|FindPlanebyId _returnvalue_2))
            (if _found_3
              (Variables|Default|SetCurrentPlane _plane_3))
            (else
              (bind (_plane_4 _found_4) (CallFunction|FindPlanebyId (- _returnvalue 1)))
              (if _found_4
                (Variables|Default|SetCurrentPlane _plane_4)))))))))