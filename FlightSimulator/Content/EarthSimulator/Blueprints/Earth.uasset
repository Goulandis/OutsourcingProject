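; Interactive Earth actor for the simulator, which the player spins by mouse drag and zooms with the wheel.
; While the left button is held, Tick adds speed-scaled, inverted axis input to the Parent component's pitch and yaw.
; Wheel input moves the player pawn along world X, only within that pawn's distance limits.
; The Autobiography flag gates the parent class Tick, and the stored initial rotation is unused here.
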(event EventBeginPlay
  (Input|EnableInput self (Game|GetPlayerController 0))
  (Variables|Default|SetInitRotation (Variables|/Script/Engine.SceneComponent|GetRelativeRotation (Variables|Default|GetParent))))

(event Collision|EventActorBeginOverlap
  (params (OtherActor :type Actor%20Object%20Reference)))

(event EventTick
  (params (DeltaSeconds :type Float%20%28single-precision%29))
  (bind _dragspeed (Variables|Default|GetDragSpeed))
  (bind _parent (Variables|Default|GetParent))
  (if (Variables|Default|GetAutobiography)
    (|CallParentFunction DeltaSeconds))
  (Utilities|FlowControl|Sequence
    (:then_0
      (if (Variables|Default|GetStartRotate)
        (Transformation|SetRelativeRotation _parent (Math|Rotator|CombineRotators (Variables|/Script/Engine.SceneComponent|GetRelativeRotation _parent) (Math|Rotator|MakeRotator 0.0 (* _dragspeed (* (Class|Actor|GetInputAxisKeyValue) -1.0)) (* (* (Class|Actor|GetInputAxisKeyValue) -1.0) _dragspeed))) false false)))))

(event Input|MouseEvents|MouseWheelAxis
  (params (AxisValue :type Float%20%28single-precision%29))
  (bind _playerpawn (Variables|Default|GetPlayerPawn))
  (bind _playerpawn_2 (Variables|Default|GetPlayerPawn))
  (bind _wheelspeed (Variables|Default|GetWheelSpeed))
  (bind _returnvalue (Transformation|GetActorLocation _playerpawn_2))
  (bind _returnvalue_2 (* AxisValue _wheelspeed))
  (bind _returnvalue_3 (+ _returnvalue_2 (.x _returnvalue)))
  (if (and (<= _returnvalue_3 (Variables|/Game/GamePlay/FlightSimulatorPawn.FlightSimulatorPawn_C|GetMinDistance _playerpawn)) (>= _returnvalue_3 (Variables|/Game/GamePlay/FlightSimulatorPawn.FlightSimulatorPawn_C|GetMaxDistance _playerpawn)))
    (Transformation|SetActorLocation (Variables|Default|GetPlayerPawn) (Math|Vector|MakeVector _returnvalue_3 (.y _returnvalue) (.z _returnvalue)) false false)))

(event Input|MouseEvents|LeftMouseButton
  (params (Key :type Key%20Structure :default "None"))
  (:Pressed
    (Variables|Default|SetStartRotate true))
  (:Released
    (Variables|Default|SetStartRotate false)))

(fn ConstructionScript
  (|CallParentFunction))