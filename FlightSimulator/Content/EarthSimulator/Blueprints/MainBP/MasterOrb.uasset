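; Master orb actor that simulates a planet's axial spin, clouds and orbit around an optional parent orb.
; Tick accumulates time into yaw rotations scaled by day and year length, follows the parent's location and can preserve world tilt.
; Helper graphs unpack settings structs, apply transforms and visibility, and build dynamic materials for surface, clouds and atmosphere.
; The construction script calls only the orb material setup; the other setup calls are disconnected.
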(event EventTick
  (params (DeltaSeconds :type Float%20%28single-precision%29))
  (bind _parentorb (Variables|SimulationSettings|GetParentOrb))
  ;[1 1 1] Global Time Setup
  (Variables|SimulationSettings|SetGlobalSpeedUpdate (+ (* DeltaSeconds -3.6e+02) (Variables|SimulationSettings|GetGlobalSpeedUpdate)))
  ;[1 1 1] Axial Rotation
  (Transformation|SetRelativeRotation (Variables|Default|GetScale%20/%20Rotation) (Math|Rotator|MakeRotator 0.0 0.0 (select (Variables|SimulationSettings|GetReversedAxialRotation) (* (/ (Variables|SimulationSettings|GetGlobalSpeedUpdate) (Variables|SimulationSettings|GetDayLength)) -1.0) (/ (Variables|SimulationSettings|GetGlobalSpeedUpdate) (Variables|SimulationSettings|GetDayLength)))) false false)
  ;[1 1 1] Clouds Simulation
  (if (Variables|CloudsMaterialSettings|GetDisableClouds)
    _
    (else
      (Transformation|SetRelativeRotation (Variables|Default|GetCloudsSimulation) (* (Variables|SimulationSettings|GetCloudsSpeed) (/ (Variables|SimulationSettings|GetGlobalSpeedUpdate) (select (Variables|SimulationSettings|GetReversedAxialRotation) -3.6e+02 3.6e+02))) false false)))
  ;[1 1 1] Orbital Direction
  (if (Utilities|IsValid _parentorb)
    (Transformation|SetWorldLocation (Variables|Default|GetParent) (Transformation|GetWorldLocation (Variables|MasterOrb_C|GetAxial%20Tilt _parentorb)) false false))
  (Variables|SimulationSettings|SetWorldRotation (Transformation|GetWorldRotation (Variables|Default|GetAxial%20Tilt)))
  (Transformation|SetRelativeRotation (Variables|Default|GetOrbitDirection) (Math|Rotator|MakeRotator 0.0 0.0 (select (Variables|SimulationSettings|GetReversedOrbitalDirection) (* (/ (/ (Variables|SimulationSettings|GetGlobalSpeedUpdate) (Variables|SimulationSettings|GetDayLength)) (Variables|SimulationSettings|GetYearLenght)) -1.0) (/ (/ (Variables|SimulationSettings|GetGlobalSpeedUpdate) (Variables|SimulationSettings|GetDayLength)) (Variables|SimulationSettings|GetYearLenght)))) false false)
  (if (Variables|SimulationSettings|GetKeepWorldRotation)
    (Transformation|SetWorldRotation (Variables|Default|GetAxial%20Tilt) (Variables|SimulationSettings|GetWorldRotation) false false)))

(fn ConstructionScript
  (Utilities|OrbMaterialSettings))

(fn OrbMaterialSetting
  (params (MaterialInterface :type Material%20Interface%20Object%20Reference))
  (bind _returnvalue (Rendering|Material|CreateDynamicMaterialInstance (Variables|Default|GetOrb) 0 MaterialInterface "None" :!class /Script/Engine.PrimitiveComponent))
  (Rendering|Material|SetTextureParameterValue _returnvalue "BaseColor" (Variables|OrbMaterialSettings|GetOrbDiffuse))
  (Rendering|Material|SetTextureParameterValue _returnvalue "Specular" (Variables|OrbMaterialSettings|GetOrbSpecular))
  (Rendering|Material|SetTextureParameterValue _returnvalue "Emissive" (Variables|OrbMaterialSettings|GetOrbEmissive))
  (Rendering|Material|SetTextureParameterValue _returnvalue "Normal" (Variables|OrbMaterialSettings|GetOrbNormal))
  (Rendering|Material|SetVectorParameterValue _returnvalue "EmissiveColor" (Variables|OrbMaterialSettings|GetOrbEmissiveColor) :!class /Script/Engine.MaterialInstanceDynamic)
  (Rendering|Material|SetScalarParameterValue _returnvalue "Contrast" (Variables|OrbMaterialSettings|GetOrbContrast) :!class /Script/Engine.MaterialInstanceDynamic)
  (Rendering|Material|SetScalarParameterValue _returnvalue "SpecularIntensity" (Variables|OrbMaterialSettings|GetOrbSpecularIntensity) :!class /Script/Engine.MaterialInstanceDynamic)
  (Rendering|Material|SetScalarParameterValue _returnvalue "RoughnessIntensity" (Variables|OrbMaterialSettings|GetOrbRoughnessIntensity) :!class /Script/Engine.MaterialInstanceDynamic)
  (Rendering|Material|SetScalarParameterValue _returnvalue "EmissiveIntensity" (Variables|OrbMaterialSettings|GetOrbEmissiveIntensity) :!class /Script/Engine.MaterialInstanceDynamic)
  (Rendering|Material|SetScalarParameterValue _returnvalue "NormalIntensity" (Variables|OrbMaterialSettings|GetOrbNormalIntensity) :!class /Script/Engine.MaterialInstanceDynamic))