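; WebSocket client actor that streams live plane route data into the game's plane manager.
; On BeginPlay a looping timer retries the server connection until connected, and the connect event notifies the game instance.
; Each incoming JSON message is decoded with VaRest into route data (position, altitude, plane ID, heading, pitch) and passed to AddPlane.
; A delayed AddPlane branch is left unwired and never runs.
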(event Custom|ConnectServer
  (if (Variables|Default|GetIsConnected)
    (Utilities|Time|ClearandInvalidateTimerbyHandle (Variables|Default|GetConnectServerTimerHandle))
    (else
      (Class|FSWebSocket|Connect)
      (CallFunction|DebugLog "ConnectServer" (Utilities|String|Append "URL:" (Variables|Default|GetServerURL))))))

(event EventBeginPlay
  (bind _returnvalue (Utilities|Time|SetTimerbyEvent (delegate Custom|ConnectServer) (Variables|Default|GetConnectInterval) true))
  (Variables|Default|SetConnectServerTimerHandle _returnvalue))

(event EventOnConnected
  (Default|CallOnWebSocketConnected (CallFunction|GetFSGameInstance))
  (Variables|Default|SetIsConnected true))

(event EventOnMessage
  (params (Message :type String))
  (CallFunction|DebugLog "OnMessage" Message)
  (bind _returnvalue (Class|VaRestSubsystem|DecodeJsonObject (|VaRestSubsystem) Message))
  (Default|AddPlane (CallFunction|GetPlaneManager) (Utilities|Struct|MakeRouteData (Class|VaRestJsonObject|GetNumberField _returnvalue "Longitude") (Class|VaRestJsonObject|GetNumberField _returnvalue "Latitude") (Class|VaRestJsonObject|GetNumberField _returnvalue "geoAltitude") (Class|VaRestJsonObject|GetIntegerField _returnvalue "planeID") (Class|VaRestJsonObject|GetNumberField _returnvalue "DirectionAngle") (Class|VaRestJsonObject|GetNumberField _returnvalue "PitchAngle"))))

(fn ConstructionScript)