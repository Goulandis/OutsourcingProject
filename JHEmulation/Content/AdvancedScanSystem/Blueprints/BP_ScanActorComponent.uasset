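; Actor component that triggers the scan effect of the Advanced Scan System, by Z key or StartScan event.
; BeginPlay loads ScanSettings from the DT_AdvancedScanSystem row at RowIndex; L and K step the index without reloading settings.
; A scan spawns BP_ScanActor at the first actor tagged with the ScanOrigin setting, passing settings and origin.
; It spawns only while no previous scan actor is valid.
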(event Custom|StartScan
  ;[0.125 0.125 0.125] Spawn Scan Actor
  (Utilities|IsValid (stale _returnvalue)
    (:Is%20Not%20Valid
      (bind _outactors (Actor|GetAllActorsOfClasswithTag "/Script/Engine.Actor" (.ScanOrigin (Utilities|Struct|BreakF_ScanStructure (Variables|Default|GetScanSettings)))))
      (Utilities|IsValid (Utilities|Array|Get(acopy) _outactors)
        (:Is%20Valid
          (bind _returnvalue (Game|SpawnActorfromClass "/Game/AdvancedScanSystem/Blueprints/BP_ScanActor.BP_ScanActor_C" (Math|Transform|MakeTransform (Transformation|GetActorLocation (Utilities|Array|Get(acopy) _outactors)) "0, 0, 0" "1.000000,1.000000,1.000000") "Undefined" 0 (Variables|Default|GetScanSettings) (Utilities|Array|Get(acopy) _outactors) 0))
          (Variables|Default|SetBPScanActor _returnvalue))))))

(event EventBeginPlay
  ;[0.125 0.125 0.125] Import Info from data table
  (bind _outrownames (DataTable|GetDataTableRowNames "/Game/AdvancedScanSystem/Blueprints/DT_AdvancedScanSystem.DT_AdvancedScanSystem"))
  (bind _returnvalue (Utilities|GetDataTableRow "/Game/AdvancedScanSystem/Blueprints/DT_AdvancedScanSystem.DT_AdvancedScanSystem" (Utilities|Array|Get(acopy) _outrownames (Variables|Default|GetRowIndex)))
    (:then
      (Variables|Default|SetScanSettings _returnvalue))))

(event Input|KeyboardEvents|Z
  (params (Key :type Key%20Structure :default "None"))
  ;[0.125 0.125 0.125] Spawn Scan Actor
  ;;[1 0.2454 0] Input Action
  (:Pressed
    (Utilities|IsValid (stale _returnvalue)
      (:Is%20Not%20Valid
        (bind _outactors (Actor|GetAllActorsOfClasswithTag "/Script/Engine.Actor" (.ScanOrigin (Utilities|Struct|BreakF_ScanStructure (Variables|Default|GetScanSettings)))))
        (Utilities|IsValid (Utilities|Array|Get(acopy) _outactors)
          (:Is%20Valid
            (bind _returnvalue (Game|SpawnActorfromClass "/Game/AdvancedScanSystem/Blueprints/BP_ScanActor.BP_ScanActor_C" (Math|Transform|MakeTransform (Transformation|GetActorLocation (Utilities|Array|Get(acopy) _outactors)) "0, 0, 0" "1.000000,1.000000,1.000000") "Undefined" 0 (Variables|Default|GetScanSettings) (Utilities|Array|Get(acopy) _outactors) 0))
            (Variables|Default|SetBPScanActor _returnvalue)))))))

(event Input|KeyboardEvents|Z
  (params (Key :type Key%20Structure :default "None")))

(event Input|KeyboardEvents|C
  (params (Key :type Key%20Structure :default "None")))

(event Input|KeyboardEvents|K
  (params (Key :type Key%20Structure :default "None"))
  (:Pressed
    (Math|Integer|DecrementInt (Variables|Default|GetRowIndex))))

(event Input|KeyboardEvents|L
  (params (Key :type Key%20Structure :default "None"))
  (:Pressed
    (Math|Integer|IncrementInt (Variables|Default|GetRowIndex))))