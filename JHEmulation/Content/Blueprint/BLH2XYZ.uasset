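; Actor Blueprint that places itself in the world from B, L, H coordinates, apparently geodetic latitude, longitude and height.
; The BLH2XYZ function converts them to XYZ, applies a Trans call with a hard-coded angle, then sets the actor location, optionally subtracting an Offset.
; Helper functions compute that Offset as S minus T, print a vector distance and test-print a rotation.
; The event graph and construction script are empty.
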(event EventBeginPlay)

(event Collision|EventActorBeginOverlap
  (params (OtherActor :type Actor%20Object%20Reference)))

(event EventTick
  (params (DeltaSeconds :type Float%20%28single-precision%29)))

(fn ConstructionScript)

(fn BLH2XYZ
  (bind _returnvalue (Class|BLFunLib|BLH2XYZ (Variables|Default|GetB) (Variables|Default|GetL) (Variables|Default|GetH)))
  (bind _returnvalue_2 (Class|BLFunLib|Trans _returnvalue "-157.500000,-18.000000,55.700000"))
  (if (Variables|Default|GetIsOffset)
    (Transformation|SetActorLocation (- _returnvalue_2 (Variables|Default|GetOffset)) false false)
    (else
      (bind _output_get (Variables|Default|SetS _returnvalue_2))
      (Transformation|SetActorLocation _output_get false false))))

(fn CalculateOffset
  (bind _output_get (Variables|Default|SetOffset (- (Variables|Default|GetS) (Variables|Default|GetT))))
  (return _output_get))

(fn Len
  (Development|PrintString (Utilities|String|ToString(Float) (Math|Vector|VectorLength (- (Variables|Default|GetLS) (Variables|Default|GetLT))))))

(fn Rotate
  (bind _returnvalue (Class|BLFunLib|Trans "10.000000,0.000000,5.000000" "0.000000,0.000000,30.000000"))
  (Development|PrintString (Utilities|String|ToString(Vector) _returnvalue)))

(fn Test)