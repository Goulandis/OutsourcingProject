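; BLHOpe is an operator Blueprint that converts a set of BLH2XYZ objects, apparently geodetic coordinates to XYZ, around a shared offset.
; Its Ope function first runs BLH2XYZ on every entry without offset, taking the offset calculated by the entry flagged IsMain.
; A second pass then enables offsetting, assigns that shared Offset to every entry and converts again.
; The event graph and construction script are empty.
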(event EventBeginPlay)

(event Collision|EventActorBeginOverlap
  (params (OtherActor :type Actor%20Object%20Reference)))

(event EventTick
  (params (DeltaSeconds :type Float%20%28single-precision%29)))

(fn ConstructionScript)

(fn Ope
  (bind _blh2xyzs (Variables|Default|GetBLH2XYZS))
  (Utilities|FlowControl|Sequence
    (:then_0
      (for _array_element _blh2xyzs
        (Variables|/Game/Blueprint/BLH2XYZ.BLH2XYZ_C|SetIsOffset _array_element false)
        (Default|BLH2XYZ _array_element)
        (if (Variables|/Game/Blueprint/BLH2XYZ.BLH2XYZ_C|GetIsMain _array_element)
          (bind _offset (Default|CalculateOffset _array_element))
          (Variables|Default|SetOffset _offset))))
    (:then_1
      (for _array_element_2 _blh2xyzs
        (Variables|/Game/Blueprint/BLH2XYZ.BLH2XYZ_C|SetIsOffset _array_element_2 true)
        (Variables|/Game/Blueprint/BLH2XYZ.BLH2XYZ_C|SetOffset _array_element_2 (Variables|Default|GetOffset))
        (Default|BLH2XYZ _array_element_2)))))