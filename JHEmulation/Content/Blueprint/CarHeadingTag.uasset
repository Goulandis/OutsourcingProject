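; CarHeadingTag is an actor that follows the runtime car pawn at a fixed drop below it, showing heading with a plane that can be toggled.
; Construction stores the starting yaw and registers the actor on the pawn.
; BeginPlay binds to the player controller's speed and heading updates; UpdateData takes only the heading.
; Tick eases yaw toward heading plus starting yaw with a fixed-alpha Lerp.
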(event EventBeginPlay
  (EventDispatchers|BindEventtoOnUpdateSpeedandHeadingAngle (CallFunction|GetJHPlayerController) (EventDispatchers|CreateEvent :!event UpdateData)))

(event EventTick
  (params (DeltaSeconds :type Float%20%28single-precision%29))
  (bind _returnvalue (Transformation|GetActorRotation))
  (bind _carpawnruntime (Variables|Default|GetCarPawnRuntime))
  (bind _returnvalue_2 (Transformation|GetActorLocation _carpawnruntime))
  (Transformation|SetActorLocation (Math|Vector|MakeVector (.x _returnvalue_2) (.y _returnvalue_2) (- (.z _returnvalue_2) 4e+01)) false false)
  (Transformation|SetActorRotation (Math|Rotator|MakeRotator (.roll _returnvalue) (.pitch _returnvalue) (Math|Float|Lerp (.yaw _returnvalue) (+ (Variables|Default|GetHeadingAngle) (Variables|Default|GetOriginAngle)) 0.1))))

(fn ConstructionScript
  (bind _carpawnruntime (Variables|Default|GetCarPawnRuntime))
  (bind _returnvalue (Transformation|GetActorLocation _carpawnruntime))
  (Transformation|SetActorLocation (Math|Vector|MakeVector (.x _returnvalue) (.y _returnvalue) (- (.z _returnvalue) 4e+01)) false false)
  (Variables|Default|SetOriginAngle (.yaw (Transformation|GetActorRotation)))
  (Variables|/Game/GamePlay/CarPawnRuntime.CarPawnRuntime_C|SetCarHeadingTag (Variables|Default|GetCarPawnRuntime) self))

(fn UpdateData
  (params (Speed :type Float%20%28double-precision%29) (HeadingAngle :type Float%20%28double-precision%29))
  (Variables|Default|SetHeadingAngle HeadingAngle))

(fn ShowTag
  (params (Show :type Boolean))
  (Development|SetHiddeninGame (Variables|Default|GetPlane) (not Show) false))

(fn LoadConfig)

(fn Init
  (Transformation|SetRelativeLocation (Variables|Default|GetPlane) (Math|Vector|MakeVector 0.0 (* 0.0 -1.0) 0.0) false false))