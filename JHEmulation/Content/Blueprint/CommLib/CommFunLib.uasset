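; Blueprint function library of shared helpers for the JH game framework, covering object access, mouse picking, parsing and coordinate conversion.
; Typed getters return the JH game instance, controller, HUD, game mode, spectator pawn and config, mostly logging failures through DLog.
; GetMousePos line-traces under the cursor, and StringToLinearColor parses comma-separated RGBA via StringToArray.
; BLHToXYZ converts geodetic coordinates to XYZ, then applies a fixed-angle transform and offset.
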(fn GetJHGameInstance
  (bind ___worldcontext (LocalVariables|Get__WorldContext))
  (bind _asjhgame_instance (Utilities|Casting|CastToJHGameInstance (Game|GetGameInstance ___worldcontext))
    (:then
      _)
    (:CastFailed
      (CallFunction|DLog "Error:GetJHGameInstance" "Failed to cast GameInstance to JHGameInstance" ___worldcontext)))
  (return _asjhgame_instance))

(fn GetJHPlayerController
  (bind ___worldcontext (LocalVariables|Get__WorldContext))
  (bind _asjhplayer_controller (Utilities|Casting|CastToJHPlayerController (Game|GetPlayerController ___worldcontext))
    (:then
      _)
    (:CastFailed
      (CallFunction|DLog "Error:GetJHPlayerController" "Failed to cast PlayerController to JHPlayerController" ___worldcontext)))
  (return _asjhplayer_controller))

(fn GetJHHUD
  (bind ___worldcontext (LocalVariables|Get__WorldContext))
  (bind _jhplayercontroller (CallFunction|GetJHPlayerController ___worldcontext))
  (Utilities|IsValid _jhplayercontroller
    (:Is%20Valid
      (bind _asjhhud (Utilities|Casting|CastToJHHUD (HUD|GetHUD _jhplayercontroller))
        (:then
          _)
        (:CastFailed
          (CallFunction|DLog "Error:GetJHHUD" "Failed to cast HUD to JHHUD" ___worldcontext)))
      (return _asjhhud))))

(fn GetJHGameMode
  (bind ___worldcontext (LocalVariables|Get__WorldContext))
  (bind _asjhgame_mode (Utilities|Casting|CastToJHGameMode (Game|GetGameMode ___worldcontext))
    (:then
      _)
    (:CastFailed
      (CallFunction|DLog "Error:GetJHGameMode" "Failed to cast GameMode to JHGameMode" ___worldcontext)))
  (return _asjhgame_mode))

(fn GetConfig
  (bind ___worldcontext (LocalVariables|Get__WorldContext))
  (bind _jhgameinstance (CallFunction|GetJHGameInstance ___worldcontext))
  (bind _config (Variables|/Game/GamePlay/JHGameInstance.JHGameInstance_C|GetConfig _jhgameinstance))
  (Utilities|IsValid _config
    (:Is%20Valid
      (return _config))
    (:Is%20Not%20Valid
      (CallFunction|DLog "[Error:GetConfig]" "Config is not valid" ___worldcontext))))

(fn GetMousePos
  (params (Multi :type Float%20%28double-precision%29))
  (bind ___worldcontext (LocalVariables|Get__WorldContext))
  (bind _returnvalue (Game|GetPlayerController ___worldcontext))
  (bind (_worldlocation _worlddirection) (Game|Player|ConvertMouseLocationToWorldSpace _returnvalue))
  (bind _outhit (Collision|LineTraceByChannel ___worldcontext _worldlocation (+ _worldlocation (* _worlddirection Multi)) "TraceTypeQuery1" false 0 "None"))
  (return (.Location (Collision|BreakHitResult _outhit)) (.HitActor (Collision|BreakHitResult _outhit))))

(fn StringtoLinearColor
  (params (ColorStr :type String))
  (bind _outarray (CallFunction|StringtoArray ColorStr "," (LocalVariables|Get__WorldContext)))
  (if (== (Utilities|Array|Length _outarray) 4)
    (return (Utilities|Struct|MakeLinearColor (Math|Conversions|ToFloat(Integer) (Utilities|Array|Get(acopy) _outarray)) (Math|Conversions|ToFloat(Integer) (Utilities|Array|Get(acopy) _outarray 1)) (Math|Conversions|ToFloat(Integer) (Utilities|Array|Get(acopy) _outarray 2)) (Math|Conversions|ToFloat(Integer) (Utilities|Array|Get(acopy) _outarray 3))))
    (else
      (CallFunction|DLog "[Error:StringToLinearColor]" (Utilities|String|Append "The string \"" ColorStr "\" is malformed, the correct format should be \"x,x,x,x\"") (LocalVariables|Get__WorldContext)))))

(fn StringtoArray
  (params (SourceStr :type String) (SplitStr :type String))
  (bind _array (LocalVariables|GetArray))
  (bind _output_get (LocalVariables|SetRightStr SourceStr))
  (while (.ReturnValue (Utilities|String|Split _output_get SplitStr))
    (Utilities|Array|Add _array (.LeftS (Utilities|String|Split _output_get SplitStr)))
    (LocalVariables|SetRightStr (.RightS (Utilities|String|Split _output_get SplitStr))))
  (if (Utilities|Enum|NotEqual(Enum) (LocalVariables|GetRightStr) "")
    (Utilities|Array|Add _array (LocalVariables|GetRightStr)))
  (return _array))

(fn GetJHSpectatorPawn
  (bind ___worldcontext (LocalVariables|Get__WorldContext))
  (bind _asjhspectator_pawn (Utilities|Casting|CastToJHSpectatorPawn (Game|Player|GetPlayerPawn ___worldcontext))
    (:then
      (return _asjhspectator_pawn))
    (:CastFailed
      (CallFunction|DLog "Error:GetJHSpectatorPawn" "Failed to cast PlayerPawn to JHSpectatoPawn" ___worldcontext))))

(fn BLHtoXYZ
  (params (B :type Float%20%28double-precision%29) (L :type Float%20%28double-precision%29) (H :type Float%20%28double-precision%29))
  (bind _returnvalue (Class|BLFunLib|BLH2XYZ B L H))
  (bind _returnvalue_2 (Class|BLFunLib|Trans _returnvalue "-157.500000,-18.000000,55.700000"))
  (return (- _returnvalue_2 (LocalVariables|GetOffset))))