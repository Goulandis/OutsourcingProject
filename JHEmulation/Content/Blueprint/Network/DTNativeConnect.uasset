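; Network Blueprint that links the game to a DTNative websocket server using URL, credentials and event name read from config.
; After a one-second delay it connects if the HUD allows, relaying connection status through GameInstance events that trigger local authentication, then event listening.
; Incoming messages are decoded with VaRest and routed by name: Weather to the HUD weather widget, Vehicle to the player controller's car pawn update.
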(event EventBeginPlay
  (bind _jhgameinstance (CallFunction|GetJHGameInstance))
  (bind _jhhud (CallFunction|GetJHHUD))
  (Utilities|FlowControl|Sequence
    (:then_0
      (CallFunction|LoadConfig)
      (EventDispatchers|BindEventtoOnServerConnented _jhgameinstance (EventDispatchers|CreateEvent :!event OnServerConnected))
      (EventDispatchers|BindEventtoOnServerVerificationSuccessful _jhgameinstance (EventDispatchers|CreateEvent :!event OnServerVerificationSuccessful)))
    (:then_1
      (Utilities|FlowControl|Delay 1.0)
      (Utilities|IsValid _jhhud
        (:Is%20Valid
          (if (Variables|/Game/GamePlay/JHHUD.JHHUD_C|GetAllowConnectServer _jhhud)
            (Class|DTNativeClientCoreSession|WebsocketConnect (Variables|Default|GetDTNativeClientCoreSession) (Variables|Default|GetServerURL) (EventDispatchers|CreateEvent :!event ConnectServer))))))))

(fn ConstructionScript)

(fn ConnectServer
  (params (Status :type EDTNativeClientCoreConnectionStatus%20Enum :default "__ZERO"))
  (bind _jhgameinstance (CallFunction|GetJHGameInstance))
  (switch Utilities|FlowControl|Switch|SwitchonEDTNativeClientCoreConnectionStatus Status
    (:DISCONNECTED
      (Default|CallOnServerDisconnenct _jhgameinstance)
      (CallFunction|DLog "Log:ServerConnect" "Server disconnected"))
    (:CONNECTED
      (Default|CallOnServerConnented _jhgameinstance)
      (CallFunction|DLog "Log:ServerConnect" "Server connected"))
    (:FAILED
      (Default|CallOnServerConnectFailly _jhgameinstance)
      (CallFunction|DLog "Error:ServerConnect" "Server connect failly"))))

(fn OnServerConnected
  (Class|DTNativeClientCoreSession|WebsocketAuthenticateLocal (Variables|Default|GetDTNativeClientCoreSession) (Variables|Default|GetUser) (Variables|Default|GetPassword) (Variables|Default|GetClientEngine) (Variables|Default|GetClientOS) (EventDispatchers|CreateEvent :!event OnAuthenticate))
  (CallFunction|DLog "Log:OnServerConnected" "Websocket start to authenticate"))

(fn OnAuthenticate
  (params (Data :type Array%20of%20DT%20Native%20Client%20Core%20Transport%20Data%20Object%20References) (Status :type Integer))
  (if (== Status 200)
    (CallFunction|DLog "Log:OnAuthenticate" "Verification successful")
    (Default|CallOnServerVerificationSuccessful (CallFunction|GetJHGameInstance))
    (else
      (CallFunction|DLog "Error:OnAuthenticate" "Validation failed"))))

(fn OnServerVerificationSuccessful
  (Class|DTNativeClientCoreSession|WebsocketAddEventListener (Variables|Default|GetDTNativeClientCoreSession) (Variables|Default|GetEventName) (EventDispatchers|CreateEvent :!event Listener))
  (CallFunction|DLog "Log:OnServerVerificationSuccessful" (Utilities|String|Append "Start listening to the server : " (Variables|Default|GetServerURL))))

(fn Listener
  (params (Data :type Array%20of%20DT%20Native%20Client%20Core%20Transport%20Data%20Object%20References) (EventName :type String))
  (CallFunction|DLog "Log:Listner" EventName)
  (if (> (Utilities|Array|Length Data) 0)
    (bind _returnvalue (Class|VaRestSubsystem|DecodeJsonObject (|VaRestSubsystem) (Class|DTNativeClientCoreTransportData|MakeJSONString (Utilities|Array|Get(acopy) Data) 0)))
    (switch string (Class|VaRestJsonObject|GetStringField (Class|VaRestJsonObject|GetObjectField _returnvalue "data") "name")
      (:weather
        (CallFunction|DatatoUWWeather (Class|VaRestJsonObject|GetObjectField (Class|VaRestJsonObject|GetObjectField _returnvalue "data") "data")))
      (:vehicle
        (CallFunction|DatatoCarPawnRuntime (Class|VaRestJsonObject|GetObjectField (Class|VaRestJsonObject|GetObjectField _returnvalue "data") "data"))))))

(fn LoadConfig
  (bind _config (CallFunction|GetConfig))
  (bind _returnvalue (Class|VaRestJsonObject|GetObjectField _config "Server"))
  (Variables|Default|SetServerURL (Class|VaRestJsonObject|GetStringField _returnvalue "ServerURL"))
  (Variables|Default|SetUser (Class|VaRestJsonObject|GetStringField _returnvalue "User"))
  (Variables|Default|SetPassword (Class|VaRestJsonObject|GetStringField _returnvalue "Password"))
  (Variables|Default|SetClientEngine (Class|VaRestJsonObject|GetStringField _returnvalue "ClientEngine"))
  (Variables|Default|SetClientOS (Class|VaRestJsonObject|GetStringField _returnvalue "ClientOS"))
  (Variables|Default|SetEventName (Class|VaRestJsonObject|GetStringField _returnvalue "EventName")))

(fn DatatoUWWeather
  (params (JsonObj :type Va%20Rest%20Json%20Object%20Object%20Reference))
  (bind _jhhud (CallFunction|GetJHHUD))
  (bind _uw_title (Variables|/Game/GamePlay/JHHUD.JHHUD_C|GetUW_Title _jhhud))
  (bind _uw_weahter (Variables|/Game/UI/UW_Title.UW_Title_C|GetUW_Weahter _uw_title))
  (Utilities|IsValid _jhhud
    (:Is%20Valid
      (Utilities|IsValid _uw_title
        (:Is%20Valid
          (Utilities|IsValid _uw_weahter
            (:Is%20Valid
              (Default|UpdateWeather _uw_weahter JsonObj))))))))

(fn DatatoCarPawnRuntime
  (params (JsonObj :type Va%20Rest%20Json%20Object%20Object%20Reference))
  (bind _jhplayercontroller (CallFunction|GetJHPlayerController))
  (Utilities|IsValid _jhplayercontroller
    (:Is%20Valid
      (Default|UpdateCarPawnRuntime _jhplayercontroller JsonObj))))