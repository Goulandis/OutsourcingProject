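; Spline actor that draws the car's trajectory as spline meshes, with color and glow loaded from config into a material parameter collection.
; AddPointEvent appends a point at the CarPawn's location, spawning a SplinePoint actor and a new mesh segment.
; Each Tick, once three or more points exist, the last point is re-added at the newest SplinePoint actor's location and the latest segment is refitted.
; The construction script meshes any pre-placed points.
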(event Custom|SpawnSpline
  (params (Target :type Vector))
  (bind _spline (Variables|Default|GetSpline))
  (bind _spline_2 (Variables|Default|GetSpline))
  (bind _returnvalue (Spline|GetNumberOfSplinePoints _spline_2))
  (bind (_location _tangent) (Spline|GetLocationandTangentatSplinePoint _spline 0 "Local"))
  (bind _returnvalue_2 (- _returnvalue 2))
  (bind _returnvalue_3 (+ _returnvalue_2 1))
  (bind (_location_2 _tangent_2) (Spline|GetLocationandTangentatSplinePoint _spline _returnvalue_3 "Local"))
  (Spline|AddSplinePoint (Variables|Default|GetSpline) Target "World" true)
  (bind _returnvalue_4 (AddComponent|AddSplineMeshComponent true))
  (Transformation|AttachComponentToComponent _returnvalue_4 0 "None" "KeepRelative" "KeepRelative" "KeepRelative" true)
  (for _index (range 0 _returnvalue_2)
    (SplineMesh|SetStartandEnd _returnvalue_4 _location _tangent _location_2 _tangent_2 true :!class /Script/Engine.SplineMeshComponent)
    (Development|PrintString (Utilities|String|Append "Start:" (Utilities|String|ToString(Vector) _location) ",End:" (Utilities|String|ToString(Vector) _location_2)))))

(event Custom|AddPointEvent
  (CallFunction|AddPoint (Transformation|GetActorLocation (Variables|Default|GetCarPawn))))

(event EventBeginPlay
  (CallFunction|ConfigLoad))

(event EventTick
  (params (DeltaSeconds :type Float%20%28single-precision%29))
  (CallFunction|UpdateCurrentSplinePoint))

(fn ConstructionScript
  (bind _spline (Variables|Default|GetSpline))
  (for _index (range 0 (- (Spline|GetNumberOfSplinePoints (Variables|Default|GetSpline)) 2))
    (bind _splinemeshcomp (CallFunction|AddSplineMeshComponent))
    (bind _output_get (Variables|Default|SetSplineMesh _splinemeshcomp))
    (Transformation|AttachComponentToComponent _output_get (Variables|Default|GetStaticMesh) "None" "KeepRelative" "KeepRelative" "KeepRelative" true)
    (SplineMesh|SetStartandEnd (Variables|Default|GetSplineMesh) (.Location (Spline|GetLocationandTangentatSplinePoint _spline _index "Local")) (.Tangent (Spline|GetLocationandTangentatSplinePoint _spline _index "Local")) (.Location (Spline|GetLocationandTangentatSplinePoint _spline (+ _index 1) "Local")) (.Tangent (Spline|GetLocationandTangentatSplinePoint _spline (+ _index 1) "Local")) true :!class /Script/Engine.SplineMeshComponent)))

(fn AddPoint
  (params (Pos :type Vector))
  (bind _spline (Variables|Default|GetSpline))
  (bind _splinepointarr (Variables|Default|GetSplinePointArr))
  (bind _returnvalue (Utilities|Array|LastIndex _splinepointarr))
  (bind _output (Utilities|Array|Get(acopy) _splinepointarr _returnvalue))
  (Utilities|FlowControl|Sequence
    (:then_0
      (Utilities|IsValid _output
        (:Is%20Valid
          (Variables|/Game/Blueprint/Spline/SplinePoint.SplinePoint_C|SetSureLocation _output false))))
    (:then_1
      (Spline|AddSplinePoint (Variables|Default|GetSpline) Pos "World" true)
      (bind _returnvalue_2 (Game|SpawnActorfromClass "/Game/Blueprint/Spline/SplinePoint.SplinePoint_C" (Math|Transform|MakeTransform Pos "0, 0, 0" "1.000000,1.000000,1.000000") "Undefined" 0 0))
      (Utilities|Array|Add (Variables|Default|GetSplinePointArr) _returnvalue_2)
      (Variables|/Game/Blueprint/Spline/SplinePoint.SplinePoint_C|SetCarPawn _returnvalue_2 (Variables|Default|GetCarPawn))
      (Default|Show _returnvalue_2 (Variables|/Game/GamePlay/CarPawn.CarPawn_C|GetShowPoint (Variables|Default|GetCarPawn)))
      (Utilities|Array|Add (Variables|Default|GetSplinePointPosArr) Pos)
      (bind _splinemeshcomp (CallFunction|AddSplineMeshComponent))
      (Utilities|Array|Add (Variables|Default|GetSplineMeshCompArr) _splinemeshcomp)
      (bind _output_get (Variables|Default|SetSplineMesh _splinemeshcomp))
      (Transformation|AttachComponentToComponent _output_get (Variables|Default|GetStaticMesh) "None" "KeepRelative" "KeepRelative" "KeepRelative" true)
      (for _index (range 0 (- (Spline|GetNumberOfSplinePoints _spline) 2))
        (SplineMesh|SetStartandEnd (Variables|Default|GetSplineMesh) (.Location (Spline|GetLocationandTangentatSplinePoint _spline _index "Local")) (.Tangent (Spline|GetLocationandTangentatSplinePoint _spline _index "Local")) (.Location (Spline|GetLocationandTangentatSplinePoint _spline (+ _index 1) "Local")) (.Tangent (Spline|GetLocationandTangentatSplinePoint _spline (+ _index 1) "Local")) true :!class /Script/Engine.SplineMeshComponent)))))

(fn UpdateCurrentSplinePoint
  (bind _spline (Variables|Default|GetSpline))
  (bind _spline_2 (Variables|Default|GetSpline))
  (bind _splinepointarr (Variables|Default|GetSplinePointArr))
  (bind _returnvalue (Spline|GetNumberOfSplinePoints _spline))
  (bind _returnvalue_2 (- _returnvalue 1))
  (if (>= _returnvalue_2 2)
    (Spline|RemoveSplinePoint _spline _returnvalue_2 true)
    (Spline|AddSplinePoint _spline_2 (Transformation|GetActorLocation (Utilities|Array|Get(acopy) _splinepointarr (Utilities|Array|LastIndex _splinepointarr))) "World" true)
    (for _index (range 0 (- (Spline|GetNumberOfSplinePoints _spline_2) 2))
      (SplineMesh|SetStartandEnd (Variables|Default|GetSplineMesh) (.Location (Spline|GetLocationandTangentatSplinePoint _spline_2 _index "Local")) (.Tangent (Spline|GetLocationandTangentatSplinePoint _spline_2 _index "Local")) (.Location (Spline|GetLocationandTangentatSplinePoint _spline_2 (+ _index 1) "Local")) (.Tangent (Spline|GetLocationandTangentatSplinePoint _spline_2 (+ _index 1) "Local")) true :!class /Script/Engine.SplineMeshComponent))))

(fn AddSplineMeshComponent
  (bind _returnvalue (AddComponent|AddSplineMeshComponent true))
  (return _returnvalue))

(fn ConfigLoad
  (bind _config (CallFunction|GetConfig))
  (bind _returnvalue (Class|VaRestJsonObject|GetObjectField _config "Car"))
  (bind _returnvalue_2 (Class|VaRestJsonObject|GetStringField _returnvalue "LocusColor"))
  (bind _linearcolor (CallFunction|StringtoLinearColor _returnvalue_2))
  (Rendering|Material|SetVectorParameterValue "/Game/Blueprint/Spline/MPC_Spline.MPC_Spline" "BaseColor" _linearcolor :!class /Script/Engine.KismetMaterialLibrary)
  (Rendering|Material|SetScalarParameterValue "/Game/Blueprint/Spline/MPC_Spline.MPC_Spline" "EmissiveStrength" (Class|VaRestJsonObject|GetNumberField _returnvalue "LocusEmissiveStrngth") :!class /Script/Engine.KismetMaterialLibrary)
  (Development|PrintString (Utilities|String|ToString(Integer) _linearcolor)))