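; SplineLocus manages a car's trajectory trail, drawn by a spawned SplineActor linked to the CarPawn.
; On BeginPlay it reads visibility, color and glow settings from a config object and pushes color and emissive strength into the MPC_Spline material parameter collection.
; SetupLocus spawns the spline at the car, AddPoint extends it, ShowLocus toggles mesh and points within config limits, and CleanLocus or destruction removes it.
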(event EventBeginPlay
  (CallFunction|LoadConfig)
  (CallFunction|Init))

(event Collision|EventActorBeginOverlap
  (params (OtherActor :type Actor%20Object%20Reference)))

(event EventTick
  (params (DeltaSeconds :type Float%20%28single-precision%29)))

(event EventDestroyed
  (bind _splineactor (Variables|Default|GetSplineActor))
  (Utilities|IsValid _splineactor
    (:Is%20Valid
      (Actor|DestroyActor _splineactor))))

(fn ConstructionScript)

(fn SetupLocus
  (params (Setup :type Boolean))
  (Utilities|IsValid (Variables|Default|GetSplineActor)
    (:Is%20Not%20Valid
      (bind _returnvalue (Game|SpawnActorfromClass "/Game/Blueprint/Spline/SplineActor.SplineActor_C" (Math|Transform|MakeTransform (.location (Transformation|GetActorTransform (Variables|Default|GetCarPawn))) (.rotation (Transformation|GetActorTransform (Variables|Default|GetCarPawn))) "1.000000,1.000000,1.000000") "Undefined" 0 0))
      (bind _output_get (Variables|Default|SetSplineActor _returnvalue))
      (Variables|/Game/Blueprint/Spline/SplineActor.SplineActor_C|SetCarPawn _output_get (Variables|Default|GetCarPawn))
      (Variables|Default|SetSetup Setup)
      (CallFunction|AddPoint))))

(fn AddPoint
  (bind _splineactor (Variables|Default|GetSplineActor))
  (Utilities|IsValid _splineactor
    (:Is%20Valid
      (Default|AddPointEvent _splineactor))))

(fn ShowLocus
  (params (Show :type Boolean))
  (bind _splineactor (Variables|Default|GetSplineActor))
  (Variables|Default|SetIsShowLocus Show)
  (Utilities|IsValid _splineactor
    (:Is%20Valid
      (if (Variables|Default|GetAllowShowLocus)
        (Default|ShowSplineMesh _splineactor (Variables|Default|GetIsShowLocus)))
      (Default|ShowPoint _splineactor (Variables|Default|GetAllowShowPoint)))))

(fn LoadConfig
  (bind _config (CallFunction|GetConfig))
  (bind _returnvalue (Class|VaRestJsonObject|GetObjectField _config "Car"))
  (bind _returnvalue_2 (Class|VaRestJsonObject|GetObjectField _returnvalue "Spline"))
  (Variables|Default|SetAllowShowLocus (Class|VaRestJsonObject|GetBoolField _returnvalue_2 "AllowShowLocus"))
  (Variables|Default|SetAllowShowPoint (Class|VaRestJsonObject|GetBoolField _returnvalue_2 "AllowShowPoint"))
  (Variables|Default|SetLocusEmissiveStrength (Class|VaRestJsonObject|GetNumberField _returnvalue_2 "LocusEmissiveStrength"))
  (Variables|Default|SetLocusColor (.OutConvertedColor (Math|Conversions|ToColor(LinearColor) (Class|VaRestJsonObject|GetStringField _returnvalue_2 "LocusColor")))))

(fn Init
  (Rendering|Material|SetVectorParameterValue "/Game/Blueprint/Spline/MPC_Spline.MPC_Spline" "BaseColor" (Variables|Default|GetLocusColor) :!class /Script/Engine.KismetMaterialLibrary)
  (Rendering|Material|SetScalarParameterValue "/Game/Blueprint/Spline/MPC_Spline.MPC_Spline" "EmissiveStrength" (Variables|Default|GetLocusEmissiveStrength) :!class /Script/Engine.KismetMaterialLibrary))

(fn CleanLocus
  (bind _splineactor (Variables|Default|GetSplineActor))
  (Utilities|IsValid _splineactor
    (:Is%20Valid
      (Actor|DestroyActor _splineactor))))