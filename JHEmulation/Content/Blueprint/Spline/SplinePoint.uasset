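; SplinePoint is a marker actor with a sphere that can track a point on a car pawn.
; Each tick, while SureLocation is set and CarPawn is valid, it moves itself to the world location of that pawn's ChildActor component.
; The Show function toggles whether the sphere is hidden in game.
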(event EventBeginPlay)

(event Collision|EventActorBeginOverlap
  (params (OtherActor :type Actor%20Object%20Reference)))

(event EventTick
  (params (DeltaSeconds :type Float%20%28single-precision%29))
  (bind _carpawn (Variables|Default|GetCarPawn))
  (if (Variables|Default|GetSureLocation)
    (Utilities|IsValid _carpawn
      (:Is%20Valid
        (Transformation|SetActorLocation (Transformation|GetWorldLocation (Variables|/Game/GamePlay/CarPawnDemo.CarPawnDemo_C|GetChildActor _carpawn)) false false)))))

(fn ConstructionScript)

(fn Show
  (params (Show :type Boolean))
  (bind _sphere (Variables|Default|GetSphere))
  (if Show
    (Development|SetHiddeninGame _sphere false false)
    (else
      (Development|SetHiddeninGame _sphere true false))))