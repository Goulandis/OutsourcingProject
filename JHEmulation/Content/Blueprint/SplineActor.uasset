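; Spline actor that renders a path with spline mesh components, built in the editor or extended at runtime.
; The construction script creates one mesh per spline segment.
; SpawnSpline appends a world-space point and adds one mesh stretched from first to last point, printing both ends; Test calls it for each Taget entry.
; Helpers trace under the mouse cursor and remove the last point; AddPoint is an empty stub.
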(event Custom|SpawnSpline
  (params (Target :type Vector))
  (bind _spline (Variables|Default|GetSpline))
  (bind _spline_2 (Variables|Default|GetSpline))
  (bind _returnvalue (Spline|GetNumberOfSplinePoints _spline_2))
  (bind (_location _tangent) (Spline|GetLocationandTangentatSplinePoint _spline 0 "Local"))
  (bind _returnvalue_2 (- _returnvalue 2))
  (bind _returnvalue_3 (+ _returnvalue_2 1))
  (bind (_location_2 _tangent_2) (Spline|GetLocationandTangentatSplinePoint _spline _returnvalue_3 "Local"))
  (Spline|AddSplinePoint (Variables|Default|GetSpline) Target "World" true)
  (bind _returnvalue_4 (AddComponent|AddSplineMeshComponent true))
  (Transformation|AttachComponentToComponent _returnvalue_4 0 "None" "KeepRelative" "KeepRelative" "KeepRelative" true)
  (for _index (range 0 _returnvalue_2)
    (SplineMesh|SetStartandEnd _returnvalue_4 _location _tangent _location_2 _tangent_2 true :!class /Script/Engine.SplineMeshComponent)
    (Development|PrintString (Utilities|String|Append "Start:" (Utilities|String|ToString(Vector) _location) ",End:" (Utilities|String|ToString(Vector) _location_2)))))

(event EventBeginPlay)

(event Collision|EventActorBeginOverlap
  (params (OtherActor :type Actor%20Object%20Reference)))

(event EventTick
  (params (DeltaSeconds :type Float%20%28single-precision%29)))

(fn ConstructionScript
  (bind _spline (Variables|Default|GetSpline))
  (for _index (range 0 (- (Spline|GetNumberOfSplinePoints (Variables|Default|GetSpline)) 2))
    (bind _splinemeshcomp (CallFunction|AddSplineMeshComponent))
    (bind _output_get (Variables|Default|SetSplineMesh _splinemeshcomp))
    (Transformation|AttachComponentToComponent _output_get 0 "None" "KeepRelative" "KeepRelative" "KeepRelative" true)
    (SplineMesh|SetStartandEnd (Variables|Default|GetSplineMesh) (.Location (Spline|GetLocationandTangentatSplinePoint _spline _index "Local")) (.Tangent (Spline|GetLocationandTangentatSplinePoint _spline _index "Local")) (.Location (Spline|GetLocationandTangentatSplinePoint _spline (+ _index 1) "Local")) (.Tangent (Spline|GetLocationandTangentatSplinePoint _spline (+ _index 1) "Local")) true :!class /Script/Engine.SplineMeshComponent)))

(fn Test
  (for _array_element (Variables|Default|GetTaget)
    (CallFunction|SpawnSpline _array_element)))

(fn AddPoint
  (params (Pos :type Vector)))

(fn GetMousePos
  (bind _returnvalue (Game|GetPlayerController 0))
  (bind (_worldlocation _worlddirection) (Game|Player|ConvertMouseLocationToWorldSpace _returnvalue))
  (bind _outhits (Collision|MultiLineTraceByChannel _worldlocation (+ _worldlocation (* _worlddirection (LocalVariables|GetMulti))) "TraceTypeQuery1" false 0 "None"))
  (return (.location (Utilities|Array|Get(acopy) _outhits)) (.hitactor (Utilities|Array|Get(acopy) _outhits))))

(fn UpdateCurrentSplinePoint
  (bind _spline (Variables|Default|GetSpline))
  (Spline|RemoveSplinePoint _spline (- (Spline|GetNumberOfSplinePoints _spline) 1) true))

(fn AddSplineMeshComponent
  (bind _returnvalue (AddComponent|AddSplineMeshComponent true))
  (return _returnvalue))