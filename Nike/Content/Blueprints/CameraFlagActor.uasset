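; CameraFlagActor is a world-placed camera flag that displays a widget component and turns it toward the first player character every tick.
; The construction script applies widget space and scale, and passes MediaSource to the widget if it is a CameraButton.
; BeginPlay instead expects a CameraFlag widget, giving it the image and a self reference.
; That widget stays hidden until the Nike HUD signals its main widget is created.
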(event Custom|ShowWidget
  (Widget|SetVisibility (Variables|Default|GetWidget) "Visible"))

(event EventBeginPlay
  (bind _ascamera_flag (Utilities|Casting|CastToCameraFlag (UserInterface|GetWidget (Variables|Default|GetWidget1))))
  (bind _output_get (Variables|Default|SetWidget _ascamera_flag))
  (Variables|/Game/UI/Widgets/CameraFlag.CameraFlag_C|SetBtnImage _output_get (Variables|Default|GetImage))
  (Variables|/Game/UI/Widgets/CameraFlag.CameraFlag_C|SetCameraFlagActor _output_get self)
  (Widget|SetVisibility (Variables|Default|GetWidget) "Hidden")
  (EventDispatchers|BindEventtoOnMainWidgetCreated (CallFunction|GetNikeHUD) (delegate Custom|ShowWidget)))

(event EventTick
  (params (DeltaSeconds :type Float%20%28single-precision%29))
  (bind _returnvalue (Game|GetPlayerCharacter 0))
  (bind _widget1 (Variables|Default|GetWidget1))
  (Utilities|IsValid _returnvalue
    (:Is%20Valid
      (Transformation|SetWorldRotation _widget1 (Math|Rotator|FindLookatRotation (Transformation|GetWorldLocation _widget1) (Transformation|GetActorLocation _returnvalue)) false false))))

(fn ConstructionScript
  (bind _widget1 (Variables|Default|GetWidget1))
  (Class|WidgetComponent|SetWidgetSpace (Variables|Default|GetWidget1) (Variables|Default|GetWidgetSpace))
  (Transformation|SetWorldScale3D _widget1 (Variables|Default|GetWidgeScale))
  (bind _ascamera_button (Utilities|Casting|CastToCameraButton (UserInterface|GetWidget _widget1)))
  (Variables|/Game/UI/Widgets/CameraButton.CameraButton_C|SetMediaSource _ascamera_button (Variables|Default|GetMediaSource)))