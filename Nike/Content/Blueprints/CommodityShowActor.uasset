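; CommodityShowActor is a display actor, apparently for showing a commodity that the player rotates by dragging the mouse.
; Left mouse press and release set and clear a StartRotate flag.
; A rotation branch would combine the current relative rotation with pitch and yaw from negated input axis values scaled by Speed.
; That branch is disconnected from Tick and every other event, so the rotation never executes.
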(event EventBeginPlay)

(event EventTick
  (params (DeltaSeconds :type Float%20%28single-precision%29)))

(event Input|MouseEvents|LeftMouseButton
  (params (Key :type Key%20Structure :default "None"))
  (:Pressed
    (Variables|Default|SetStartRotate true))
  (:Released
    (Variables|Default|SetStartRotate false)))

(fn ConstructionScript)