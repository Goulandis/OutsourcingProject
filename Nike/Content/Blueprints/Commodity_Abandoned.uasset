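; Commodity actor, apparently abandoned, whose mesh shifts toward a target transform and spins while the current pawn is inside its Box.
; Box overlap events set the IsOverlap and SelfRotate flags that Tick reads.
; Tick lerps between the construction-cached InitialTransform and TargetTransform using an Alpha this graph never advances, setting AtTarget on exact match.
; Yaw grows by RotationSpeed each frame, without delta-time scaling.
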(event OnComponentBeginOverlap(Box)
  (params (OverlappedComponent :type Primitive%20Component%20Object%20Reference) (OtherActor :type Actor%20Object%20Reference) (OtherComp :type Primitive%20Component%20Object%20Reference) (OtherBodyIndex :type Integer) (bFromSweep :type Boolean) (SweepResult :type Hit%20Result%20Structure%20%28by%20ref%29))
  (if (and (== OtherActor (CallFunction|GetCurrentPawn)) (not (Variables|Default|GetIsOverlap)))
    (Variables|Default|SetIsOverlap true)
    (Variables|Default|SetSelfRotate true)))

(event OnComponentEndOverlap(Box)
  (params (OverlappedComponent :type Primitive%20Component%20Object%20Reference) (OtherActor :type Actor%20Object%20Reference) (OtherComp :type Primitive%20Component%20Object%20Reference) (OtherBodyIndex :type Integer))
  (if (== OtherActor (CallFunction|GetCurrentPawn))
    (Variables|Default|SetIsOverlap false)
    (Variables|Default|SetSelfRotate false)))

(event EventBeginPlay)

(event Collision|EventActorBeginOverlap
  (params (OtherActor :type Actor%20Object%20Reference)))

(event EventTick
  (params (DeltaSeconds :type Float%20%28single-precision%29))
  (bind _staticmesh (Variables|Default|GetStaticMesh))
  (bind _staticmesh_2 (Variables|Default|GetStaticMesh))
  (bind _staticmesh_3 (Variables|Default|GetStaticMesh))
  (bind _returnvalue (Transformation|GetWorldRotation _staticmesh_3))
  (Utilities|FlowControl|Sequence
    (:then_0
      (if (Variables|Default|GetIsOverlap)
        (if (not (Variables|Default|GetAtTarget))
          (Transformation|SetWorldTransform _staticmesh (Math|Transform|Lerp(Transform) (Variables|Default|GetInitialTransform) (Variables|Default|GetTargetTransform) (Variables|Default|GetAlpha)) false false)
          (if (== (Transformation|GetWorldTransform _staticmesh) (Variables|Default|GetTargetTransform))
            (Variables|Default|SetAtTarget true)))
        (elif (Variables|Default|GetAtTarget)
          (Transformation|SetWorldTransform _staticmesh_2 (Math|Transform|Lerp(Transform) (Variables|Default|GetTargetTransform) (Variables|Default|GetInitialTransform) (Variables|Default|GetAlpha)) false false)
          (if (== (Transformation|GetWorldTransform _staticmesh_2) (Variables|Default|GetInitialTransform))
            (Variables|Default|SetAtTarget false)))))
    (:then_1
      (if (Variables|Default|GetSelfRotate)
        (Transformation|SetWorldRotation _staticmesh_3 (Math|Rotator|MakeRotator (.roll _returnvalue) (.pitch _returnvalue) (+ (.yaw _returnvalue) (Variables|Default|GetRotationSpeed))) false false)))))

(fn ConstructionScript
  (Variables|Default|SetInitialTransform (Transformation|GetWorldTransform (Variables|Default|GetStaticMesh))))