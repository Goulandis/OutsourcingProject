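; Manager for a building floor heat map view that focuses one floor and restores it on exit.
; It indexes BP_LouCeng actors by floor; Tick eases the chosen one toward a focus or initial transform, hiding the others during focus.
; SetFocus toggles heat map material and camera buttons, while ShowOutline uses custom depth.
; Config supplies per-floor button positions, merged with existing video entries and optionally hot-reloaded through a delayed Tick.
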(event EventBeginPlay
  (bind _outactors (Actor|GetAllActorsOfClass "/Game/Mod/ReLiTu/BP_LouCeng.BP_LouCeng_C"))
  (for _array_element _outactors
    (Utilities|Map|Add (Variables|Default|GetFloors) (Variables|/Game/Mod/ReLiTu/BP_LouCeng.BP_LouCeng_C|GetFloorNum _array_element) _array_element)
    (Utilities|Map|Add (Variables|Default|GetFloorsInitTtransform) (Variables|/Game/Mod/ReLiTu/BP_LouCeng.BP_LouCeng_C|GetFloorNum _array_element) (Transformation|GetActorTransform _array_element)))
  (CallFunction|SetFloorCameraDatabyConfig))

(event EventTick
  (params (DeltaSeconds :type Float%20%28single-precision%29))
  (Utilities|FlowControl|Sequence
    (:then_0
      (if (Variables|Default|GetIsFocus)
        (CallFunction|FocusFloor)
        (else
          (CallFunction|RecoverFloor))))
    (:then_1
      (if (Variables|Default|GetHeatMapCameraDynamicSetting)
        (Utilities|FlowControl|Delay 1.0)
        (Default|LoadConfig (Default|GetConfigObj (CallFunction|GetNikeGameInstance)))
        (CallFunction|SetFloorCameraDatabyConfig)
        (Default|UpdateHeatMapCameraButton (Variables|/Game/UI/Widgets/Main.Main_C|GetHeatMapShow (CallFunction|GetNikeMainWidget)))))))

(fn ConstructionScript)

(fn FocusFloor
  (bind _keys (Utilities|Map|Keys (Variables|Default|GetFloors)))
  (for _array_element _keys
    (if (Utilities|Enum|Equal(Enum) _array_element (Variables|Default|GetFocusFloorNum))
      (if (.ReturnValue (Utilities|Map|Find (Variables|Default|GetFloors) _array_element))
        (Rendering|SetActorHiddenInGame (.Value (Utilities|Map|Find (Variables|Default|GetFloors) _array_element)) false)
        (Transformation|SetActorTransform (.Value (Utilities|Map|Find (Variables|Default|GetFloors) _array_element)) (Math|Transform|Lerp(Transform) (Transformation|GetActorTransform (.Value (Utilities|Map|Find (Variables|Default|GetFloors) _array_element))) (Variables|Default|GetFocusTransform) (Variables|Default|GetLerpAlhpa))))
      (elif (.ReturnValue (Utilities|Map|Find (Variables|Default|GetFloors) _array_element))
        (Rendering|SetActorHiddenInGame (.Value (Utilities|Map|Find (Variables|Default|GetFloors) _array_element)) true)))))

(fn SetFocus
  (params (IsFocus :type Boolean) (FloorNum :type FloorNum%20Enum :default "NewEnumerator0"))
  (bind _nikehud (CallFunction|GetNikeHUD))
  (bind _mainwidget (Variables|/Game/GamePlay/NikeHUD.NikeHUD_C|GetMainWidget _nikehud))
  (bind _heatmapshow (Variables|/Game/UI/Widgets/Main.Main_C|GetHeatMapShow _mainwidget))
  (bind _btnheatmapcameraarr (Variables|/Game/UI/Widgets/HeatMapShow.HeatMapShow_C|GetBtnHeatMapCameraArr _heatmapshow))
  (bind _output_get (Variables|Default|SetIsFocus IsFocus))
  (bind _output_get_2 (Variables|Default|SetFocusFloorNum FloorNum))
  (Variables|/Game/UI/Widgets/HeatMapShow.HeatMapShow_C|SetCurrentFloor (Variables|/Game/UI/Widgets/Main.Main_C|GetHeatMapShow (Variables|/Game/GamePlay/NikeHUD.NikeHUD_C|GetMainWidget (CallFunction|GetNikeHUD))) _output_get_2)
  (if _output_get
    (if (.ReturnValue (Utilities|Map|Find (Variables|Default|GetFloors) _output_get_2))
      (Default|SetHeatMapMaterial (.Value (Utilities|Map|Find (Variables|Default|GetFloors) _output_get_2)))
      (for _array_element _btnheatmapcameraarr
        (Widget|SetVisibility _array_element "Visible")))
    (else
      (Default|ReveseMaterial (.Value (Utilities|Map|Find (Variables|Default|GetFloors) _output_get_2)))
      (for _array_element_2 _btnheatmapcameraarr
        (Widget|SetVisibility _array_element_2 "Hidden")))))

(fn RecoverFloor
  (bind _floorsinitttransform (Variables|Default|GetFloorsInitTtransform))
  (bind _focusfloornum (Variables|Default|GetFocusFloorNum))
  (bind (_value _returnvalue) (Utilities|Map|Find _floorsinitttransform _focusfloornum))
  (bind _keys (Utilities|Map|Keys (Variables|Default|GetFloors)))
  (for _array_element _keys
    (if (Utilities|Enum|Equal(Enum) _array_element _focusfloornum)
      (if (and (.ReturnValue (Utilities|Map|Find (Variables|Default|GetFloors) _array_element)) _returnvalue)
        (Transformation|SetActorTransform (.Value (Utilities|Map|Find (Variables|Default|GetFloors) _array_element)) (Math|Transform|Lerp(Transform) (Transformation|GetActorTransform (.Value (Utilities|Map|Find (Variables|Default|GetFloors) _array_element))) _value (Variables|Default|GetLerpAlhpa))))
      (elif (and (.ReturnValue (Utilities|Map|Find (Variables|Default|GetFloors) _array_element)) _returnvalue)
        (Rendering|SetActorHiddenInGame (.Value (Utilities|Map|Find (Variables|Default|GetFloors) _array_element)) false)))))

(fn RecoverFloorQuik
  (params (FloorNum :type FloorNum%20Enum :default "NewEnumerator0"))
  (bind _floors (Variables|Default|GetFloors))
  (bind _floorsinitttransform (Variables|Default|GetFloorsInitTtransform))
  (bind (_value _returnvalue) (Utilities|Map|Find _floors FloorNum))
  (bind (_value_2 _returnvalue_2) (Utilities|Map|Find _floorsinitttransform FloorNum))
  (if (and _returnvalue _returnvalue_2)
    (Transformation|SetActorTransform _value _value_2)))

(fn ShowOutline
  (params (Floor :type FloorNum%20Enum :default "NewEnumerator0") (Show :type Boolean))
  (bind _floors (Variables|Default|GetFloors))
  (bind (_value _returnvalue) (Utilities|Map|Find _floors Floor))
  (if _returnvalue
    (for _array_element (Components|GetChildrenComponents (Variables|/Script/Engine.Actor|GetRootComponent _value) false)
      (bind _asstatic_mesh_component (Utilities|Casting|CastToStaticMeshComponent _array_element))
      (Rendering|SetRenderCustomDepth _asstatic_mesh_component Show))))

(fn UpdateHeatMapCameraSetting
  (bind _floorcameradata (Variables|Default|GetFloorCameraData))
  (bind _focusfloornum (Variables|Default|GetFocusFloorNum))
  (bind _value (Utilities|Map|Find _floorcameradata _focusfloornum))
  (for _array_element (Variables|/Game/Blueprints/LoadConfig.LoadConfig_C|GetHeatMapCameraPostions (Default|GetConfigObj (CallFunction|GetNikeGameInstance)))
    (if (Utilities|Enum|Equal(Enum) (.floornum _array_element) (Variables|Default|GetFocusFloorNum))
      (if (.ReturnValue (Utilities|Map|Find (Variables|Default|GetFloorCameraData) (.floornum _array_element)))
        (if (== (Utilities|Array|Length (.cameradataarr (.Value (Utilities|Map|Find (Variables|Default|GetFloorCameraData) (.floornum _array_element))))) (Utilities|Array|Length (.positions _array_element)))
          (for (_array_element_2 _array_index) (.positions _array_element)
            (Utilities|Array|SetArrayElem (.cameradataarr _value) _array_index (Utilities|Struct|MakeHeatMapCameraData (Math|Vector2D|MakeVector2D (.x _array_element_2) (.y _array_element_2)) (.video (Utilities|Array|Get(acopy) (.cameradataarr _value) _array_index)))))))))
  (CallFunction|SetHeatMapCameraPosition))

(fn SetHeatMapCameraPosition
  (bind _mainwidget (CallFunction|GetNikeMainWidget))
  (bind _floorcameradata (Variables|Default|GetFloorCameraData))
  (bind _focusfloornum (Variables|Default|GetFocusFloorNum))
  (bind (_value _returnvalue) (Utilities|Map|Find _floorcameradata _focusfloornum))
  (bind _heatmapshow (Variables|/Game/UI/Widgets/Main.Main_C|GetHeatMapShow _mainwidget))
  (bind _btnheatmapcameraarr (Variables|/Game/UI/Widgets/HeatMapShow.HeatMapShow_C|GetBtnHeatMapCameraArr _heatmapshow))
  (Utilities|IsValid (Variables|/Game/GamePlay/NikeHUD.NikeHUD_C|GetMainWidget (CallFunction|GetNikeHUD))
    (:Is%20Valid
      (if _returnvalue
        (if (== (Utilities|Array|Length (.cameradataarr _value)) (Utilities|Array|Length _btnheatmapcameraarr))
          (for (_array_element _array_index) (.cameradataarr _value)
            (Class|CanvasPanelSlot|SetPosition (Class|WidgetLayoutLibrary|SlotasCanvasSlot (Utilities|Array|Get(acopy) _btnheatmapcameraarr _array_index)) (.margin _array_element))))))))

(fn SetFloorCameraDatabyConfig
  (bind _floorcameradata (Variables|Default|GetFloorCameraData))
  (LocalVariables|SetTemp _floorcameradata)
  (Utilities|Map|Clear _floorcameradata)
  (for _array_element (Variables|/Game/Blueprints/LoadConfig.LoadConfig_C|GetHeatMapCameraPostions (Default|GetConfigObj (CallFunction|GetNikeGameInstance)))
    (LocalVariables|SetFloorNum (.floornum _array_element))
    (if (.ReturnValue (Utilities|Map|Find (LocalVariables|GetTemp) (LocalVariables|GetFloorNum)))
      (if (== (Utilities|Array|Length (.positions _array_element)) (Utilities|Array|Length (.cameradataarr (.Value (Utilities|Map|Find (LocalVariables|GetTemp) (LocalVariables|GetFloorNum))))))
        (for (_array_element_2 _array_index) (.positions _array_element)
          (Utilities|Array|Add (LocalVariables|GetCameraDatas) (Utilities|Struct|MakeHeatMapCameraData (Math|Vector2D|MakeVector2D (.x _array_element_2) (.y _array_element_2)) (.video (Utilities|Array|Get(acopy) (.cameradataarr (.Value (Utilities|Map|Find (LocalVariables|GetTemp) (LocalVariables|GetFloorNum)))) _array_index)))))
        (Utilities|Map|Add (Variables|Default|GetFloorCameraData) (LocalVariables|GetFloorNum) (Utilities|Struct|MakeHeatMapCameraDataArr (LocalVariables|GetCameraDatas)))
        (Utilities|Array|Clear (LocalVariables|GetCameraDatas))
        (else
          (CallFunction|DebugLog "SetFloorCameraDataByConfig" (Utilities|String|Append "Array length no match, Position=" (Utilities|String|ToString(Integer) (Utilities|Array|Length (.positions _array_element))) ",but Temp=" (Utilities|String|ToString(Integer) (Utilities|Array|Length (.cameradataarr (.Value (Utilities|Map|Find (LocalVariables|GetTemp) (LocalVariables|GetFloorNum))))))))))
      (else
        (CallFunction|DebugLog "SetFloorCameraDataByConfig" (Utilities|String|Append "Failed to find " (Utilities|String|EnumtoString (LocalVariables|GetFloorNum)) " in TempMap"))))))