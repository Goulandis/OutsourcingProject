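; Config Blueprint that loads game settings from Config/Config.json in the content directory through the VaRest plugin.
; LoadConfig reads language, resolution list, default resolution and screen mode, then builds per-floor (B1 to F3) heat map camera positions from nested JSON arrays.
; It prints parse failures and the loaded JSON.
; SetDefaultResolution updates the stored default, while SaveConfig is an empty stub.
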(fn LoadConfig
  (bind _returnvalue (Class|BlueprintPathsLibrary|ProjectContentDir))
  (bind _returnvalue_2 (Utilities|String|Append _returnvalue "Config/Config.json"))
  (Development|PrintString 0 (Utilities|String|Append "Loaded file " _returnvalue_2))
  (bind _returnvalue_3 (Class|VaRestSubsystem|LoadJsonfromFile (|VaRestSubsystem) "Config/Config.json" true))
  (Utilities|IsValid _returnvalue_3
    (:Is%20Valid
      (Variables|Default|SetLanguage (Class|VaRestJsonObject|GetStringField _returnvalue_3 "Language"))
      (Variables|Default|SetResolutions (Class|VaRestJsonObject|GetStringArrayField _returnvalue_3 "Resolution"))
      (Variables|Default|SetDefaultResolution (Class|VaRestJsonObject|GetStringField _returnvalue_3 "DefaultResolution"))
      (Variables|Default|SetDefaultScreenMode (Class|VaRestJsonObject|GetStringField _returnvalue_3 "DefaultScreenMode"))
      (for _array_element (Class|VaRestJsonObject|GetArrayField _returnvalue_3 "HeamtMapCameraPostion")
        (bind _returnvalue_4 (Class|VaRestJsonValue|AsObject _array_element))
        (Utilities|IsValid _returnvalue_4
          (:Is%20Valid
            (for _array_element_2 (Class|VaRestJsonObject|GetArrayField _returnvalue_4 "Positions")
              (bind _returnvalue_5 (Class|VaRestJsonValue|AsObject _array_element_2))
              (Utilities|IsValid _returnvalue_5
                (:Is%20Valid
                  (Utilities|Array|Add (LocalVariables|GetPostions) (Utilities|Struct|MakeHeatMapCameraConfigPos (Class|VaRestJsonObject|GetIntegerField _returnvalue_5 "Index") (Class|VaRestJsonObject|GetNumberField _returnvalue_5 "X") (Class|VaRestJsonObject|GetNumberField _returnvalue_5 "Y"))))
                (:Is%20Not%20Valid
                  (Development|PrintString 0 "[LoadConfig]Failed to parse Positions item to json object"))))
            (switch string (Class|VaRestJsonObject|GetStringField _returnvalue_4 "FloorNum")
              (:F3
                (LocalVariables|SetFloorNum "NewEnumerator3"))
              (:F2
                (LocalVariables|SetFloorNum "NewEnumerator2"))
              (:F1
                (LocalVariables|SetFloorNum "NewEnumerator1"))
              (:B1
                (LocalVariables|SetFloorNum "NewEnumerator0")))
            (Utilities|Array|Add (Variables|Default|GetHeatMapCameraPostions) (Utilities|Struct|MakeHeatMapCameraConfigObj (LocalVariables|GetFloorNum) (LocalVariables|GetPostions)))
            (Utilities|Array|Clear (LocalVariables|GetPostions)))
          (:Is%20Not%20Valid
            (Development|PrintString 0 "[LoadConfig]Failed to parse HeamtMapCameraPostion item to json object"))))
      (Development|PrintString 0 (Utilities|String|Append "Loaded the json:" (Class|VaRestJsonObject|EncodeJsontoSingleString _returnvalue_3))))
    (:Is%20Not%20Valid
      (Development|PrintString 0 (Utilities|String|Append "Failed to load Config.josn that path is " _returnvalue_2)))))

(fn SetDefaultResolution
  (params (Resolution :type String))
  (Variables|Default|SetDefaultResolution Resolution))

(fn SaveConfig
  (params (Resolutions :type Array%20of%20Strings) (DefaultResolution :type String) (DefaultScreenMode :type String) (HeatMapCameraPostion :type Array%20of%20Heat%20Map%20Camera%20Config%20Obj%20Structures)))