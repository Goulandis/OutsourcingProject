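; ViewManager is an actor that supplies viewpoint images for each building floor and controls a level sequence.
; GetFloorViewImages maps a floor (B1 to F3) to three hardcoded Chinese viewpoint keys, which AddFloorViewImages looks up in ViewPointsMap to collect images.
; PlaySequencer loops, stops or pauses the assigned Sequencer's player.
; Missing keys and an invalid sequencer are reported through DebugLog.
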(event EventBeginPlay)

(event Collision|EventActorBeginOverlap
  (params (OtherActor :type Actor%20Object%20Reference)))

(event EventTick
  (params (DeltaSeconds :type Float%20%28single-precision%29)))

(fn ConstructionScript)

(fn GetFloorViewImages
  (params (FloorNum :type FloorNum%20Enum :default "NewEnumerator0"))
  (bind _floorviewimages (LocalVariables|GetFloorViewImages))
  (bind _floorviewimages_2 (LocalVariables|GetFloorViewImages))
  (switch Utilities|FlowControl|Switch|SwitchonFloorNum FloorNum
    (:NewEnumerator0
      (CallFunction|AddFloorViewImages "负一楼一号视点" _floorviewimages_2)
      (CallFunction|AddFloorViewImages "负一楼二号视点" _floorviewimages_2)
      (CallFunction|AddFloorViewImages "负一楼三号视点" _floorviewimages_2))
    (:NewEnumerator1
      (CallFunction|AddFloorViewImages "一楼一号视点" _floorviewimages_2)
      (CallFunction|AddFloorViewImages "一楼二号视点" _floorviewimages_2)
      (CallFunction|AddFloorViewImages "一楼三号视点" _floorviewimages_2))
    (:NewEnumerator2
      (CallFunction|AddFloorViewImages "二楼一号视点" _floorviewimages)
      (CallFunction|AddFloorViewImages "二楼二号视点" _floorviewimages)
      (CallFunction|AddFloorViewImages "二楼三号视点" _floorviewimages))
    (:NewEnumerator3
      (CallFunction|AddFloorViewImages "三楼一号视点" _floorviewimages)
      (CallFunction|AddFloorViewImages "三楼二号视点" _floorviewimages)
      (CallFunction|AddFloorViewImages "三楼三号视点" _floorviewimages)))
  (return (LocalVariables|GetFloorViewImages)))

(fn AddFloorViewImages
  (params (Key :type String) (InImages :type Array%20of%20Texture%20Object%20References))
  (bind _viewpointsmap (Variables|Default|GetViewPointsMap))
  (bind (_value _returnvalue) (Utilities|Map|Find _viewpointsmap Key))
  (if _returnvalue
    (Utilities|Array|Add InImages (.image _value))
    (else
      (CallFunction|DebugLog "AddFloorViewImages" (Utilities|String|Append "The view no set image that key is " Key)))))

(fn PlaySequencer
  (params (Play :type String))
  (bind _sequencer (Variables|Default|GetSequencer))
  (bind _sequenceplayer (Variables|/Script/LevelSequence.LevelSequenceActor|GetSequencePlayer _sequencer))
  (Utilities|IsValid _sequencer
    (:Is%20Valid
      (switch string Play
        (:Play
          (Class|MovieSceneSequencePlayer|PlayLooping _sequenceplayer 100))
        (:Stop
          (Sequencer|Player|Stop _sequenceplayer :!class /Script/MovieScene.MovieSceneSequencePlayer))
        (:Pause
          (Sequencer|Player|Pause _sequenceplayer))))
    (:Is%20Not%20Valid
      (CallFunction|DebugLog "PlaySequencer" "LevelSequencer is not valid"))))