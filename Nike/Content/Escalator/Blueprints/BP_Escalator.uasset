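; Modular escalator actor that also builds as a flat moving walkway, with animated steps and handrail.
; The construction script sets module meshes, repeats middle segments by Extension, positions the end module and spawns steps along the path.
; AnimateEscalator scrolls the handrail material and offsets steps by a per-call Speed in either direction, wrapping them at the ends.
; BP_EscalatorManager drives animation when present, disabling Tick; otherwise Tick does.
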(event Custom|Animate
  (CallFunction|AnimateEscalator))

(event EventBeginPlay
  (bind _outactors (Actor|GetAllActorsOfClass "/Game/Escalator/Blueprints/BP_EscalatorManager.BP_EscalatorManager_C"))
  (if (Utilities|Array|IsValidIndex _outactors)
    (EventDispatchers|BindEventtoUpdateEscalators (Utilities|Array|Get(acopy) _outactors) (delegate Custom|Animate))
    (Variables|Default|SetHas%20Manager true)
    (Actor|Tick|SetActorTickEnabled false)
    (else
      (Variables|Default|SetHas%20Manager false))))

(event EventTick
  (params (DeltaSeconds :type Float%20%28single-precision%29))
  ;[1 1 1] Tick
  (if (not (Variables|Default|GetHas%20Manager))
    (CallFunction|AnimateEscalator)))

(fn ConstructionScript
  (bind _escalator (Variables|Escalator|Parameters|GetEscalator))
  (bind _elevationend (Variables|Default|GetElevationEnd))
  (bind _ending (Variables|Default|GetEnding))
  (bind _beginning (Variables|Default|GetBeginning))
  (bind _ending_2 (Variables|Default|GetEnding))
  (bind _elevationstart (Variables|Default|GetElevationStart))
  (bind _beginning_2 (Variables|Default|GetBeginning))
  (bind _ending_3 (Variables|Default|GetEnding))
  (bind _escalator_2 (Variables|Escalator|Parameters|GetEscalator))
  (bind _extension (Variables|Escalator|Parameters|GetExtension))
  (bind _returnvalue (select _escalator "ECR_Block" "ECR_Ignore"))
  (bind _relativelocation (Variables|/Script/Engine.SceneComponent|GetRelativeLocation _ending))
  (bind _relativelocation_2 (Variables|/Script/Engine.SceneComponent|GetRelativeLocation _beginning))
  (bind _relativelocation_3 (Variables|/Script/Engine.SceneComponent|GetRelativeLocation _ending_2))
  (bind _relativelocation_4 (Variables|/Script/Engine.SceneComponent|GetRelativeLocation _beginning_2))
  (bind _relativelocation_5 (Variables|/Script/Engine.SceneComponent|GetRelativeLocation _ending_3))
  (bind _returnvalue_2 (- _relativelocation_2 _relativelocation_3))
  (bind _returnvalue_3 (- _relativelocation_4 _relativelocation_5))
  (bind _returnvalue_4 (Math|Vector|VectorLength _returnvalue_2))
  (bind _returnvalue_5 (Math|Vector|VectorLength _returnvalue_3))
  (bind _returnvalue_6 (/ _returnvalue_4 32.5))
  (bind _returnvalue_7 (/ _returnvalue_5 32.5))
  (bind _returnvalue_8 (Math|Float|Ceil _returnvalue_7))
  (bind _returnvalue_9 (Math|Float|Ceil _returnvalue_6))
  (bind _returnvalue_10 (+ _returnvalue_8 3))
  (bind _returnvalue_11 (+ _returnvalue_9 2))
  ;[1 1 1] Static Mesh Modules
  (for (_array_element _array_index) (Utilities|Array|MakeArray (Variables|Default|GetBeginning) (Variables|Default|GetBeginningFloor) (Variables|Default|GetElevationStart) (Variables|Default|GetRubberSegment01) (Variables|Default|GetEnding) (Variables|Default|GetEndingFloor) (Variables|Default|GetElevationEnd) (Variables|Default|GetRubberSegment02))
    (Utilities|IsValid _array_element
      (:Is%20Valid
        (Components|StaticMesh|SetStaticMesh _array_element (Utilities|Array|Get(acopy) (Utilities|Array|MakeArray (Variables|Escalator|Modules|GetBeginning%20Module) (Variables|Escalator|Modules|GetBeginning%20Floor) (Variables|Escalator|Modules|GetElevation%20Start) (Variables|Escalator|Modules|GetHandrail%20Segment%2001) (Variables|Escalator|Modules|GetEnding%20Module) (Variables|Escalator|Modules|GetEnding%20Floor) (Variables|Escalator|Modules|GetElevation%20End) (Variables|Escalator|Modules|GetHandrail%20Segment%2002)) _array_index)))))
  ;[1 1 1] Material Management
  (bind _returnvalue_12 (Rendering|Material|CreateDynamicMaterialInstance "/Game/Escalator/Materials/MI_Escalator_Rubber.MI_Escalator_Rubber" "Handrail" :!class /Script/Engine.KismetMaterialLibrary))
  (Variables|Default|SetHandrail%20Material _returnvalue_12)
  (for _array_element_2 (Utilities|Array|MakeArray (Variables|Default|GetElevationStart) (Variables|Default|GetEnding) (Variables|Default|GetElevationEnd) (Variables|Default|GetBeginning))
    (Rendering|Material|SetMaterial _array_element_2 (Rendering|Material|GetMaterialIndex _array_element_2 "Rubber") (Variables|Default|GetHandrail%20Material)))
  ;[1 1 1] Clear Array
  (Utilities|Array|Clear (Variables|Default|GetSteps))
  ;[1 1 1] Hide/Show Inclination Modules
  (Rendering|SetVisibility (Variables|Default|GetRubberSegment01) (not _escalator) false)
  (Rendering|SetVisibility _elevationend _escalator_2 false)
  (Collision|SetCollisionResponsetoAllChannels _elevationend _returnvalue)
  (Rendering|SetVisibility _elevationstart _escalator_2 false)
  (Collision|SetCollisionResponsetoAllChannels _elevationstart _returnvalue)
  ;[1 1 1] Array Middle Segments
  (for _index (range 0 (- (Variables|Escalator|Parameters|GetExtension) 1))
    (if (Variables|Escalator|Parameters|GetEscalator)
      (bind _returnvalue_13 (AddComponent|AddStaticMeshComponent false (Math|Transform|MakeTransform (+ (Variables|/Script/Engine.SceneComponent|GetRelativeLocation (Variables|Default|GetElevationStart)) (* "-38.292725, 0,26.819998" _index)) "0, 0, 0" "1,1,1")))
      (Components|StaticMesh|SetStaticMesh _returnvalue_13 "/Game/Escalator/Meshes/SM_Module04.SM_Module04")
      (Rendering|Material|SetMaterial _returnvalue_13 (Rendering|Material|GetMaterialIndex _returnvalue_13 "Rubber") (Variables|Default|GetHandrail%20Material))
      (else
        (bind _returnvalue_14 (AddComponent|AddStaticMeshComponent false (Math|Transform|MakeTransform (+ "-68.684502, 0, 0" (* "-46.750000, 0,0.000000" _index)) "0, 0, 0" "1,1,1")))
        (Components|StaticMesh|SetStaticMesh _returnvalue_14 "/Game/Escalator/Meshes/SM_Module06.SM_Module06")
        (Rendering|Material|SetMaterial _returnvalue_14 (Rendering|Material|GetMaterialIndex _returnvalue_14 "Rubber") (Variables|Default|GetHandrail%20Material)))))
  ;[1 1 1] Offset Beginning and End
  (Transformation|SetRelativeLocation (Variables|Default|GetEnding) (Math|Vector|Lerp(Vector) (+ (* "-46.750000, 0, 0" _extension) "-90.500000,0.000000,0.000000") (+ (* "-38.292725, 0,26.819998" _extension) "-259.967834,0.000000,53.380001") (Math|Conversions|ToFloat(Boolean) (Variables|Escalator|Parameters|GetEscalator))) false false)
  (if (Variables|Escalator|Parameters|GetEscalator)
    ;[1 1 1] Add Steps to Escalators
    (for _index_2 (range 0 _returnvalue_10)
      ;;[1 1 1] Offset By Step
      (Utilities|FlowControl|Sequence
        (:then_0
          (if (> (* (+ (* (* _index_2 -32.5) -0.700231) -103.790543) 0.8461) (.z _relativelocation))
            (Utilities|FlowControl|DoOnce false :!label _label
              (:Completed
                (Variables|Default|SetAmount%20of%20Steps%20Until%20End (- _index_2 1))))
            (else
              (goto _label Reset))))
        (:then_1
          ;;[1 1 1] Add Static Mesh and store inside array "Steps"
          (bind _returnvalue_15 (AddComponent|AddStaticMeshComponent false (Math|Transform|MakeTransform (+ (Variables|Default|GetFirst%20Step%20Location) (Math|Vector|MakeVector (Math|Float|Lerp (Math|Float|Lerp (- (* _index_2 -32.5) (* (/ (- (* _index_2 -32.5) -148.223297) 32.5) 5.0)) (* _index_2 -32.5) (Math|Conversions|ToFloat(Boolean) (> (* _index_2 -32.5) -148.223297))) (+ (Math|Float|Lerp (- (* _index_2 -32.5) (* (/ (- (* _index_2 -32.5) -148.223297) 32.5) 5.0)) (* _index_2 -32.5) (Math|Conversions|ToFloat(Boolean) (> (* _index_2 -32.5) -148.223297))) (* (- (* _index_2 -32.5) (* (Variables|Default|GetAmount%20of%20Steps%20Until%20End) -32.5)) 0.152382)) (Math|Conversions|ToFloat(Boolean) (> (* (+ (* (* _index_2 -32.5) -0.700231) -103.790543) 0.8461) (.z _relativelocation)))) 0.0 (Math|Float|Lerp (Math|Float|Clamp(Float) (* (+ (* (* _index_2 -32.5) -0.700231) -103.790543) 0.8461) -5e+05 (.z _relativelocation)) 0.0 (Math|Conversions|ToFloat(Boolean) (> (* _index_2 -32.5) -148.223297))))) "0, 0, 0" "1,1,1")))
          (Components|StaticMesh|SetStaticMesh _returnvalue_15 "/Game/Escalator/Meshes/SM_Module07.SM_Module07")
          (Utilities|Array|Add (Variables|Default|GetSteps) _returnvalue_15)
          ;;[1 1 1] Store Last Step Location
          (if (== _index_2 _returnvalue_10)
            (Variables|Default|SetLast%20Step%20Location (+ (Variables|Default|GetFirst%20Step%20Location) (Math|Vector|MakeVector (Math|Float|Lerp (Math|Float|Lerp (- (* _index_2 -32.5) (* (/ (- (* _index_2 -32.5) -148.223297) 32.5) 5.0)) (* _index_2 -32.5) (Math|Conversions|ToFloat(Boolean) (> (* _index_2 -32.5) -148.223297))) (+ (Math|Float|Lerp (- (* _index_2 -32.5) (* (/ (- (* _index_2 -32.5) -148.223297) 32.5) 5.0)) (* _index_2 -32.5) (Math|Conversions|ToFloat(Boolean) (> (* _index_2 -32.5) -148.223297))) (* (- (* _index_2 -32.5) (* (Variables|Default|GetAmount%20of%20Steps%20Until%20End) -32.5)) 0.152382)) (Math|Conversions|ToFloat(Boolean) (> (* (+ (* (* _index_2 -32.5) -0.700231) -103.790543) 0.8461) (.z _relativelocation)))) 0.0 (Math|Float|Lerp (Math|Float|Clamp(Float) (* (+ (* (* _index_2 -32.5) -0.700231) -103.790543) 0.8461) -5e+05 (.z _relativelocation)) 0.0 (Math|Conversions|ToFloat(Boolean) (> (* _index_2 -32.5) -148.223297))))))))))
    (else
      ;[1 1 1] Add Steps To Non Escalators
      (for _index_3 (range 0 _returnvalue_11)
        ;;[1 1 1] Add Static Mesh and store inside array "Steps"
        (bind _returnvalue_16 (AddComponent|AddStaticMeshComponent false (Math|Transform|MakeTransform (+ "30.000000, 0,-10.000000" (Math|Vector|MakeVector (* _index_3 -32.5) 0.0 0.0)) "0, 0, 0" "1,1,1")))
        (Components|StaticMesh|SetStaticMesh _returnvalue_16 "/Game/Escalator/Meshes/SM_Module07.SM_Module07")
        (Utilities|Array|Add (Variables|Default|GetSteps) _returnvalue_16))
      ;;[1 1 1] Store Last Step Location
      (Variables|Default|SetLast%20Step%20Location (+ "30.000000, 0,-10.000000" (Math|Vector|MakeVector (* _returnvalue_11 -32.5) 0.0 0.0))))))

(fn AnimateEscalator
  (bind _speed (Variables|Escalator|Parameters|GetSpeed))
  (bind _change_direction (Variables|Escalator|Parameters|GetChange%20Direction))
  (bind _speed_2 (Variables|Escalator|Parameters|GetSpeed))
  (bind _change_direction_2 (Variables|Escalator|Parameters|GetChange%20Direction))
  (bind _speed_3 (Variables|Escalator|Parameters|GetSpeed))
  (bind _returnvalue (Math|Conversions|ToFloat(Boolean) _change_direction))
  (bind _returnvalue_2 (- 0.0 _speed))
  (bind _returnvalue_3 (Math|Conversions|ToFloat(Boolean) _change_direction_2))
  (bind _returnvalue_4 (- 0.0 _speed_2))
  (bind _returnvalue_5 (Math|Float|Lerp _speed _returnvalue_2 _returnvalue))
  (bind _returnvalue_6 (Math|Float|Lerp _speed_2 _returnvalue_4 _returnvalue_3))
  (Rendering|Material|SetScalarParameterValue (Variables|Default|GetHandrail%20Material) "V Speed" (* (Variables|Escalator|Parameters|GetSpeed) 2.0 (Math|Float|Lerp 1.0 -1.0 (Math|Conversions|ToFloat(Boolean) (Variables|Escalator|Parameters|GetChange%20Direction)))) :!class /Script/Engine.MaterialInstanceDynamic)
  (if (Variables|Escalator|Parameters|GetEscalator)
    ;[1 1 1] Move Escalator
    (for _array_element (Variables|Default|GetSteps)
      (if (Variables|Escalator|Parameters|GetChange%20Direction)
        (if (< (.x (Variables|/Script/Engine.SceneComponent|GetRelativeLocation _array_element)) (.x (Variables|Default|GetLast%20Step%20Location)))
          (Utilities|MoveSteptoBeginning _array_element))
        (Transformation|AddLocalOffset _array_element (Math|Vector|MakeVector (Math|Float|Lerp _returnvalue_5 (* _returnvalue_5 0.85) (Math|Conversions|ToFloat(Boolean) (and (< (.z (Variables|/Script/Engine.SceneComponent|GetRelativeLocation _array_element)) (.z (Variables|Default|GetLast%20Step%20Location))) (< (.x (Variables|/Script/Engine.SceneComponent|GetRelativeLocation _array_element)) -118.578598)))) 0.0 (Math|Float|Lerp 0.0 (* _returnvalue_5 -0.700231 0.85) (Math|Conversions|ToFloat(Boolean) (and (< (.z (Variables|/Script/Engine.SceneComponent|GetRelativeLocation _array_element)) (.z (Variables|Default|GetLast%20Step%20Location))) (< (.x (Variables|/Script/Engine.SceneComponent|GetRelativeLocation _array_element)) -118.578598))))) false false)
        (else
          (if (> (.x (Variables|/Script/Engine.SceneComponent|GetRelativeLocation _array_element)) (.x (Variables|Default|GetFirst%20Step%20Location)))
            (Utilities|MoveSteptoEnd _array_element))
          (Transformation|AddLocalOffset _array_element (Math|Vector|MakeVector (Math|Float|Lerp _returnvalue_6 (* _returnvalue_6 0.85) (Math|Conversions|ToFloat(Boolean) (and (> (.x (Variables|/Script/Engine.SceneComponent|GetRelativeLocation _array_element)) (+ (.x (Variables|/Script/Engine.SceneComponent|GetRelativeLocation (Variables|Default|GetEnding))) 63.0)) (> (.z (Variables|/Script/Engine.SceneComponent|GetRelativeLocation _array_element)) (.z (Variables|Default|GetFirst%20Step%20Location)))))) 0.0 (Math|Float|Lerp 0.0 (* _returnvalue_6 -0.700231 0.85) (Math|Conversions|ToFloat(Boolean) (and (> (.x (Variables|/Script/Engine.SceneComponent|GetRelativeLocation _array_element)) (+ (.x (Variables|/Script/Engine.SceneComponent|GetRelativeLocation (Variables|Default|GetEnding))) 63.0)) (> (.z (Variables|/Script/Engine.SceneComponent|GetRelativeLocation _array_element)) (.z (Variables|Default|GetFirst%20Step%20Location))))))) false false))))
    (else
      ;[1 1 1] Move Non Escalator
      (for _array_element_2 (Variables|Default|GetSteps)
        (if (Variables|Escalator|Parameters|GetChange%20Direction)
          (if (< (.x (Variables|/Script/Engine.SceneComponent|GetRelativeLocation _array_element_2)) (.x (Variables|Default|GetLast%20Step%20Location)))
            (Transformation|SetRelativeLocation _array_element_2 (- (Variables|/Script/Engine.SceneComponent|GetRelativeLocation _array_element_2) (- (Variables|Default|GetLast%20Step%20Location) (Variables|Default|GetFirst%20Step%20Location))) false false))
          (elif (> (.x (Variables|/Script/Engine.SceneComponent|GetRelativeLocation _array_element_2)) (.x (Variables|Default|GetFirst%20Step%20Location)))
            (Transformation|SetRelativeLocation _array_element_2 (+ (- (Variables|Default|GetLast%20Step%20Location) (Variables|Default|GetFirst%20Step%20Location)) (Variables|/Script/Engine.SceneComponent|GetRelativeLocation _array_element_2)) false false)))
        (Transformation|AddLocalOffset _array_element_2 (Math|Vector|MakeVector (Math|Float|Lerp _speed_3 (- 0.0 _speed_3) (Math|Conversions|ToFloat(Boolean) (Variables|Escalator|Parameters|GetChange%20Direction))) 0.0 0.0) false false)))))