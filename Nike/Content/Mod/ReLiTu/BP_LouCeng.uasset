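; BP_LouCeng is a building floor actor (LouCeng) whose mesh, SMReLiTu01, can toggle a heat map (ReLiTu) look.
; When the mesh has exactly two materials, its construction script caches the first one as OldMaterial.
; SetHeatMapMaterial puts HeatMapMaterial on slot 1, and ReveseMaterial puts OldMaterial on that slot, although it was read from slot 0.
; The event graph holds only disabled stubs.
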(event EventBeginPlay)

(event Collision|EventActorBeginOverlap
  (params (OtherActor :type Actor%20Object%20Reference)))

(event EventTick
  (params (DeltaSeconds :type Float%20%28single-precision%29)))

(fn ConstructionScript
  (bind _sm_relitu_01 (Variables|Default|GetSM_ReLiTu_01))
  (bind _returnvalue (Rendering|Material|GetMaterials _sm_relitu_01))
  (if (== (Utilities|Array|Length _returnvalue) 2)
    (Variables|Default|SetOldMaterial (Utilities|Array|Get(acopy) _returnvalue))))

(fn SetHeatMapMaterial
  (Rendering|Material|SetMaterial (Variables|Default|GetSM_ReLiTu_01) 1 (Variables|Default|GetHeatMapMaterial)))

(fn ReveseMaterial
  (Rendering|Material|SetMaterial (Variables|Default|GetSM_ReLiTu_01) 1 (Variables|Default|GetOldMaterial)))