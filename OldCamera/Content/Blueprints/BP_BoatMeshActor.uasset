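; Boat mesh actor that displays a submarine-style static mesh with selectable color variants.
; The ChangeMaterial event takes an index and sets the first material slot to an aqua, green or yellow sci-fi submarine material instance.
; Any other index leaves the material unchanged, and the actor has no other active logic.
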(event EventBeginPlay)

(event Collision|EventActorBeginOverlap
  (params (OtherActor :type Actor%20Object%20Reference)))

(event EventTick
  (params (DeltaSeconds :type Float%20%28single-precision%29)))

(event EventChangeMaterial
  (params (material_idx :type Integer))
  (Utilities|FlowControl|Sequence
    (:then_0
      (if (== material_idx 0)
        (Rendering|Material|SetMaterial (Variables|Default|GetStaticMesh) 0 "/Game/SciFiOceanSubmarine/Materials/ScifiOceanSubmarine/Hull/MI_ScifiOceanSubmarine_Aqua.MI_ScifiOceanSubmarine_Aqua")))
    (:then_1
      (if (== material_idx 1)
        (Rendering|Material|SetMaterial (Variables|Default|GetStaticMesh) 0 "/Game/SciFiOceanSubmarine/Materials/ScifiOceanSubmarine/Hull/MI_ScifiOceanSubmarine_Green.MI_ScifiOceanSubmarine_Green")))
    (:then_2
      (if (== material_idx 2)
        (Rendering|Material|SetMaterial (Variables|Default|GetStaticMesh) 0 "/Game/SciFiOceanSubmarine/Materials/ScifiOceanSubmarine/Hull/MI_ScifiOceanSubmarine_Yellow.MI_ScifiOceanSubmarine_Yellow")))))

(fn ConstructionScript)