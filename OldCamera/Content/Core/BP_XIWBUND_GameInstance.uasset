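; Game instance for XIWBUND that plays indexed game audio and runs post-loading initialization.
; PlayAudio compares the index in a sequence of branches and starts the audio component of the matching Sport, Daojishou, Huanhu or Shenli reference.
; AfterLoadingInit casts the first player controller to set main UMG visibility and initialize the camera, then raises the CanStartPlayerTick flag.
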(event EventPlayAudio
  (params (audio_idx :type Integer))
  (Utilities|FlowControl|Sequence
    (:then_0
      (if (== audio_idx 0)
        (Audio|Components|Audio|Play (Variables|/Script/Engine.AmbientSound|GetAudioComponent (Variables|Default|Getsport)) 0.0)))
    (:then_1
      (if (== audio_idx 1)
        (Audio|Components|Audio|Play (Variables|/Script/Engine.AmbientSound|GetAudioComponent (Variables|Default|Getdaojishou)) 0.0)))
    (:then_2
      (if (== audio_idx 2)
        (Audio|Components|Audio|Play (Variables|/Script/Engine.AmbientSound|GetAudioComponent (Variables|Default|Gethuanhu)) 0.0)))
    (:then_3
      (if (== audio_idx 3)
        (Audio|Components|Audio|Play (Variables|/Script/Engine.AmbientSound|GetAudioComponent (Variables|Default|Getshenli)) 0.0)))))

(fn AfterLoadingInit
  (Utilities|FlowControl|Sequence
    (:then_0
      (bind _asbp_xiwbund_player_controller (Utilities|Casting|CastTo (Game|GetPlayerController 0)))
      (CallFunction|SetMainUMGVisibility _asbp_xiwbund_player_controller)
      (CallFunction|InitCamera _asbp_xiwbund_player_controller))
    (:then_1
      (Variables|Default|Setcan_start_player_tick true))))