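; Player controller for the Bund experience, which spans past, present and future levels plus a boat minigame.
; Tick sets the camera rig rail position from the game instance's CurTime, while InitValue sets timing thresholds for level and boat-game transitions.
; Events open loading levels, build per-era UI, crossfade loading widgets, drive cloud thickness through a material parameter collection and run boat-game stages.
; Keys call trigger handlers, and a Nuitrack actor is respawned if missing.
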(event EventBeginPlay
  (CallFunction|InitValue))

(event EventBPStartBoatGame
  (bind _asxiwbund_game_instance (Utilities|Casting|CastTo (Game|GetGameInstance)))
  (bind _asbp_boat (Utilities|Casting|CastTo (Variables|Default|Getboat_pawn _asxiwbund_game_instance)))
  (CallFunction|ChangeMaterial _asbp_boat (Variables|Default|Getselect_role_idx))
  (Pawn|Possess (Game|GetPlayerController 0) _asbp_boat)
  (CallFunction|CreateBoatPlay (Variables|Default|GetWBP_main_widget)))

(event EventCheckNuitrackActorExit
  (CallFunction|BPCheckNuiTrackExit))

(event EventDeleteNuitrackActorPointer
  (Variables|Default|Setnuitrack_actor_ins 0))

(event EventGradualyChangeUMG
  (params (value :type Float%20%28single-precision%29))
  (Widget|SetRenderOpacity (Variables|Default|GetLoadingUMG) value)
  (Widget|SetRenderOpacity (Variables|Default|GetWBP_main_widget) (- 1.0 value)))

(event EventShowLoadingUMG
  (params (CurMapID :type Byte :default 0))
  (bind _returnvalue (UserInterface|CreateWidget "/Game/UMG/BP_LoadingUW.BP_LoadingUW_C"))
  (Default|InitLoadingIdx _returnvalue CurMapID)
  (UserInterface|Viewport|AddtoViewport _returnvalue 1)
  (bind _output_get (Variables|Default|SetLoadingUMG _returnvalue))
  (Widget|SetRenderOpacity _output_get 0.0))

(event EventBPStartCasting
  (CallFunction|CreateBoatCasting (Variables|Default|GetWBP_main_widget))
  (bind _asxiwbund_game_instance (Utilities|Casting|CastTo (Game|GetGameInstance)))
  (bind _returnvalue (Actor|GetActorOfClass 0))
  (CallFunction|SetPawnPos _returnvalue (Transformation|GetActorLocation (Variables|Default|Getcasting_actor _asxiwbund_game_instance)) (Transformation|GetActorRotation (Variables|Default|Getcasting_actor _asxiwbund_game_instance))))

(event EventBPBoatAwardsCeremony
  (CallFunction|CreateBoatFinish (Variables|Default|GetWBP_main_widget)))

(event EventBPCreateUMG
  (params (Eplayer_stay_map :type Byte :default 0))
  (bind _returnvalue (UserInterface|CreateWidget 0))
  (Widget|SetVisibility _returnvalue "Collapsed")
  (Variables|Default|SetWBP_main_widget _returnvalue)
  (UserInterface|Viewport|AddtoViewport _returnvalue 0)
  (switch Utilities|FlowControl|Switch|Switchon Eplayer_stay_map
    (:OldLD
      (CallFunction|CreateOldLevelUI (Variables|Default|GetWBP_main_widget)))
    (:NowLD
      (CallFunction|CreateModelLevelUI (Variables|Default|GetWBP_main_widget)))
    (:FutureLD
      (CallFunction|CreateCyberpunkUI (Variables|Default|GetWBP_main_widget)))))

(event EventMoveBoat
  (params (bstart :type Boolean))
  (bind _asxiwbund_game_instance (Utilities|Casting|CastTo (Game|GetGameInstance)))
  (bind _asbp_boat (Utilities|Casting|CastTo (Variables|Default|Getboat_pawn _asxiwbund_game_instance)))
  (CallFunction|StartStopBoat _asbp_boat bstart))

(event EventBPChangeLevel
  (params (Eplayer_stay_map :type Byte :default 0))
  ;[1 1 1] change level
  (bind _asxiwbund_game_instance (Utilities|Casting|CastTo (Game|GetGameInstance)))
  (Variables|Default|Setcan_start_player_tick _asxiwbund_game_instance false)
  (switch Utilities|FlowControl|Switch|Switchon Eplayer_stay_map
    (:OldLD
      (Game|OpenLevel(byObjectReference) "/Game/LEVELS/BUND_HISTORYLOADING_LD.BUND_HISTORYLOADING_LD"))
    (:NowLD
      (Game|OpenLevel(byObjectReference) "/Game/LEVELS/BUND_MORDENLOADING_LD.BUND_MORDENLOADING_LD"))
    (:FutureLD
      (Game|OpenLevel(byObjectReference) "/Game/LEVELS/BUND_CYBERLOADING_LD.BUND_CYBERLOADING_LD"))))

(event EventQGame
  (Game|QuitGame 0 "Quit" false))

(event EventTick
  (params (delta_time :type Float%20%28single-precision%29))
  (bind _asxiwbund_game_instance (Utilities|Casting|CastTo (Game|GetGameInstance)))
  (bind _asbp_xiwbund_game_instance (Utilities|Casting|CastTo (Game|GetGameInstance)))
  (Variables|/Script/CinematicCamera.CameraRig_Rail|SetCurrentPositionOnRail (Variables|Default|Getcamera_rig_rail_ins _asbp_xiwbund_game_instance) (Variables|Default|Getcur_time _asxiwbund_game_instance)))

(event EventSetCloudParameterValue
  (params (value :type Float%20%28single-precision%29))
  (Rendering|Material|SetScalarParameterValue "/Game/ARTWORKS/NeoChen/MATERIALS/UI/MPC_UI_01.MPC_UI_01" "云厚度" (/ value (Variables|Default|Getshow_change_level_cloud_time)) :!class /Script/Engine.KismetMaterialLibrary))

(event Input|KeyboardEvents|Right
  (params (Key :type Key%20Structure :default "None"))
  (:Pressed
    (CallFunction|OnTriggerRightPressed))
  (:Released
    (CallFunction|OnTriggerRightUpReleased)))

(event Input|KeyboardEvents|Left
  (params (Key :type Key%20Structure :default "None"))
  (:Pressed
    (CallFunction|OnTriggerLeftPressed))
  (:Released
    (CallFunction|OnTriggerLeftReleased)))

(event Input|KeyboardEvents|O
  (params (Key :type Key%20Structure :default "None"))
  (:Pressed
    (CallFunction|OnTriggerLeftUpPressed)))

(event Input|KeyboardEvents|P
  (params (Key :type Key%20Structure :default "None"))
  (:Pressed
    (CallFunction|OnTriggerRightUpPressed)))

(fn ConstructionScript)

(fn InitValue
  (Utilities|FlowControl|Sequence
    (:then_0
      (Utilities|FlowControl|Sequence
        (:then_0
          (Variables|Default|Setrotate_speed 0.5))
        (:then_1
          (Variables|Default|Setmax_rotate_angle 5e+01))
        (:then_2
          (Variables|Default|Setrig_rail_speed 0.005))
        (:then_3
          (bind _output_get (Variables|Default|Setshow_change_level_cloud_time 2.0))
          (Variables|Default|Setchange_level_cloud_value_timer _output_get))))
    (:then_1
      (Utilities|FlowControl|Sequence
        (:then_0
          (Variables|Default|Setcan_enter_old_level_time 0.03))
        (:then_1
          (Variables|Default|Setauto_enter_old_level_time 0.05))
        (:then_2
          (Variables|Default|Setexit_old_level_time 0.17))))
    (:then_2
      (Utilities|FlowControl|Sequence
        (:then_0
          (Variables|Default|Setcan_enter_future_level_time 0.7))
        (:then_1
          (Variables|Default|Setauto_enter_future_level_time 0.836))
        (:then_2
          (Variables|Default|Setauto_enter_boat_game 0.95))
        (:then_3
          (Variables|Default|Setexit_future_level_time 0.99))))))

(fn SetMainUMGVisibility
  (Widget|SetVisibility (Variables|Default|GetWBP_main_widget) "SelfHitTestInvisible"))

(fn BPCheckNuiTrackExit
  (Utilities|IsValid (Variables|Default|Getnuitrack_actor_ins)
    (:Is%20Not%20Valid
      (bind _returnvalue (Game|SpawnActorfromClass 0 (Math|Transform|MakeTransform "0, 0, 0") "Undefined" self 0))
      (Variables|Default|Setnuitrack_actor_ins _returnvalue))))