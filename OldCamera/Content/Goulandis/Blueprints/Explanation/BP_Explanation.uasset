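; BP_Explanation runs a narrated story intro, showing timed image and text slides in a UW_Explanation widget over a cine camera view tagged ReadBook.
; BeginPlay creates the widget, shows the cursor, finds the tagged sequence player, switches view and calls SpeekStory.
; Each SpeekStory call waits, optionally plays the sequence by tag, and advances one ExplanationConfig entry.
; After the last, it removes the widget and hides the cursor.
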(event Custom|SpeekStory
  (bind _explanationconfig (Variables|Default|GetExplanationConfig))
  (Utilities|IsValid (Variables|Default|GetUW_Explanation)
    (:Is%20Valid
      (if (< (Variables|Default|GetIndex) (Utilities|Array|Length (Variables|Default|GetExplanationConfig)))
        (Utilities|FlowControl|Delay (.interval (Utilities|Array|Get(acopy) _explanationconfig (Variables|Default|GetIndex))))
        (switch string (.tag (Utilities|Array|Get(acopy) _explanationconfig (Variables|Default|GetIndex)))
          (:Default
            _)
          (:PhotoWall
            (Sequencer|Player|Play (Variables|/Game/Goulandis/GamePlay/OCPlayerController.OCPlayerController_C|GetCurrentLevelSeqPlayer (CallFunction|GetOCPlayerController)) :!class /Script/MovieScene.MovieSceneSequencePlayer :!label _label))
          (:ReadBook
            (goto _label)))
        (Default|SetContent (Variables|Default|GetUW_Explanation) (.image (Utilities|Array|Get(acopy) _explanationconfig (Variables|Default|GetIndex))) (.text (Utilities|Array|Get(acopy) _explanationconfig (Variables|Default|GetIndex))))
        (bind _result (Math|Integer|IncrementInt (Variables|Default|GetIndex))
          (:%20%20
            (Variables|Default|SetIndex _result)))
        (else
          (Utilities|FlowControl|Delay (.interval (Utilities|Array|Get(acopy) _explanationconfig (Utilities|Array|LastIndex _explanationconfig))))
          (Widget|RemovefromParent (Variables|Default|GetUW_Explanation))
          (Variables|/Script/Engine.PlayerController|SetbShowMouseCursor (CallFunction|GetOCPlayerController) false))))))

(event EventBeginPlay
  (bind _ocplayercontroller (CallFunction|GetOCPlayerController))
  (CallFunction|CreateUI)
  (Variables|/Script/Engine.PlayerController|SetbShowMouseCursor (CallFunction|GetOCPlayerController) true)
  (Utilities|FlowControl|Sequence
    (:then_0
      (Default|FindLevelSeqPlayerwithTag _ocplayercontroller "ReadBook"))
    (:then_1
      (bind _outactors (Actor|GetAllActorsOfClasswithTag "/Script/CinematicCamera.CineCameraActor" "ReadBook"))
      (if (== (Utilities|Array|Length _outactors) 1)
        (Game|Player|SetViewTargetwithBlend _ocplayercontroller (Utilities|Array|Get(acopy) _outactors) 0.0 "VTBlend_Linear" 0.0 false)))
    (:then_2
      (CallFunction|SpeekStory))))

(event Collision|EventActorBeginOverlap
  (params (OtherActor :type Actor%20Object%20Reference)))

(event EventTick
  (params (DeltaSeconds :type Float%20%28single-precision%29)))

(fn ConstructionScript)

(fn CreateUI
  (bind _returnvalue (UserInterface|CreateWidget "/Game/Goulandis/Blueprints/Explanation/UW_Explanation.UW_Explanation_C" (CallFunction|GetOCPlayerController)))
  (bind _output_get (Variables|Default|SetUW_Explanation _returnvalue))
  (UserInterface|Viewport|AddtoViewport _output_get 0)
  (Variables|/Game/Goulandis/Blueprints/Explanation/UW_Explanation.UW_Explanation_C|SetBP_Explanation _output_get self))