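; InteractiveCameraBody is the body of an interactive camera, with two box sockets that parts snap onto.
; Each tick, a box overlapping exactly one InteractiveCameraPart casts it to that socket's class: Part1 for Box1, Part2 for Box2.
; A match is deselected, cleared from InteractiveCameraPawn and moved to the box location plus AttachOffset, without true attachment.
; A DoOnce per socket limits this to once, resetting when the overlap count differs from one.
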(event EventTick
  (params (DeltaSeconds :type Float%20%28single-precision%29))
  (bind _box1 (Variables|Default|GetBox1))
  (bind _box2 (Variables|Default|GetBox2))
  (bind _attachoffset (Variables|Default|GetAttachOffset))
  (bind _box1_2 (Variables|Default|GetBox1))
  (bind _attachoffset_2 (Variables|Default|GetAttachOffset))
  (bind _box2_2 (Variables|Default|GetBox2))
  (bind _returnvalue (Transformation|GetWorldLocation _box1_2))
  (bind _overlappingactors (Collision|GetOverlappingActors _box2 "/Game/Goulandis/Blueprints/InteractiveCamera/InteractiveCameraPart.InteractiveCameraPart_C" :!class /Script/Engine.PrimitiveComponent))
  (bind _returnvalue_2 (Transformation|GetWorldLocation _box2_2))
  (bind _overlappingactors_2 (Collision|GetOverlappingActors _box1 "/Game/Goulandis/Blueprints/InteractiveCamera/InteractiveCameraPart.InteractiveCameraPart_C" :!class /Script/Engine.PrimitiveComponent))
  (Utilities|FlowControl|Sequence
    (:then_0
      (if (== (Utilities|Array|Length _overlappingactors_2) 1)
        (bind _asinteractive_camera_part_1 (Utilities|Casting|CastToInteractiveCameraPart1 (Utilities|Array|Get(acopy) _overlappingactors_2)))
        (Utilities|FlowControl|DoOnce false :!label _label
          (:Completed
            (Variables|/Game/Goulandis/Blueprints/InteractiveCamera/InteractiveCameraPart.InteractiveCameraPart_C|SetIsSelected _asinteractive_camera_part_1 false)
            (Variables|/Game/Goulandis/Blueprints/InteractiveCamera/IntercativeCameraPawn.IntercativeCameraPawn_C|SetCurrentSelectedActor (Variables|Default|GetInteractiveCameraPawn) 0)
            (Transformation|SetActorLocation _asinteractive_camera_part_1 (Math|Vector|MakeVector (+ (.x _returnvalue) _attachoffset_2) (+ (.y _returnvalue) _attachoffset_2) (+ (.z _returnvalue) _attachoffset_2)) false false)))
        (else
          (goto _label Reset))))
    (:then_1
      (if (== (Utilities|Array|Length _overlappingactors) 1)
        (bind _asinteractive_camera_part_2 (Utilities|Casting|CastToInteractiveCameraPart2 (Utilities|Array|Get(acopy) _overlappingactors)))
        (Utilities|FlowControl|DoOnce false :!label _label_2
          (:Completed
            (Variables|/Game/Goulandis/Blueprints/InteractiveCamera/InteractiveCameraPart.InteractiveCameraPart_C|SetIsSelected _asinteractive_camera_part_2 false)
            (Variables|/Game/Goulandis/Blueprints/InteractiveCamera/IntercativeCameraPawn.IntercativeCameraPawn_C|SetCurrentSelectedActor (Variables|Default|GetInteractiveCameraPawn) 0)
            (Transformation|SetActorLocation _asinteractive_camera_part_2 (Math|Vector|MakeVector (+ (.x _returnvalue_2) _attachoffset) (+ (.y _returnvalue_2) _attachoffset) (+ (.z _returnvalue_2) _attachoffset)) false false)))
        (else
          (goto _label_2 Reset))))))

(fn ConstructionScript)