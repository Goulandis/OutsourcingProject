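; InteractiveCameraPart is an actor that follows the mouse cursor through the world while it is selected.
; Each tick, while IsSelected is true, it deprojects player 0's mouse position and runs a sphere trace along that direction over TraceLen on the Visibility channel.
; It then moves itself to the hit location with a small fixed offset in X and Y, without checking whether the trace hit anything.
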(event EventTick
  (params (DeltaSeconds :type Float%20%28single-precision%29))
  (bind _returnvalue (Game|GetPlayerController 0))
  (bind (_worldlocation _worlddirection) (Game|Player|ConvertMouseLocationToWorldSpace _returnvalue))
  (if (Variables|Default|GetIsSelected)
    (bind _outhit (Collision|SphereTraceByChannel _worldlocation (+ _worldlocation (* _worlddirection (Variables|Default|GetTraceLen))) 5.0 "TraceTypeQuery1" false 0 "None"))
    (Transformation|SetActorLocation (Math|Vector|MakeVector (- (.X (Math|Vector|BreakVector (.Location (Collision|BreakHitResult _outhit)))) 2e+01) (- (.Y (Math|Vector|BreakVector (.Location (Collision|BreakHitResult _outhit)))) 2e+01) (.Z (Math|Vector|BreakVector (.Location (Collision|BreakHitResult _outhit))))) false false)))

(fn ConstructionScript)