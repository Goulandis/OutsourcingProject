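; InteractiveCameraPawn2 is a pawn for viewing and clicking parts of an interactive camera with the mouse.
; Dragging with the left button held turns the control rotation in yaw and pitch, scaled by ControllerScale.
; A left press line-traces from the cursor, snaps any hit InteractiveCameraPart to its TargetTrans and adds a new UW_InteractiveCamera widget.
; Selection-toggle and rotation-offset logic remains in the graph but is disconnected.
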(event EventBeginPlay)

(event Collision|EventActorBeginOverlap
  (params (OtherActor :type Actor%20Object%20Reference)))

(event EventTick
  (params (DeltaSeconds :type Float%20%28single-precision%29)))

(event Input|MouseEvents|MouseX
  (params (AxisValue :type Float%20%28single-precision%29))
  (bind _returnvalue (Game|GetPlayerController 0))
  (bind _returnvalue_2 (Pawn|GetControlRotation _returnvalue :!class /Script/Engine.Controller))
  (if (Game|Player|IsInputKeyDown _returnvalue "LeftMouseButton")
    (Pawn|SetControlRotation (Game|GetPlayerController 0) (Math|Rotator|MakeRotator (.roll _returnvalue_2) (.pitch _returnvalue_2) (+ (.yaw _returnvalue_2) (* AxisValue (Variables|Default|GetControllerScale)))))))

(event Input|MouseEvents|MouseY
  (params (AxisValue :type Float%20%28single-precision%29))
  (bind _returnvalue (Game|GetPlayerController 0))
  (bind _returnvalue_2 (Pawn|GetControlRotation _returnvalue :!class /Script/Engine.Controller))
  (if (Game|Player|IsInputKeyDown _returnvalue "LeftMouseButton")
    (Pawn|SetControlRotation (Game|GetPlayerController 0) (Math|Rotator|MakeRotator (.roll _returnvalue_2) (+ (.pitch _returnvalue_2) (* AxisValue (Variables|Default|GetControllerScale))) (.yaw _returnvalue_2)))))

(event Input|MouseEvents|LeftMouseButton
  (params (Key :type Key%20Structure :default "None"))
  (bind _returnvalue (Game|GetPlayerController 0))
  (bind (_worldlocation _worlddirection) (Game|Player|ConvertMouseLocationToWorldSpace _returnvalue))
  (:Pressed
    (bind _outhit (Collision|LineTraceByChannel _worldlocation (+ _worldlocation (* _worlddirection (Variables|Default|GetLineTraceLen))) "TraceTypeQuery1" false 0 "None"))
    (bind _asinteractive_camera_part (Utilities|Casting|CastToInteractiveCameraPart (.HitActor (Collision|BreakHitResult _outhit))))
    (Transformation|SetActorTransform _asinteractive_camera_part (Variables|/Game/Goulandis/Blueprints/InteractiveCamera/InteractiveCameraPart.InteractiveCameraPart_C|GetTargetTrans _asinteractive_camera_part))
    (bind _returnvalue_2 (UserInterface|CreateWidget "/Game/Goulandis/Blueprints/InteractiveCamera/UW_InteractiveCamera.UW_InteractiveCamera_C" (CallFunction|GetOCPlayerController)))
    (UserInterface|Viewport|AddtoViewport _returnvalue_2 0)))

(fn ConstructionScript)