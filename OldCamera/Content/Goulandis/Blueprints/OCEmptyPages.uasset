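; OCEmptyPages is a book actor child Blueprint that can be picked up and read, with scale applied at construction.
; PickUpBook disables physics and collision, then plays cover and page-folding animations.
; Depending on the spawn state, it first hides the fake pages or rebuilds the book by spawning, adding and stacking page actors.
; ReadBook restores visibility, picks up the book and calls TurnToPage, which defers to the parent.
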(event EventBeginPlay
  (|CallParentFunction))

(event Collision|EventActorBeginOverlap
  (params (OtherActor :type Actor%20Object%20Reference)))

(event EventTick
  (params (DeltaSeconds :type Float%20%28single-precision%29)))

(fn ConstructionScript
  (|CallParentFunction)
  (Transformation|SetActorScale3D (Variables|Default|GetSacle)))

(fn PickUpBook
  (params (SceneComponent :type Scene%20Component%20Object%20Reference))
  (if (Variables|Default|GetCanPickUpBook?)
    (Variables|Default|SetBookPickedUp? true)
    (switch Utilities|FlowControl|Switch|SwitchonE_Spawn (Variables|Default|GetPagesSpawnState)
      (:NewEnumerator0
        _)
      (:NewEnumerator1
        (Rendering|SetVisibility (Variables|Default|GetPagesFake) false false))
      (:NewEnumerator4
        (Utilities|Array|Clear (Variables|Default|GetPageArray))
        (Utilities|Array|Resize (Variables|Default|GetPageArray) (Variables|Default|GetBookPageLimit))
        (Variables|Default|SetTotalAmountOfPages 0)
        (if (> (Utilities|Array|Length (Variables|Default|GetPages)) 0)
          (for _array_element (Variables|Default|GetPages)
            (if (Utilities|IsValidClass _array_element)
              (bind _returnvalue (Game|SpawnActorfromClass _array_element (Math|Transform|MakeTransform "0, 0, 0" "0, 0, 0" "1.000000,1.000000,1.000000") "AlwaysSpawn" 0 0))
              (CallFunction|AddPagetoBook "NewEnumerator0" _returnvalue false)))
          (CallFunction|StackPageOrder 0 false)
          (Rendering|SetVisibility (Variables|Default|GetPagesFake) false false)
          (else
            (return)))))
    (Physics|SetSimulatePhysics (Variables|Default|GetBookCollision) false)
    (Collision|SetCollisionEnabled (Variables|Default|GetBookCollision) "NoCollision")
    (Components|Animation|SetAnimation (Variables|Default|GetCoverSkeletonMesh) "/Game/Goulandis/InteractiveBook/Mesh/Animation/Anim_Cover_Play.Anim_Cover_Play")
    (for _array_element_2 (Variables|Default|GetPageArray)
      (Utilities|IsValid _array_element_2
        (:Is%20Valid
          (Components|Animation|SetAnimation (Variables|/Game/Goulandis/InteractiveBook/Blueprints/BP_MasterPage.BP_MasterPage_C|GetPageSkeletonMesh _array_element_2) "/Game/Goulandis/InteractiveBook/Mesh/Animation/Anim_Page_Folding.Anim_Page_Folding"))))
    (CallFunction|AddWidgetDebug)
    (return)
    (else
      (return))))

(fn ReadBook
  (CallFunction|SetBookVisibility true) ; Toggles visibility back on for drop
  (CallFunction|PickUpBook)
  (CallFunction|TurntoPage "NewEnumerator0" 5))

(fn TurntoPage
  (params (GoTo :type E_GoToSelection%20Enum :default "NewEnumerator0") (SpesificIndex :type Integer))
  (|CallParentFunction GoTo SpesificIndex))