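; OCFunLib is a function library of shared helpers for fetching the game's OC framework objects and writing debug messages.
; GetOCPlayerController casts player 0's controller to OCPlayerController, and GetOCHUD uses it to return the OCHUD, each logging failed casts.
; DLog splits a colon-delimited key into a bracketed Debug prefix and prints the message to the log only, not on screen.
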(fn GetOCPlayerController
  (bind ___worldcontext (LocalVariables|Get__WorldContext))
  (bind _asocplayer_controller (Utilities|Casting|CastToOCPlayerController (Game|GetPlayerController ___worldcontext))
    (:then
      (return _asocplayer_controller))
    (:CastFailed
      (CallFunction|DLog "Error:GetOCPlayerController" "Failed to cast PlayerController to OcPlayerController" ___worldcontext))))

(fn DLog
  (params (Key :type String) (Log :type String))
  (bind (_lefts _rights) (Utilities|String|Split Key ":"))
  (Development|PrintString (LocalVariables|Get__WorldContext) (Utilities|String|Append "[Debug" _lefts ":" _rights "] " Log) false))

(fn GetOCHUD
  (bind ___worldcontext (LocalVariables|Get__WorldContext))
  (bind _ocplayercontroller (CallFunction|GetOCPlayerController ___worldcontext))
  (Utilities|IsValid _ocplayercontroller
    (:Is%20Valid
      (bind _asochud (Utilities|Casting|CastToOCHUD (HUD|GetHUD _ocplayercontroller))
        (:then
          (return _asochud))
        (:CastFailed
          (CallFunction|DLog "Error:GetOCHUD" "Failed to cast HUD to OCHUD" ___worldcontext))))))