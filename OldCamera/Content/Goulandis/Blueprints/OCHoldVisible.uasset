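; OCHoldVisible is a hold-to-interact trigger actor that, by TriggerType, reads a book, switches level, possesses a camera pawn or starts a product explanation.
; Init finds the book or spawns an interact manager, and the component activates after ShowTime, with an optional Timeline height animation.
; Component events show progress on TextRender, and completion runs the type's action.
; The construction script applies input keys and can swap text for a light.
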(event OnInteractionStarted(InteractionComponent_HoldVisible)
  (CallFunction|SetText "Interaction started" "(R=1.000000,G=1.000000,B=1.000000,A=1.000000)"))

(event OnInteractionCompleted(InteractionComponent_HoldVisible)
  (bind _ocplayercontroller (CallFunction|GetOCPlayerController))
  (bind _ocplayercontroller_2 (CallFunction|GetOCPlayerController))
  (bind _book (Variables|Default|GetBook))
  (switch string (Variables|Default|GetTriggerType)
    (:Book
      (Utilities|IsValid _book
        (:Is%20Valid
          (Default|ReadBook _book)
          (Utilities|IsValid (Variables|Default|GetBP_Explanation)
            (:Is%20Valid
              (Utilities|IsValid (Variables|/Game/Goulandis/Blueprints/Explanation/BP_Explanation.BP_Explanation_C|GetLevelSquence (Variables|Default|GetBP_Explanation))
                (:Is%20Valid
                  (Sequencer|Player|Play (Variables|/Script/LevelSequence.LevelSequenceActor|GetSequencePlayer (Variables|/Game/Goulandis/Blueprints/Explanation/BP_Explanation.BP_Explanation_C|GetLevelSquence (Variables|Default|GetBP_Explanation))) :!class /Script/MovieScene.MovieSceneSequencePlayer))))))))
    (:InFactory
      (Default|Fade (CallFunction|GetOCHUD) false)
      (Utilities|FlowControl|Delay 0.5)
      (Variables|/Game/Goulandis/GamePlay/OCPlayerController.OCPlayerController_C|SetLevelName (CallFunction|GetOCPlayerController) "xiangjichangchejian"))
    (:Camera
      (bind _returnvalue (Actor|GetActorOfClass "/Game/Goulandis/Blueprints/InteractiveCamera/InteractiveCameraPawn2.InteractiveCameraPawn2_C"))
      (Utilities|IsValid _returnvalue
        (:Is%20Valid
          (Utilities|IsValid (Variables|Default|GetCharactor)
            (:Is%20Valid
              (Rendering|SetActorHiddenInGame (Variables|Default|GetCharactor) true)
              (Input|DisableInput (Variables|Default|GetCharactor) _ocplayercontroller_2)
              (Game|Player|SetViewTargetwithBlend _ocplayercontroller_2 _returnvalue 1.0 "VTBlend_Linear" 0.0 false)
              (Utilities|FlowControl|Delay 1.0)
              (Pawn|Possess _ocplayercontroller_2 _returnvalue)
              (Input|EnableInput _returnvalue _ocplayercontroller_2)
              (Variables|/Script/Engine.PlayerController|SetbShowMouseCursor _ocplayercontroller_2 true))))))
    (:Explanation
      (Utilities|IsValid (Variables|Default|GetCharactor)
        (:Is%20Valid
          (Rendering|SetActorHiddenInGame (Variables|Default|GetCharactor) true)
          (Game|Player|SetViewTargetwithBlend _ocplayercontroller (Variables|Default|GetCamera) 0.5 "VTBlend_Linear" 0.0 false)
          (Variables|/Script/Engine.PlayerController|SetbShowMouseCursor _ocplayercontroller true)
          (bind _returnvalue_2 (UserInterface|CreateWidget "/Game/Goulandis/Blueprints/Explanation/UW_ProductIntroduction.UW_ProductIntroduction_C" _ocplayercontroller))
          (UserInterface|Viewport|AddtoViewport _returnvalue_2 0)
          (Variables|/Game/Goulandis/Blueprints/Explanation/UW_ProductIntroduction.UW_ProductIntroduction_C|SetCharactor _returnvalue_2 (Variables|Default|GetCharactor))
          (Variables|/Game/Goulandis/Blueprints/Explanation/UW_ProductIntroduction.UW_ProductIntroduction_C|SetBP_Explanation _returnvalue_2 (Variables|Default|GetBP_Explanation))
          (Utilities|IsValid (Variables|Default|GetBP_Explanation)
            (:Is%20Valid
              (Variables|/Game/Goulandis/Blueprints/Explanation/BP_Explanation.BP_Explanation_C|SetIndex (Variables|Default|GetBP_Explanation) (Variables|Default|GetStartIndex))
              (Default|SpeekStory (Variables|Default|GetBP_Explanation)))))))))

(event OnInteractionUpdate(InteractionComponent_HoldVisible)
  (params (Value :type Float%20%28double-precision%29) (Repetitions :type Integer))
  (|IsRepeatEvent
    (:then
      (CallFunction|SetText (Utilities|Text|ToText(String) (Utilities|String|Append "Repetitions: " (Utilities|String|ToString(Integer) Repetitions))) "(R=1.000000,G=1.000000,B=1.000000,A=1.000000)"))
    (:else
      (CallFunction|SetText (Utilities|Text|ToText(String) (Utilities|String|Append "Interaction Progress: " (Utilities|String|ToString(Float) Value))) "(R=1.000000,G=1.000000,B=1.000000,A=1.000000)"))))

(event OnInteractionCancelled(InteractionComponent_HoldVisible)
  (CallFunction|SetText "Interaction Cancelled" "(R=1.000000,G=0.000000,B=0.000000,A=1.000000)")
  (Utilities|FlowControl|Delay 3.0)
  (CallFunction|SetText "Ready to interact" "(R=1.000000,G=1.000000,B=1.000000,A=1.000000)"))

(event Custom|Init
  (Variables|/Game/Goulandis/InteractionEssentials/Blueprints/Components/InteractionComponent.InteractionComponent_C|SetbIsActivated (Variables|Default|GetInteractionComponent_HoldVisible) false)
  (switch string (Variables|Default|GetTriggerType)
    (:Book
      (Utilities|FlowControl|Delay 2.0)
      (bind _returnvalue (Actor|GetActorOfClass "/Game/Goulandis/Blueprints/Book/OCEmptyPages.OCEmptyPages_C"))
      (Utilities|IsValid _returnvalue
        (:Is%20Valid
          (Variables|Default|SetBook _returnvalue))
        (:Is%20Not%20Valid
          (CallFunction|DLog "Error:Init" "There no OCEmptyPage actor in the level"))))
    (:Camera
      (bind _returnvalue_2 (Game|SpawnActorfromClass "/Game/Goulandis/InteractionEssentials/Blueprints/Actors/BP_InteractManager.BP_InteractManager_C" (Math|Transform|MakeTransform "0, 0, 0" "0, 0, 0" "1.000000,1.000000,1.000000") "AdjustIfPossibleButAlwaysSpawn" (Game|Player|GetPlayerPawn 0) 0 :!label _label))
      (Variables|/Game/Goulandis/InteractionEssentials/Blueprints/Components/InteractionComponent.InteractionComponent_C|SetInteractManager (Variables|Default|GetInteractionComponent_HoldVisible) _returnvalue_2))
    (:Explanation
      (goto _label))))

(event EventBeginPlay
  (bind _returnvalue (Transformation|GetActorLocation))
  (CallFunction|Init)
  (Utilities|FlowControl|Delay (Variables|Default|GetShowTime))
  (Variables|/Game/Goulandis/InteractionEssentials/Blueprints/Components/InteractionComponent.InteractionComponent_C|SetbIsActivated (Variables|Default|GetInteractionComponent_HoldVisible) true)
  (if (Variables|Default|GetMove)
    (bind _test (Timeline|Timeline_0 PlayFromStart)
      (:Update
        (Transformation|SetActorLocation (Math|Vector|MakeVector (.x _returnvalue) (.y _returnvalue) (Math|Float|MapRangeClamped _test 0.0 1.0 -4e+01 2.5e+02)) false false)))))

(event EventTick
  (params (DeltaSeconds :type Float%20%28single-precision%29)))

(fn ConstructionScript
  (bind _interactioncomponent_holdvisible (Variables|Default|GetInteractionComponent_HoldVisible))
  (Variables|/Game/Goulandis/InteractionEssentials/Blueprints/Components/InteractionComponent.InteractionComponent_C|SetInputKey_PC _interactioncomponent_holdvisible (Variables|Default|GetInputKey_PC))
  (Variables|/Game/Goulandis/InteractionEssentials/Blueprints/Components/InteractionComponent.InteractionComponent_C|SetInputKey_Gamepad _interactioncomponent_holdvisible (Variables|Default|GetInputKey_Gamepad))
  (if (Variables|Default|GetUseLight)
    (Rendering|SetVisibility (Variables|Default|GetPointLight) true false)
    (Rendering|SetVisibility (Variables|Default|GetTextRender) false false)))

(fn SetText
  (params (Value :type Text) (Color :type Linear%20Color%20Structure))
  (bind _textrender (Variables|Default|GetTextRender))
  (Rendering|Components|TextRender|SetText _textrender (Utilities|Text|MakeLiteralText Value))
  (Rendering|Components|TextRender|SetTextRenderColor _textrender (Math|Conversions|ToColor(LinearColor) Color)))