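; Pedestrian actor that moves a skeletal mesh along its own spline, starting at BeginPlay.
; The Action event plays a timeline whose Alpha maps to distance along the spline, setting the mesh's world location and rotation with a -90 yaw offset.
; The timeline's play rate is refreshed from the Rate variable on each update.
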(event Custom|Action
  (bind _spline (Variables|Default|GetSpline))
  (bind _alpha (Timeline|Timeline Play)
    (:Update
      (Transformation|SetWorldLocationAndRotation (Variables|Default|GetSkeletalMesh) (.location (Spline|GetTransformatDistanceAlongSpline _spline (Math|Float|Lerp 0.0 (Spline|GetSplineLength _spline) _alpha) "World" false)) (Math|Rotator|MakeRotator (.roll (.rotation (Spline|GetTransformatDistanceAlongSpline _spline (Math|Float|Lerp 0.0 (Spline|GetSplineLength _spline) _alpha) "World" false))) (.pitch (.rotation (Spline|GetTransformatDistanceAlongSpline _spline (Math|Float|Lerp 0.0 (Spline|GetSplineLength _spline) _alpha) "World" false))) (+ (.yaw (.rotation (Spline|GetTransformatDistanceAlongSpline _spline (Math|Float|Lerp 0.0 (Spline|GetSplineLength _spline) _alpha) "World" false))) -9e+01)) false false)
      (Components|Timeline|SetPlayRate (Variables|Default|GetTimeline) (Variables|Default|GetRate)))))

(event EventBeginPlay
  (CallFunction|Action))

(event Collision|EventActorBeginOverlap
  (params (OtherActor :type Actor%20Object%20Reference)))

(event EventTick
  (params (DeltaSeconds :type Float%20%28single-precision%29)))

(fn ConstructionScript)