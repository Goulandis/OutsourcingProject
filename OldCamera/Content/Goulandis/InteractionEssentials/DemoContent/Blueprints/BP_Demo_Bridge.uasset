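; Demo interaction actor for a bridge sequence that takes over the camera and character while the interaction runs.
; On start it disables input, blends the view to itself, poses the character mesh, loops camera shakes and animates the camera's rotation, FOV and position.
; After a delay it shrinks the interaction radius and slides BP_Demo_Bridge_Falling along X.
; Cancel or completion blends back, restores the radius and re-enables input.
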(event OnInteractionUpdate(InteractionComponent)
  (params (Value :type Float%20%28double-precision%29) (Repetitions :type Integer)))

(event OnInteractionStarted(InteractionComponent)
  (bind _output (CallFunction|FallingActor))
  (bind _camera (Variables|Default|GetCamera))
  (bind _returnvalue (Transformation|GetActorLocation _output))
  (|HandleBlendIn)
  (Variables|Default|SetIsActive true)
  (Utilities|FlowControl|Sequence
    (:then_0
      (Utilities|LoopCameraShake "/Game/Goulandis/InteractionEssentials/DemoContent/Blueprints/CS_Demo.CS_Demo_C" 0.25 0.5))
    (:then_1
      (Utilities|LoopCameraShake "/Game/Goulandis/InteractionEssentials/DemoContent/Blueprints/CS_Demo1.CS_Demo1_C" 0.8 0.75)
      (Utilities|FlowControl|Sequence
        (:then_0
          (bind _newtrack_0 (Timeline|Timeline_2 Play)
            (:Update
              (Transformation|SetRelativeRotation (Variables|Default|GetCamera) (Math|Rotator|Lerp(Rotator) "-55.000000,50.000000,-3.000000" "-20.000000,25.000000,0.000000" _newtrack_0 true) false false)
              (Camera|SetFieldOfView (Variables|Default|GetCamera) (Math|Float|Lerp 3e+01 6e+01 _newtrack_0)))))
        (:then_1
          (bind _newtrack_0_2 (Timeline|Timeline_3 Play)
            (:Update
              (Transformation|SetRelativeLocation _camera (Math|Vector|MakeVector (.x (Variables|/Script/Engine.SceneComponent|GetRelativeLocation _camera)) (Math|Float|Lerp 0.0 2e+01 _newtrack_0_2) (Math|Float|Lerp 0.0 -5e+01 _newtrack_0_2)) false false))))
        (:then_2
          (Utilities|FlowControl|Delay 1.0)
          (Variables|/Game/Goulandis/InteractionEssentials/Blueprints/Components/InteractionComponent.InteractionComponent_C|SetInteractionRadius (Variables|Default|GetInteractionComponent) 1e+01)
          (Components|Timeline|SetPlayRate (Variables|Default|GetMoveTimeline) 2.0)
          (bind _newtrack_0_3 (Timeline|MoveTimeline Play)
            (:Update
              (Transformation|SetActorLocation (CallFunction|FallingActor) (Math|Vector|MakeVector (Math|Float|Lerp 8.2e+03 7.13e+03 _newtrack_0_3) (.y _returnvalue) (.z _returnvalue)) false false))))))))

(event OnInteractionCompleted(InteractionComponent)
  (bind _output (CallFunction|FallingActor))
  (bind _returnvalue (Transformation|GetActorLocation _output))
  (Variables|Default|SetbComplete true)
  (|HandleBlendOut)
  (Variables|/Game/Goulandis/InteractionEssentials/Blueprints/Components/InteractionComponent.InteractionComponent_C|SetInteractionRadius (Variables|Default|GetInteractionComponent) (Variables|Default|GetCacheInteractionRadius))
  (Variables|Default|SetIsActive false)
  (bind _newtrack_0 (Timeline|MoveTimeline Stop)
    (:Update
      (Transformation|SetActorLocation (CallFunction|FallingActor) (Math|Vector|MakeVector (Math|Float|Lerp 8.2e+03 7.13e+03 _newtrack_0) (.y _returnvalue) (.z _returnvalue)) false false))))

(event OnInteractionCancelled(InteractionComponent)
  (bind _output (CallFunction|FallingActor))
  (bind _returnvalue (Transformation|GetActorLocation _output))
  (Variables|Default|SetbComplete false)
  (|HandleBlendOut)
  (Variables|/Game/Goulandis/InteractionEssentials/Blueprints/Components/InteractionComponent.InteractionComponent_C|SetInteractionRadius (Variables|Default|GetInteractionComponent) (Variables|Default|GetCacheInteractionRadius))
  (Variables|Default|SetIsActive false)
  (bind _newtrack_0 (Timeline|MoveTimeline Stop)
    (:Update
      (Transformation|SetActorLocation (CallFunction|FallingActor) (Math|Vector|MakeVector (Math|Float|Lerp 8.2e+03 7.13e+03 _newtrack_0) (.y _returnvalue) (.z _returnvalue)) false false))))

(event EventBeginPlay
  (Variables|Default|SetCacheInteractionRadius (Variables|/Game/Goulandis/InteractionEssentials/Blueprints/Components/InteractionComponent.InteractionComponent_C|GetInteractionRadius (Variables|Default|GetInteractionComponent))))

(fn ConstructionScript)

(fn GetCharAnimInstance
  (bind _asthird_person_anim_bp (Utilities|Casting|CastToThirdPerson_AnimBP (Components|SkeletalMesh|GetAnimInstance (Variables|/Script/Engine.Character|GetMesh (CallFunction|GetDemoCharacter)))))
  (return _asthird_person_anim_bp))

(fn InterpRelativeCameraY
  (params (Target :type Vector) (InterpSpeed :type Float%20%28double-precision%29))
  (bind _camera (Variables|Default|GetCamera))
  (bind _relativelocation (Variables|/Script/Engine.SceneComponent|GetRelativeLocation _camera))
  (Transformation|SetRelativeLocation _camera (Math|Vector|MakeVector (.x _relativelocation) (Math|Interpolation|FInterpTo (.y _relativelocation) (.Y (Math|Vector|BreakVector Target)) (Variables|Default|GetDeltaX) InterpSpeed) (.z _relativelocation)) false false)
  (return))

(fn FallingActor
  (bind _outactors (Actor|GetAllActorsOfClass "/Game/Goulandis/InteractionEssentials/DemoContent/Blueprints/BP_Demo_Bridge_Falling.BP_Demo_Bridge_Falling_C"))
  (return (Utilities|Array|Get(acopy) _outactors)))