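; Demo bridge that breaks when a character enters its box, leaving the player hanging in a RepeatEventInvisible interaction.
; Timelines tilt the bridge pieces and move the character mesh into the hang while the view blends to the bridge camera and looping shakes play.
; Completion restores the mesh and moves the character to NewCharLoc behind a camera fade.
; Cancellation drops the mesh with a camera drop and FOV widening, then triggers BP_Demo_Deadzone.
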(event OnInteractionCancelled(RepeatEventInvisible)
  (Variables|Default|SetbComplete false)
  (Utilities|FlowControl|Delay 0.0)
  (|HandleFall 1.2))

(event OnInteractionCompleted(RepeatEventInvisible)
  (Variables|Default|SetbComplete true)
  (|HandleBlendOut_2)
  (Variables|Default|SetIsActive false))

(event OnComponentBeginOverlap(Box)
  (params (OverlappedComponent :type Primitive%20Component%20Object%20Reference) (OtherActor :type Actor%20Object%20Reference) (OtherComp :type Primitive%20Component%20Object%20Reference) (OtherBodyIndex :type Integer) (bFromSweep :type Boolean) (SweepResult :type Hit%20Result%20Structure%20%28by%20ref%29))
  (Utilities|Casting|CastToCharacter OtherActor)
  (Variables|/Game/Goulandis/InteractionEssentials/DemoContent/DemoCharacter_3P/ThirdPersonCharacter.ThirdPersonCharacter_C|SetbIsRunning (CallFunction|GetDemoCharacter) false)
  (|FadeInBreak 3.0
    (:then
      (|HandleBlendIn_2)
      (bind _repeateventinvisible (Variables|Default|GetRepeatEventInvisible)
        (:then
          (Default|ActivateInteraction (CallFunction|GetInteractionManager _repeateventinvisible) false)
          (Variables|Default|SetIsActive true)
          (Utilities|LoopCamShake "/Game/Goulandis/InteractionEssentials/DemoContent/Blueprints/CS_Demo.CS_Demo_C" 0.8 0.5
            (:then_1
              (Utilities|LoopCamShake "/Game/Goulandis/InteractionEssentials/DemoContent/Blueprints/CS_Demo1.CS_Demo1_C" 1.2 0.75))))
        (:else)))))

(fn ConstructionScript)

(fn GetCharAnimInstance
  (bind _asthird_person_anim_bp (Utilities|Casting|CastToThirdPerson_AnimBP (Components|SkeletalMesh|GetAnimInstance (Variables|/Script/Engine.Character|GetMesh (CallFunction|GetDemoCharacter)))))
  (return _asthird_person_anim_bp))