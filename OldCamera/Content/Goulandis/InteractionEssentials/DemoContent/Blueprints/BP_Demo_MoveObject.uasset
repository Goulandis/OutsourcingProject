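; Interaction Essentials demo actor where the player moves an object: an InteractionComponent triggers a timeline that slides the Cube along local Y.
; On start it overrides the interaction radius, disables input, blends the view to itself, loops camera shakes and lerps the character mesh into a held pose at the SkeletalMesh.
; Completion or cancel stops the slide and restores radius, view, mesh transform and, after a delay, input, with timings depending on the outcome.
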(event OnInteractionUpdate(InteractionComponent)
  (params (Value :type Float%20%28double-precision%29) (Repetitions :type Integer))
  (bind (_returnvalue _returnvalue2) (|CollapseGraph_0_2 Value))
  (Transformation|SetWorldLocationAndRotation (Variables|/Script/Engine.Character|GetMesh (CallFunction|GetDemoCharacter)) _returnvalue _returnvalue2 false false))

(event OnInteractionStarted(InteractionComponent)
  (bind _cube (Variables|Default|GetCube))
  (bind _relativelocation (Variables|/Script/Engine.SceneComponent|GetRelativeLocation _cube))
  (|HandleBlendIn
    (:then
      (Variables|Default|SetIsActive true)
      (Utilities|FlowControl|Sequence
        (:then_0
          (Utilities|LoopCameraShake "/Game/Goulandis/InteractionEssentials/DemoContent/Blueprints/CS_Demo.CS_Demo_C" 0.25 0.5))
        (:then_1
          (Utilities|LoopCameraShake "/Game/Goulandis/InteractionEssentials/DemoContent/Blueprints/CS_Demo1.CS_Demo1_C" 1.5 0.75)
          (Variables|Default|SetTemp (Transformation|GetActorLocation (CallFunction|GetDemoCharacter)))
          (Variables|/Game/Goulandis/InteractionEssentials/Blueprints/Components/InteractionComponent.InteractionComponent_C|SetInteractionRadius (Variables|Default|GetInteractionComponent) 1e+01)
          (bind _newtrack_0 (Timeline|MoveTimeline Play)
            (:Update
              (Transformation|SetRelativeLocation _cube (Math|Vector|MakeVector (.x _relativelocation) (Math|Float|Lerp 0.0 (Math|Float|MakeLiteralFloat 2.2e+02) _newtrack_0) (.z _relativelocation)) false false))))))))

(event OnInteractionCompleted(InteractionComponent)
  (bind _cube (Variables|Default|GetCube))
  (bind _relativelocation (Variables|/Script/Engine.SceneComponent|GetRelativeLocation _cube))
  (Variables|Default|SetbComplete true)
  (|HandleBlendOut)
  (Variables|/Game/Goulandis/InteractionEssentials/Blueprints/Components/InteractionComponent.InteractionComponent_C|SetInteractionRadius (Variables|Default|GetInteractionComponent) (Variables|Default|GetCacheInteractionRadius))
  (Variables|Default|SetIsActive false)
  (bind _newtrack_0 (Timeline|MoveTimeline Stop)
    (:Update
      (Transformation|SetRelativeLocation _cube (Math|Vector|MakeVector (.x _relativelocation) (Math|Float|Lerp 0.0 (Math|Float|MakeLiteralFloat 2.2e+02) _newtrack_0) (.z _relativelocation)) false false))))

(event OnInteractionCancelled(InteractionComponent)
  (bind _cube (Variables|Default|GetCube))
  (bind _relativelocation (Variables|/Script/Engine.SceneComponent|GetRelativeLocation _cube))
  (Variables|Default|SetbComplete false)
  (|HandleBlendOut)
  (Variables|/Game/Goulandis/InteractionEssentials/Blueprints/Components/InteractionComponent.InteractionComponent_C|SetInteractionRadius (Variables|Default|GetInteractionComponent) (Variables|Default|GetCacheInteractionRadius))
  (Variables|Default|SetIsActive false)
  (bind _newtrack_0 (Timeline|MoveTimeline Stop)
    (:Update
      (Transformation|SetRelativeLocation _cube (Math|Vector|MakeVector (.x _relativelocation) (Math|Float|Lerp 0.0 (Math|Float|MakeLiteralFloat 2.2e+02) _newtrack_0) (.z _relativelocation)) false false))))

(event EventBeginPlay
  (Variables|Default|SetCacheInteractionRadius (Variables|/Game/Goulandis/InteractionEssentials/Blueprints/Components/InteractionComponent.InteractionComponent_C|GetInteractionRadius (Variables|Default|GetInteractionComponent))))

(fn ConstructionScript)

(fn GetCharAnimInstance
  (bind _asthird_person_anim_bp (Utilities|Casting|CastToThirdPerson_AnimBP (Components|SkeletalMesh|GetAnimInstance (Variables|/Script/Engine.Character|GetMesh (CallFunction|GetDemoCharacter)))))
  (return _asthird_person_anim_bp))

(fn InterpRelativeCameraY
  (params (Target :type Vector) (InterpSpeed :type Float%20%28double-precision%29))
  (bind _camera (Variables|Default|GetCamera))
  (bind _relativelocation (Variables|/Script/Engine.SceneComponent|GetRelativeLocation _camera))
  (Transformation|SetRelativeLocation _camera (Math|Vector|MakeVector (.x _relativelocation) (Math|Interpolation|FInterpTo (.y _relativelocation) (.Y (Math|Vector|BreakVector Target)) (Variables|Default|GetDeltaX) InterpSpeed) (.z _relativelocation)) false false)
  (return))