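; BP_Demo_Pickup is a demo pickup actor that the player collects through its HoldInvisible interaction component.
; Starting the interaction stops the demo character and disables its movement, and either completing or cancelling restores it.
; On completion, a timeline shrinks and rotates the Cube, then destroys the actor, while movement is re-enabled without waiting for the animation to finish.
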(event OnInteractionStarted(HoldInvisible)
  (bind _returnvalue (CallFunction|GetDemoCharacter))
  (Variables|/Game/Goulandis/InteractionEssentials/DemoContent/DemoCharacter_3P/ThirdPersonCharacter.ThirdPersonCharacter_C|SetCanMove _returnvalue false)
  (Components|Movement|StopMovementImmediately (Variables|/Script/Engine.Character|GetCharacterMovement _returnvalue)))

(event OnInteractionCompleted(HoldInvisible)
  (bind _cube (Variables|Default|GetCube))
  (Utilities|FlowControl|Sequence
    (:then_0
      (bind _newtrack_0 (Timeline|Timeline_0 PlayFromStart)
        (:Update
          (Transformation|SetRelativeScale3D _cube (Math|Conversions|ToVector(Float) (Math|Float|Lerp 0.5 0.01 _newtrack_0)))
          (Transformation|SetRelativeRotation _cube (Math|Rotator|Lerp(Rotator) "0, 0, 0" "-45.000000, 0,45.000000" _newtrack_0) false false))
        (:Finished
          (Actor|DestroyActor))))
    (:then_1
      (Variables|/Game/Goulandis/InteractionEssentials/DemoContent/DemoCharacter_3P/ThirdPersonCharacter.ThirdPersonCharacter_C|SetCanMove (CallFunction|GetDemoCharacter) true))))

(event OnInteractionCancelled(HoldInvisible)
  (Variables|/Game/Goulandis/InteractionEssentials/DemoContent/DemoCharacter_3P/ThirdPersonCharacter.ThirdPersonCharacter_C|SetCanMove (CallFunction|GetDemoCharacter) true))

(fn ConstructionScript)