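; Demo actor for the InteractionEssentials content that destroys itself when its InteractionComponent completes an interaction.
; The construction script optionally copies input, trigger method and duration settings onto that component when Customize is set.
; Tick turns the text label toward the player camera and sets it once to the actor's name.
; If Move is set, a timeline drives the actor's world Z between fixed heights.
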(event OnInteractionCompleted(InteractionComponent)
  (Actor|DestroyActor))

(event EventBeginPlay
  (bind _returnvalue (Transformation|GetActorLocation))
  (if (Variables|Default|GetMove)
    (bind _test (Timeline|Timeline_0 PlayFromStart)
      (:Update
        (Transformation|SetActorLocation (Math|Vector|MakeVector (.x _returnvalue) (.y _returnvalue) (Math|Float|MapRangeClamped _test 0.0 1.0 -4e+01 2.5e+02)) false false)))))

(event EventTick
  (params (DeltaSeconds :type Float%20%28single-precision%29))
  ;[1 1 1] rotate text
  (Transformation|SetWorldRotation (Variables|Default|GetTextRender) (Math|Rotator|FindLookatRotation (Transformation|GetWorldLocation (Variables|Default|GetTextRender)) (Camera|GetCameraLocation (Game|GetPlayerCameraManager 0))) false false)
  (Utilities|FlowControl|DoOnce false
    (:Completed
      (Rendering|Components|TextRender|SetText (Variables|Default|GetTextRender) (Utilities|Text|ToText(String) (Utilities|GetDisplayName self))))))

(fn ConstructionScript
  (bind _interactioncomponent (Variables|Default|GetInteractionComponent))
  (bind _interactioncomponent_2 (Variables|Default|GetInteractionComponent))
  (if (Variables|Default|GetCustomize)
    (Variables|/Game/Goulandis/InteractionEssentials/Blueprints/Components/InteractionComponent.InteractionComponent_C|SetInputKey_PC _interactioncomponent (Variables|Default|GetInInput_PC))
    (Variables|/Game/Goulandis/InteractionEssentials/Blueprints/Components/InteractionComponent.InteractionComponent_C|SetInputKey_Gamepad _interactioncomponent (Variables|Default|GetInInput_Gamepad))
    (Variables|/Game/Goulandis/InteractionEssentials/Blueprints/Components/InteractionComponent.InteractionComponent_C|SetInteractionInputMethod _interactioncomponent (Variables|Default|GetInputMethod))
    (Variables|/Game/Goulandis/InteractionEssentials/Blueprints/Components/InteractionComponent.InteractionComponent_C|SetInteractionKeyMapping _interactioncomponent (Variables|Default|GetInputMapping))
    (Variables|/Game/Goulandis/InteractionEssentials/Blueprints/Components/InteractionComponent.InteractionComponent_C|SetInteractionTriggerMethod _interactioncomponent_2 (Variables|Default|GetTriggerMethod))
    (Variables|/Game/Goulandis/InteractionEssentials/Blueprints/Components/InteractionComponent.InteractionComponent_C|SetInteractionDuration _interactioncomponent_2 (Variables|Default|GetDuration))))