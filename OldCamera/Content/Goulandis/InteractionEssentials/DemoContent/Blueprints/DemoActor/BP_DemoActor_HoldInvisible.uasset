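; Demo actor for InteractionEssentials that showcases a hold-invisible interaction component, reporting its state on a coloured text render.
; Component events show start, progress or repetition count, cancellation and completion, with completion reactivating the interaction through its manager after timed delays.
; The construction script passes PC and gamepad keys to the component and optionally shows a point light.
; An optional timeline moves the actor vertically; the text-facing-camera logic is disconnected.
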(event OnInteractionCompleted(InteractionComponent_HoldInvisible)
  (Utilities|FlowControl|Delay 0.2)
  (CallFunction|SetText "Interaction Completed" "(R=0.027313,G=1.000000,B=0.000000,A=1.000000)")
  (Utilities|FlowControl|Delay 5.0)
  (CallFunction|SetText "Come Back later." "(R=1.000000,G=0.000000,B=0.000000,A=1.000000)")
  (Utilities|FlowControl|Delay 3.0)
  (Default|ActivateInteraction (CallFunction|GetInteractionManager (Variables|Default|GetInteractionComponent_HoldInvisible)) true)
  (CallFunction|SetText "Ready to interact" "(R=1.000000,G=1.000000,B=1.000000,A=1.000000)"))

(event OnInteractionStarted(InteractionComponent_HoldInvisible)
  (CallFunction|SetText "Interaction started" "(R=1.000000,G=1.000000,B=1.000000,A=1.000000)"))

(event OnInteractionUpdate(InteractionComponent_HoldInvisible)
  (params (Value :type Float%20%28double-precision%29) (Repetitions :type Integer))
  (|IsRepeatEvent
    (:then
      (CallFunction|SetText (Utilities|Text|ToText(String) (Utilities|String|Append "Repetitions: " (Utilities|String|ToString(Integer) Repetitions))) "(R=1.000000,G=1.000000,B=1.000000,A=1.000000)"))
    (:else
      (CallFunction|SetText (Utilities|Text|ToText(String) (Utilities|String|Append "Interaction Progress: " (Utilities|String|ToString(Float) Value))) "(R=1.000000,G=1.000000,B=1.000000,A=1.000000)"))))

(event OnInteractionCancelled(InteractionComponent_HoldInvisible)
  (CallFunction|SetText "Interaction Cancelled" "(R=1.000000,G=0.000000,B=0.000000,A=1.000000)")
  (Utilities|FlowControl|Delay 3.0)
  (CallFunction|SetText "Ready to interact" "(R=1.000000,G=1.000000,B=1.000000,A=1.000000)"))

(event EventBeginPlay
  (bind _returnvalue (Transformation|GetActorLocation))
  (if (Variables|Default|GetMove)
    (bind _test (Timeline|Timeline_0 PlayFromStart)
      (:Update
        (Transformation|SetActorLocation (Math|Vector|MakeVector (.x _returnvalue) (.y _returnvalue) (Math|Float|MapRangeClamped _test 0.0 1.0 -4e+01 2.5e+02)) false false)))))

(event EventTick
  (params (DeltaSeconds :type Float%20%28single-precision%29)))

(fn ConstructionScript
  (bind _interactioncomponent_holdinvisible (Variables|Default|GetInteractionComponent_HoldInvisible))
  (Variables|/Game/Goulandis/InteractionEssentials/Blueprints/Components/InteractionComponent.InteractionComponent_C|SetInputKey_PC _interactioncomponent_holdinvisible (Variables|Default|GetInputKey_PC))
  (Variables|/Game/Goulandis/InteractionEssentials/Blueprints/Components/InteractionComponent.InteractionComponent_C|SetInputKey_Gamepad _interactioncomponent_holdinvisible (Variables|Default|GetInputKey_Gamepad))
  (if (Variables|Default|GetUseLight)
    (Rendering|SetVisibility (Variables|Default|GetPointLight) true false)))

(fn SetText
  (params (Value :type Text) (Color :type Linear%20Color%20Structure))
  (bind _textrender (Variables|Default|GetTextRender))
  (Rendering|Components|TextRender|SetText _textrender (Utilities|Text|MakeLiteralText Value))
  (Rendering|Components|TextRender|SetTextRenderColor _textrender (Math|Conversions|ToColor(LinearColor) Color)))