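; Demo deadzone volume that returns the demo character to the nearest spawn point when entered.
; A box overlap by a Character or involving a skeletal mesh component, or the Trigger event, starts the reset.
; The screen fades out, the character teleports to the closest "Spawn"-tagged actor and refreshes its pose.
; The view then blends back to the character before the screen fades in.
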(event OnComponentBeginOverlap(Box)
  (params (OverlappedComponent :type Primitive%20Component%20Object%20Reference) (OtherActor :type Actor%20Object%20Reference) (OtherComp :type Primitive%20Component%20Object%20Reference) (OtherBodyIndex :type Integer) (bFromSweep :type Boolean) (SweepResult :type Hit%20Result%20Structure%20%28by%20ref%29))
  (Utilities|Casting|CastToCharacter OtherActor
    (:then
      _)
    (:CastFailed
      (Utilities|Casting|CastToSkeletalMeshComponent OverlappedComponent
        (:then
          _)
        (:CastFailed
          (Utilities|Casting|CastToSkeletalMeshComponent OtherComp)))))
  (CameraFades|StartCameraFade :self (Game|GetPlayerCameraManager 0) :ToAlpha 1.0 :Duration 0.25 :bHoldWhenFinished true)
  (Utilities|FlowControl|Delay 0.25)
  (Transformation|SetActorLocation (CallFunction|GetDemoCharacter) (CallFunction|FindNearestSpawn) false true)
  (Default|RefreshPose (CallFunction|GetDemoCharacter))
  (Game|Player|SetViewTargetwithBlend (Game|GetPlayerController 0) (CallFunction|GetDemoCharacter) 0.6 "VTBlend_Cubic" 0.0 true)
  (Utilities|FlowControl|Delay 0.6)
  (CameraFades|StartCameraFade (Game|GetPlayerCameraManager 0) 1.0 0.0 0.5 "(R=0.000000,G=0.000000,B=0.000000,A=1.000000)" false true))

(event Custom|Trigger
  (CameraFades|StartCameraFade :self (Game|GetPlayerCameraManager 0) :ToAlpha 1.0 :Duration 0.25 :bHoldWhenFinished true)
  (Utilities|FlowControl|Delay 0.25)
  (Transformation|SetActorLocation (CallFunction|GetDemoCharacter) (CallFunction|FindNearestSpawn) false true)
  (Default|RefreshPose (CallFunction|GetDemoCharacter))
  (Game|Player|SetViewTargetwithBlend (Game|GetPlayerController 0) (CallFunction|GetDemoCharacter) 0.6 "VTBlend_Cubic" 0.0 true)
  (Utilities|FlowControl|Delay 0.6)
  (CameraFades|StartCameraFade (Game|GetPlayerCameraManager 0) 1.0 0.0 0.5 "(R=0.000000,G=0.000000,B=0.000000,A=1.000000)" false true))

(fn ConstructionScript)

(fn FindNearestSpawn
  (bind _outactors (Actor|GetAllActorswithTag "Spawn"))
  (for _array_element _outactors
    (Utilities|IsValid _array_element
      (:Is%20Valid
        (Utilities|Array|Add (LocalVariables|GetDistances) (Transformation|GetDistanceTo (CallFunction|GetDemoCharacter) _array_element))
        (Utilities|Array|Add (LocalVariables|GetActors) _array_element))))
  (return (Transformation|GetActorLocation (Utilities|Array|Get(acopy) (LocalVariables|GetActors) (.IndexOfMinValue (Math|Float|MinOfFloatArray (LocalVariables|GetDistances)))))))