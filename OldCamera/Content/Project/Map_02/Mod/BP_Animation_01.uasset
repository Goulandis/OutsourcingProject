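; BP_Animation_01 is a map actor that moves a skeletal mesh along its spline when play begins.
; A timeline's Position output, scaled by spline length, samples location and rotation along the path on each update.
; Local spline points are offset by the root's world location only, so root rotation and scale are not applied to the path.
; The mesh's yaw is turned back 90 degrees from the spline direction.
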(event EventBeginPlay
  (bind _spline (Variables|Default|GetSpline))
  (bind _position (Timeline|Timeline_0 Play)
    (:Update
      (Transformation|SetWorldTransform (Variables|Default|GetSkeletalMesh) (Math|Transform|MakeTransform (+ (Spline|GetLocationatDistanceAlongSpline _spline (* _position (Spline|GetSplineLength _spline)) "Local") (Transformation|GetWorldLocation (Variables|Default|GetDefaultSceneRoot))) (Math|Rotator|MakeRotator (.roll (Spline|GetRotationatDistanceAlongSpline _spline (* _position (Spline|GetSplineLength _spline)) "Local")) (.pitch (Spline|GetRotationatDistanceAlongSpline _spline (* _position (Spline|GetSplineLength _spline)) "Local")) (- (.yaw (Spline|GetRotationatDistanceAlongSpline _spline (* _position (Spline|GetSplineLength _spline)) "Local")) 9e+01)) (Variables|Default|GetScale)) false false))))

(event EventTick
  (params (DeltaSeconds :type Float%20%28single-precision%29)))

(fn ConstructionScript)