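; BP_Door_01 is a door that swings open when a FirstPersonCharacter enters its Capsule trigger.
; The overlap plays a timeline whose alpha lerps the Chinge component's relative rotation from zero to a quarter-turn.
; A check on the character's world forward X picks the swing, but both branches set the same rotation.
; Ending any overlap with the capsule reverses the timeline to close it, without a character check.
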(event OnComponentBeginOverlap(Capsule)
  (params (OverlappedComponent :type Primitive%20Component%20Object%20Reference) (OtherActor :type Actor%20Object%20Reference) (OtherComp :type Primitive%20Component%20Object%20Reference) (OtherBodyIndex :type Integer) (bFromSweep :type Boolean) (SweepResult :type Hit%20Result%20Structure%20%28by%20ref%29))
  (bind _asfirst_person_character (Utilities|Casting|CastToFirstPersonCharacter OtherActor))
  (if (> (.X (Math|Vector|BreakVector (Transformation|GetActorForwardVector _asfirst_person_character))) 0.0)
    (Variables|Default|SetDoorRot "0,-90.000000, 0")
    (bind _alpha (Timeline|Timeline_0 Play)
      (:Update
        (Transformation|SetRelativeRotation (Variables|Default|GetChinge) (Math|Rotator|Lerp(Rotator) "0, 0, 0" (Variables|Default|GetDoorRot) _alpha true) false false)))
    (else
      (Variables|Default|SetDoorRot "0,-90.000000, 0")
      (Timeline|Timeline_0 Play))))

(event OnComponentEndOverlap(Capsule)
  (params (OverlappedComponent :type Primitive%20Component%20Object%20Reference) (OtherActor :type Actor%20Object%20Reference) (OtherComp :type Primitive%20Component%20Object%20Reference) (OtherBodyIndex :type Integer))
  (bind _alpha (Timeline|Timeline_0 Reverse)
    (:Update
      (Transformation|SetRelativeRotation (Variables|Default|GetChinge) (Math|Rotator|Lerp(Rotator) "0, 0, 0" (Variables|Default|GetDoorRot) _alpha true) false false))))

(fn ConstructionScript)