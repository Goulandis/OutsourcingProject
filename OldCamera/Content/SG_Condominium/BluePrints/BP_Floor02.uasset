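; BP_Floor02 is a condominium floor actor whose material can be switched between Marquina and white marble.
; Overlapping its Box creates the BP_FloorTile widget and shows the mouse cursor with game-and-UI input; leaving removes all widgets and restores game-only input.
; The I_Marquina and I_WhiteMarble events, which look like interface calls, each set the matching floor material on the StaticMesh.
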(event OnComponentBeginOverlap(Box)
  (params (OverlappedComponent :type Primitive%20Component%20Object%20Reference) (OtherActor :type Actor%20Object%20Reference) (OtherComp :type Primitive%20Component%20Object%20Reference) (OtherBodyIndex :type Integer) (bFromSweep :type Boolean) (SweepResult :type Hit%20Result%20Structure%20%28by%20ref%29))
  (bind _returnvalue (Game|GetPlayerController 0))
  ;[1 1 1] Widget Control
  (bind _returnvalue_2 (UserInterface|CreateWidget "/Game/SG_Condominium/BluePrints/BP_FloorTile.BP_FloorTile_C"))
  (UserInterface|Viewport|AddtoViewport _returnvalue_2 0)
  (Input|SetInputModeGameandUI _returnvalue 0 "DoNotLock" true)
  (Variables|/Script/Engine.PlayerController|SetbShowMouseCursor _returnvalue true))

(event OnComponentEndOverlap(Box)
  (params (OverlappedComponent :type Primitive%20Component%20Object%20Reference) (OtherActor :type Actor%20Object%20Reference) (OtherComp :type Primitive%20Component%20Object%20Reference) (OtherBodyIndex :type Integer))
  (bind _returnvalue (Game|GetPlayerController 0))
  ;[1 1 1] Widget Control
  (Viewport|RemoveAllWidgets)
  (Input|SetInputModeGameOnly _returnvalue)
  (Variables|/Script/Engine.PlayerController|SetbShowMouseCursor _returnvalue false))

(event Custom|I_Marquina
  (Rendering|Material|SetMaterial (Variables|Default|GetStaticMesh) 0 "/Game/SG_Condominium/Materials/M_Floor_Marquina.M_Floor_Marquina"))

(event Custom|I_WhiteMarble
  (Rendering|Material|SetMaterial (Variables|Default|GetStaticMesh) 0 "/Game/SG_Condominium/Materials/M_Floor_Marble.M_Floor_Marble"))

(fn ConstructionScript)