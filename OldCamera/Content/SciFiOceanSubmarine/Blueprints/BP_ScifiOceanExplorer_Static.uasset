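; Static sci-fi ocean submarine prop with configurable lighting, materials and collision, with no active event logic.
; The construction script tunes or destroys the spotlights and interior lights, then applies hull, interior and glass materials.
; Interior meshes and lights are gathered into arrays so that materials and intensity are set in bulk.
; Turning off the Collision flag disables collision on the submarine's meshes.
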(event EventBeginPlay)

(event Collision|EventActorBeginOverlap
  (params (OtherActor :type Actor%20Object%20Reference)))

(event EventTick
  (params (DeltaSeconds :type Float%20%28single-precision%29)))

(fn ConstructionScript
  (|AdjustSpotlights)
  (|InteriorLights)
  (|AddInteriorMeshestoArray) ; We group Interior Meshes into an array to easily modify variables for all of them simultaniously
  (CallFunction|SetMaterials)
  (if (not (Variables|Default|GetCollision))
    (Collision|SetCollisionEnabled (Variables|Default|GetSM_ScifiOceanSubmarine_Seat) "NoCollision")))

(fn SetMaterials
  (bind _sm_scifioceansubmarine_glass (Variables|Default|GetSM_ScifiOceanSubmarine_Glass))
  ;[1 1 1] Set Hull Material
  (Rendering|Material|SetMaterial (Variables|Default|GetSM_ScifiOceanSubmarine) 0 (Variables|Materials|GetExteriorMaterial))
  ;[1 1 1] Set Interior Material
  (for _array_element (Variables|Materials|GetInteriorMeshes)
    (Rendering|Material|SetMaterial _array_element 0 (Variables|Materials|GetInteriorMaterial))
    ;[1 1 1] Set Glass Material
    (Rendering|Material|SetMaterial _sm_scifioceansubmarine_glass 0 (Variables|Materials|GetGlass_Material_Ext))
    (Rendering|Material|SetMaterial _sm_scifioceansubmarine_glass 1 (Variables|Materials|GetGlass_Material_Int))))