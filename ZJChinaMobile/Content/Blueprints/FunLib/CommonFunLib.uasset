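; Blueprint function library of shared getters for the game's core objects: game instance, its Config, player controller and HUD.
; GetConfig builds on GetGGameInstance, and GetGHUD builds on GetGPlayerController for player index 0, each guarded by IsValid.
; Failed casts to the G-prefixed classes report through DLog.
; GetGPlayerController also prints the controller's display name on every call, including those made through GetGHUD.
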(fn GetGGameInstance
  (bind ___worldcontext (LocalVariables|Get__WorldContext))
  (bind _asggame_instance (Utilities|Casting|CastToGGameInstance (Game|GetGameInstance ___worldcontext))
    (:then
      (return _asggame_instance))
    (:CastFailed
      (CallFunction|DLog "Error:GetGGameInstance" "Failed to cast GameInstance to GGameInstance" ___worldcontext))))

(fn GetConfig
  (bind ___worldcontext (LocalVariables|Get__WorldContext))
  (bind _ggameinstance (CallFunction|GetGGameInstance ___worldcontext))
  (Utilities|IsValid _ggameinstance
    (:Is%20Valid
      (return (Variables|/Game/GamePlay/GGameInstance.GGameInstance_C|GetConfig _ggameinstance)))))

(fn GetGPlayerController
  (bind ___worldcontext (LocalVariables|Get__WorldContext))
  (bind _returnvalue (Game|GetPlayerController ___worldcontext))
  (Development|PrintString ___worldcontext (Utilities|GetDisplayName _returnvalue))
  (bind _asgplayer_controller (Utilities|Casting|CastToGPlayerController _returnvalue)
    (:then
      (return _asgplayer_controller))
    (:CastFailed
      (CallFunction|DLog "Error:GetGPlayerController" "Failed to cast PlayerController to GPlayerController" ___worldcontext))))

(fn GetGHUD
  (bind ___worldcontext (LocalVariables|Get__WorldContext))
  (bind _gplayercontroller (CallFunction|GetGPlayerController ___worldcontext))
  (Utilities|IsValid _gplayercontroller
    (:Is%20Valid
      (bind _asghud (Utilities|Casting|CastToGHUD (HUD|GetHUD _gplayercontroller))
        (:then
          (return _asghud))
        (:CastFailed
          (CallFunction|DLog "Error:GetGHUD" "Failed to cast HUD to GHUD" ___worldcontext))))))