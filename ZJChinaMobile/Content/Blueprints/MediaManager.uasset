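; Media manager actor that fills the level's keyed display screens with external images and videos at BeginPlay.
; Reads PPTDir from config, defaulting to DiyContents in the project, then sorts folders into image, video and optional content matched to screens by key.
; Builds dynamic materials from textures and runtime media players, sources and textures from each folder's first video file.
; Multi-key DisplayScreenRoboticArm screens receive content per key through a separate pass.
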(event EventBeginPlay
  (CallFunction|LoadConfig)
  (CallFunction|Init))

(event Collision|EventActorBeginOverlap
  (params (OtherActor :type Actor%20Object%20Reference)))

(event EventTick
  (params (DeltaSeconds :type Float%20%28single-precision%29)))

(fn ConstructionScript)

(fn Init
  (if (Utilities|Enum|Equal(Enum) (Variables|Default|GetPPTDir) "")
    (LocalVariables|SetPPTDirSelf (Class|KismetSystemLibrary|ConverttoAbsolutePath (Utilities|String|Append (Class|KismetSystemLibrary|GetProjectDirectory) "DiyContents")))
    (else
      (LocalVariables|SetPPTDirSelf (Variables|Default|GetPPTDir))))
  (bind (_imagedirs _videodirs _optionaldirs) (Class|CommonFunLib|GetClassifyDir (LocalVariables|GetPPTDirSelf)))
  (Variables|Default|SetImageDirs _imagedirs)
  (Variables|Default|SetVideoDirs _videodirs)
  (Variables|Default|SetOptionalDirs _optionaldirs)
  (Utilities|FlowControl|Sequence
    (:then_0
      (bind _returnvalue (Class|CommonFunLib|LoadAllTexturefromDirList (Variables|Default|GetImageDirs)))
      (bind _output_get (LocalVariables|SetTexList _returnvalue))
      (CallFunction|InitPNG _output_get)
      (CallFunction|InitDisplayScreenRoboticArm _output_get (Variables|Default|GetVideoDirs) "NewEnumerator0"))
    (:then_1
      (CallFunction|InitMedia (Variables|Default|GetVideoDirs))
      (CallFunction|InitDisplayScreenRoboticArm (LocalVariables|GetTexList) (Variables|Default|GetVideoDirs) "NewEnumerator1"))
    (:then_2
      (CallFunction|InitOptionalContent (Variables|Default|GetOptionalDirs)))))

(fn GetDisplaybyKey
  (params (Key :type String))
  (for _array_element (Variables|Default|GetDisplayers)
    (if (Utilities|Enum|Equal(Enum) Key (.Key (Utilities|Struct|BreakSDisplayComb _array_element)))
      (return _array_element true)))
  (return "" false))

(fn LoadConfig
  (bind _outvalue (|GetJsonField (CallFunction|GetConfig) "Display"))
  (bind _outvalue_2 (|GetJsonField _outvalue "PPTDir"))
  (Variables|Default|SetPPTDir _outvalue_2))

(fn SetDisplayTexsbyKey
  (params (Key :type String) (Texs :type Array%20of%20Texture%202D%20Object%20References))
  (bind _index (CallFunction|GetDisplayIndexbyKey Key))
  (bind _displayers (Variables|Default|GetDisplayers))
  (bind _output (Utilities|Array|Get(acopy) _displayers _index))
  (if (and (>= _index 0) (< _index (Utilities|Array|Length (Variables|Default|GetDisplayers))))
    (Utilities|Array|SetArrayElem _displayers _index (Utilities|Struct|MakeSDisplayComb (.key _output) "NewEnumerator0" (.displayscreen _output) Texs (.mats _output) (.mediaplayers _output) (.mediasources _output) (.mediatexture _output)))))

(fn SetDisplaybyKey
  (params (Key :type String) (DisplayComb :type S%20Display%20Comb%20Structure))
  (bind (_array_element _array_index) (Utilities|Array|ForEachLoopwithBreak (Variables|Default|GetDisplayers))
    (:LoopBody
      (if (Utilities|Enum|Equal(Enum) Key (.Key (Utilities|Struct|BreakSDisplayComb _array_element)))
        (Utilities|Array|SetArrayElem (Variables|Default|GetDisplayers) _array_index DisplayComb)))))

(fn GetDisplayIndexbyKey
  (params (Key :type String))
  (for (_array_element _array_index) (Variables|Default|GetDisplayers)
    (if (Utilities|Enum|Equal(Enum) Key (.Key (Utilities|Struct|BreakSDisplayComb _array_element)))
      (return _array_index)
      (else
        (bind _asdisplay_screen_robotic_arm (Utilities|Casting|CastToDisplayScreenRoboticArm (.DisplayScreen (Utilities|Struct|BreakSDisplayComb _array_element))))
        (if (Utilities|Array|ContainsItem (Variables|/Game/Blueprints/Screen/DisplayScreenRoboticArm.DisplayScreenRoboticArm_C|GetKeys _asdisplay_screen_robotic_arm) Key)
          (return _array_index)))))
  (return -1))

(fn PPT2PNG
  (Class|CommonFunLib|InitPPT2PNGScript)
  (Class|CommonFunLib|SetupPPT2PNGServer))

(fn CreateMatbyTex
  (for (_array_element _array_index) (Variables|Default|GetDisplayers)
    (for _array_element_2 (.texs _array_element)
      (bind _returnvalue (Rendering|Material|CreateDynamicMaterialInstance "/Game/Blueprints/Screen/Materials/M_ScreenBase.M_ScreenBase" "None" "None" :!class /Script/Engine.KismetMaterialLibrary))
      (Rendering|Material|SetTextureParameterValue _returnvalue "Texture" _array_element_2)
      (Utilities|Array|Add (LocalVariables|GetMats) _returnvalue))
    (Utilities|Array|SetArrayElem (Variables|Default|GetDisplayers) _array_index (Utilities|Struct|MakeSDisplayComb (.key _array_element) "NewEnumerator0" (.displayscreen _array_element) (.texs _array_element) (LocalVariables|GetMats) (.mediaplayers _array_element) (.mediasources _array_element) (.mediatexture _array_element)))
    (Utilities|Array|Clear (LocalVariables|GetMats))))

(fn InitMedia
  (params (MediaPaths :type Array%20of%20Strings))
  (bind _displayers (Variables|Default|GetDisplayers))
  (for _array_element MediaPaths
    (bind _returnvalue (Class|CommonFunLib|GetFilesfromDir _array_element))
    (if (> (Utilities|Array|Length _returnvalue) 0)
      (bind _returnvalue_2 (Game|ConstructObjectfromClass "/Script/MediaAssets.FileMediaSource"))
      (Class|FileMediaSource|SetFilePath _returnvalue_2 (Utilities|Array|Get(acopy) _returnvalue))
      (bind _returnvalue_3 (Class|CommonFunLib|GetKeybyDir _array_element))
      (bind _returnvalue_4 (Game|ConstructObjectfromClass "/Script/MediaAssets.MediaPlayer"))
      (bind _returnvalue_5 (Game|ConstructObjectfromClass "/Script/MediaAssets.MediaTexture"))
      (Media|MediaSoundComponent|SetMediaPlayer _returnvalue_5 _returnvalue_4)
      (Class|MediaTexture|UpdateResource _returnvalue_5)
      (if (and (>= (CallFunction|GetDisplayIndexbyKey _returnvalue_3) 0) (< (CallFunction|GetDisplayIndexbyKey _returnvalue_3) (Utilities|Array|Length (Variables|Default|GetDisplayers))))
        (Utilities|Array|SetArrayElem _displayers (CallFunction|GetDisplayIndexbyKey _returnvalue_3) (Utilities|Struct|MakeSDisplayComb (.key (Utilities|Array|Get(acopy) _displayers (CallFunction|GetDisplayIndexbyKey _returnvalue_3))) "NewEnumerator1" (.displayscreen (Utilities|Array|Get(acopy) _displayers (CallFunction|GetDisplayIndexbyKey _returnvalue_3))) (.texs (Utilities|Array|Get(acopy) _displayers (CallFunction|GetDisplayIndexbyKey _returnvalue_3))) (.mats (Utilities|Array|Get(acopy) _displayers (CallFunction|GetDisplayIndexbyKey _returnvalue_3))) _returnvalue_4 _returnvalue_2 _returnvalue_5))
        (bind _returnvalue_6 (Game|AddComponentbyClass "/Script/MediaAssets.MediaSoundComponent" false))
        (Transformation|AttachComponentToComponent _returnvalue_6 (Variables|/Game/Blueprints/Screen/DisplayScreen.DisplayScreen_C|GetDefaultSceneRoot (.displayscreen (Utilities|Array|Get(acopy) _displayers (CallFunction|GetDisplayIndexbyKey _returnvalue_3)))) "None" "KeepRelative" "KeepRelative" "KeepRelative" true)
        (Media|MediaSoundComponent|SetMediaPlayer _returnvalue_6 _returnvalue_4)
        (Variables|/Game/Blueprints/Screen/DisplayScreen.DisplayScreen_C|SetMediaSoundComp (.displayscreen (Utilities|Array|Get(acopy) _displayers (CallFunction|GetDisplayIndexbyKey _returnvalue_3))) _returnvalue_6))))
  (for _array_element_2 (Variables|Default|GetDisplayers)
    (if (and (Utilities|Enum|Equal(Enum) (.Key (Utilities|Struct|BreakSDisplayComb _array_element_2)) (Variables|/Game/Blueprints/Screen/DisplayScreen.DisplayScreen_C|GetKey (.DisplayScreen (Utilities|Struct|BreakSDisplayComb _array_element_2)))) (Utilities|Enum|Equal(Enum) (.DisplayType (Utilities|Struct|BreakSDisplayComb _array_element_2)) "NewEnumerator1"))
      (Default|SetContent (.DisplayScreen (Utilities|Struct|BreakSDisplayComb _array_element_2)) (.Texs (Utilities|Struct|BreakSDisplayComb _array_element_2)) (.Mats (Utilities|Struct|BreakSDisplayComb _array_element_2)) (.MediaPlayers (Utilities|Struct|BreakSDisplayComb _array_element_2)) (.MediaSources (Utilities|Struct|BreakSDisplayComb _array_element_2)) (.DisplayType (Utilities|Struct|BreakSDisplayComb _array_element_2)) (.MediaTexture (Utilities|Struct|BreakSDisplayComb _array_element_2)))
      (Default|ShowPage (.DisplayScreen (Utilities|Struct|BreakSDisplayComb _array_element_2)) true))))

(fn KeyIsExists
  (params (Key :type Integer))
  (for _array_element (Variables|Default|GetDisplayers)
    (if (Utilities|Enum|Equal(Enum) "" (.Key (Utilities|Struct|BreakSDisplayComb _array_element)))
      (return true)))
  (return false))

(fn InitPNG
  (params (ImgList :type Array%20of%20Tex%20List%20Structures))
  (for _array_element ImgList
    (CallFunction|SetDisplayTexsbyKey (.Key (Utilities|Struct|BreakTexList _array_element)) (.Texs (Utilities|Struct|BreakTexList _array_element))))
  (CallFunction|CreateMatbyTex)
  (for _array_element_2 (Variables|Default|GetDisplayers)
    (if (and (Utilities|Enum|Equal(Enum) (.Key (Utilities|Struct|BreakSDisplayComb _array_element_2)) (Variables|/Game/Blueprints/Screen/DisplayScreen.DisplayScreen_C|GetKey (.DisplayScreen (Utilities|Struct|BreakSDisplayComb _array_element_2)))) (Utilities|Enum|Equal(Enum) (.DisplayType (Utilities|Struct|BreakSDisplayComb _array_element_2)) "NewEnumerator0"))
      (Default|SetContent (.DisplayScreen (Utilities|Struct|BreakSDisplayComb _array_element_2)) (.Texs (Utilities|Struct|BreakSDisplayComb _array_element_2)) (.Mats (Utilities|Struct|BreakSDisplayComb _array_element_2)) (.MediaPlayers (Utilities|Struct|BreakSDisplayComb _array_element_2)) (.MediaSources (Utilities|Struct|BreakSDisplayComb _array_element_2)) (.DisplayType (Utilities|Struct|BreakSDisplayComb _array_element_2)) (.MediaTexture (Utilities|Struct|BreakSDisplayComb _array_element_2)))
      (Default|ShowPage (.DisplayScreen (Utilities|Struct|BreakSDisplayComb _array_element_2)) true))))

(fn InitDisplayScreenRoboticArm
  (params (TexList :type Array%20of%20Tex%20List%20Structures) (MediaPaths :type Array%20of%20Strings) (DisplayType :type EDisplayType%20Enum :default "NewEnumerator0"))
  (switch Utilities|FlowControl|Switch|SwitchonEDisplayType DisplayType
    (:NewEnumerator0
      (for _array_element (Variables|Default|GetDisplayers)
        (LocalVariables|SetDisplay 0)
        (bind _asdisplay_screen_robotic_arm (Utilities|Casting|CastToDisplayScreenRoboticArm (.DisplayScreen (Utilities|Struct|BreakSDisplayComb _array_element))))
        (LocalVariables|SetDisplay _asdisplay_screen_robotic_arm)
        (for _array_element_2 (Variables|/Game/Blueprints/Screen/DisplayScreenRoboticArm.DisplayScreenRoboticArm_C|GetKeys _asdisplay_screen_robotic_arm)
          (bind _array_element_3 (Utilities|Array|ForEachLoopwithBreak TexList :!label _label)
            (:LoopBody
              (if (Utilities|Enum|Equal(Enum) _array_element_2 (.Key (Utilities|Struct|BreakTexList _array_element_3)))
                (Default|SetTexsandMatsbyKey (LocalVariables|GetDisplay) (.Key (Utilities|Struct|BreakTexList _array_element_3)) (.Texs (Utilities|Struct|BreakTexList _array_element_3)) "NewEnumerator0")
                (goto _label Break)))))
        (Default|ShowPage (LocalVariables|GetDisplay) true)))
    (:NewEnumerator1
      (for _array_element_4 (Variables|Default|GetDisplayers)
        (bind _asdisplay_screen_robotic_arm_2 (Utilities|Casting|CastToDisplayScreenRoboticArm (.DisplayScreen (Utilities|Struct|BreakSDisplayComb _array_element_4))))
        (LocalVariables|SetDisplay _asdisplay_screen_robotic_arm_2)
        (for _array_element_5 (Variables|/Game/Blueprints/Screen/DisplayScreenRoboticArm.DisplayScreenRoboticArm_C|GetKeys _asdisplay_screen_robotic_arm_2)
          (LocalVariables|SetCurrentKey _array_element_5)
          (LocalVariables|SetMediaPathsIndex -1)
          (bind (_array_element_6 _array_index) (Utilities|Array|ForEachLoopwithBreak MediaPaths :!label _label_2)
            (:LoopBody
              (bind _returnvalue (Class|CommonFunLib|GetKeybyDir _array_element_6))
              (if (Utilities|Enum|Equal(Enum) _returnvalue (LocalVariables|GetCurrentKey))
                (LocalVariables|SetMediaPathsIndex _array_index)
                (goto _label_2 Break)))
            (:Completed
              (if (>= (LocalVariables|GetMediaPathsIndex) 0)
                (bind _returnvalue_2 (Game|ConstructObjectfromClass "/Script/MediaAssets.FileMediaSource"))
                (bind _returnvalue_3 (Class|CommonFunLib|GetFilesfromDir (Utilities|Array|Get(acopy) MediaPaths (LocalVariables|GetMediaPathsIndex))))
                (if (> (Utilities|Array|Length _returnvalue_3) 0)
                  (Class|FileMediaSource|SetFilePath _returnvalue_2 (Utilities|Array|Get(acopy) _returnvalue_3))
                  (bind _returnvalue_4 (Game|ConstructObjectfromClass "/Script/MediaAssets.MediaPlayer"))
                  (bind _returnvalue_5 (Game|ConstructObjectfromClass "/Script/MediaAssets.MediaTexture"))
                  (Media|MediaSoundComponent|SetMediaPlayer _returnvalue_5 _returnvalue_4)
                  (Class|MediaTexture|UpdateResource _returnvalue_5)
                  (Default|SetMediaContentbyKey (LocalVariables|GetDisplay) _returnvalue_2 _returnvalue_4 _returnvalue_5 (LocalVariables|GetCurrentKey)))))))
        (Default|ShowPage (LocalVariables|GetDisplay) true)))))

(fn InitOptionalContent
  (params (OptionalDirs :type Array%20of%20Strings))
  (for _array_element OptionalDirs
    (bind _returnvalue (Class|CommonFunLib|GetKeybyDir _array_element))
    (bind _returnvalue_2 (Class|CommonFunLib|GetAllSubdirectories _array_element))
    (Variables|/Game/Blueprints/Screen/DisplayScreen.DisplayScreen_C|SetOptionalDirs (.displayscreen (Utilities|Array|Get(acopy) (Variables|Default|GetDisplayers) (CallFunction|GetDisplayIndexbyKey _returnvalue))) _returnvalue_2)
    (Default|ShowPage (.displayscreen (Utilities|Array|Get(acopy) (Variables|Default|GetDisplayers) (CallFunction|GetDisplayIndexbyKey _returnvalue))) true)))