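; Trigger box that brings a MetaHuman narrator to its arrow when the first-person player enters and drops it below the floor on exit.
; It plays index-paired sounds and animations, chaining to the next topic as each clip finishes and syncing the HUD combo box.
; Controller mute and pause events control speech.
; An optional extra skeletal mesh animates on overlap, as does the display screen's robotic arm during topic updates.
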(event EventBeginPlay
  (bind _gplayercontroller (CallFunction|GetGPlayerController))
  (EventDispatchers|BindEventtoOnMetahumenMute _gplayercontroller (EventDispatchers|CreateEvent :!event OnMetahumenMute))
  (EventDispatchers|BindEventtoOnMetahumenSpeekPause _gplayercontroller (EventDispatchers|CreateEvent :!event OnMetahumenSpeekPause))
  (EventDispatchers|BindEventtoOnAudioFinished (Variables|Default|GetAudio) (EventDispatchers|CreateEvent :!event OnAudioFinished))
  (EventDispatchers|BindEventtoOnUWComboxCompleted (CallFunction|GetGHUD) (EventDispatchers|CreateEvent :!event OnUWComboBoxCompleted))
  (Components|Animation|SetAnimation (Variables|/Script/Engine.Character|GetMesh (Variables|Default|GetNarrator)) (Variables|Default|GetAS_Idle)))

(fn ConstructionScript
  (bind _box (Variables|Default|GetBox))
  (Collision|BindEventtoOnComponentBeginOverlap _box (EventDispatchers|CreateEvent :!event OnBoxOverlapBegin))
  (Collision|BindEventtoOnComponentEndOverlap _box (EventDispatchers|CreateEvent :!event OnBoxOverlapBoxEnd)))

(fn OnBoxOverlapBegin
  (params (OverlappedComponent :type Primitive%20Component%20Object%20Reference) (OtherActor :type Actor%20Object%20Reference) (OtherComp :type Primitive%20Component%20Object%20Reference) (OtherBodyIndex :type Integer) (bFromSweep :type Boolean) (SweepResult :type Hit%20Result%20Structure))
  (bind _narrator (Variables|Default|GetNarrator))
  (Utilities|Casting|CastToGFirstPersonCharacter OtherActor)
  (Variables|Default|SetInBox true)
  (Variables|/Game/GamePlay/GHUD.GHUD_C|SetCurrentNarratorTrrigerBox (CallFunction|GetGHUD) self)
  (if (Variables|Default|GetIsMute)
    _
    (else
      (Utilities|IsValid _narrator
        (:Is%20Valid
          (Audio|Components|Audio|Play (Variables|/Script/Engine.Character|GetMesh _narrator) true)
          (CallFunction|UpdateSpeekSound)))))
  (CallFunction|ShowNarrator true)
  (CallFunction|OtherBeginAction))

(fn OnBoxOverlapBoxEnd
  (params (OverlappedComponent :type Primitive%20Component%20Object%20Reference) (OtherActor :type Actor%20Object%20Reference) (OtherComp :type Primitive%20Component%20Object%20Reference) (OtherBodyIndex :type Integer))
  (bind _ghud (CallFunction|GetGHUD))
  (bind _narrator (Variables|Default|GetNarrator))
  (bind _narrator_2 (Variables|Default|GetNarrator))
  (Utilities|Casting|CastToGFirstPersonCharacter OtherActor)
  (Variables|Default|SetInBox false)
  (Utilities|IsValid _ghud
    (:Is%20Valid
      (if (== (Variables|/Game/GamePlay/GHUD.GHUD_C|GetCurrentNarratorTrrigerBox _ghud) self)
        (if (Variables|Default|GetIsMute) :!label _label
          _
          (else
            (Utilities|IsValid _narrator_2
              (:Is%20Valid
                (Components|Animation|SetAnimation (Variables|/Script/Engine.Character|GetMesh _narrator_2) (Variables|Default|GetAS_Idle))
                (Audio|Components|Audio|Stop (Variables|Default|GetAudio))))))
        (CallFunction|ShowNarrator false)
        (else
          (Utilities|IsValid _narrator
            (:Is%20Valid
              (Components|Animation|SetAnimation (Variables|/Script/Engine.Character|GetMesh _narrator) (Variables|Default|GetAS_Idle))
              (Audio|Components|Audio|Stop (Variables|Default|GetAudio)))))))
    (:Is%20Not%20Valid
      (goto _label)))
  (CallFunction|OtherEndAction))

(fn OnMetahumenMute
  (params (Mute :type Boolean))
  (bind _ghud (CallFunction|GetGHUD))
  (bind _narrator (Variables|Default|GetNarrator))
  (bind _narrator_2 (Variables|Default|GetNarrator))
  (bind _uw_main (Variables|/Game/GamePlay/GHUD.GHUD_C|GetUW_Main _ghud))
  (bind _output_get (Variables|Default|SetIsMute Mute))
  (if _output_get
    (if (Variables|Default|GetInBox)
      (Utilities|IsValid _narrator_2
        (:Is%20Valid
          (Components|Animation|SetAnimation (Variables|/Script/Engine.Character|GetMesh _narrator_2) (Variables|Default|GetAS_Idle))
          (Audio|Components|Audio|Stop (Variables|Default|GetAudio)))))
    (elif (Variables|Default|GetInBox)
      (Utilities|IsValid _narrator
        (:Is%20Valid
          (Audio|Components|Audio|Play (Variables|/Script/Engine.Character|GetMesh _narrator) true)
          (if (Utilities|Array|ContainsItem (Variables|Default|GetDisplayClass) (Utilities|GetClass (Variables|/Game/UI/UW_Main.UW_Main_C|GetDisplayScreen _uw_main)))
            (CallFunction|UpdateSpeekSound (Variables|/Game/UI/UW_ComboBox.UW_ComboBox_C|GetCurrentTopicName (Variables|/Game/UI/UW_Main.UW_Main_C|GetUW_ComboBox _uw_main)))
            (else
              (CallFunction|UpdateSpeekSound))))))))

(fn OnAudioFinished
  (bind _subdirnames (Variables|Default|GetSubDirNames))
  (bind _soundindex (Variables|Default|GetSoundIndex))
  (if (and (< _soundindex (Utilities|Array|Length _subdirnames)) (Variables|Default|GetInBox))
    (if (not (Variables|Default|GetIsMute))
      (CallFunction|UpdateSpeekSound (Utilities|Array|Get(acopy) _subdirnames _soundindex)))))

(fn OnUWComboBoxCompleted
  (params (SubDirsNames :type Array%20of%20Strings))
  (Variables|Default|SetSubDirNames SubDirsNames))

(fn UpdateSpeekSound
  (params (Name :type String))
  (bind _gplayercontroller (CallFunction|GetGPlayerController))
  (bind _ghud (CallFunction|GetGHUD))
  (bind _audio (Variables|Default|GetAudio))
  (bind _sounds (Variables|Default|GetSounds))
  (bind _subdirnames (Variables|Default|GetSubDirNames))
  (bind _audio_2 (Variables|Default|GetAudio))
  (bind _returnvalue (Utilities|Array|FindItem _subdirnames Name))
  (bind _uw_main (Variables|/Game/GamePlay/GHUD.GHUD_C|GetUW_Main _ghud))
  (bind _uw_combobox (Variables|/Game/UI/UW_Main.UW_Main_C|GetUW_ComboBox _uw_main))
  (Utilities|IsValid _gplayercontroller
    (:Is%20Valid
      (if (not (Variables|/Game/GamePlay/GPlayerController.GPlayerController_C|GetMetahumenMute _gplayercontroller))
        (Utilities|FlowControl|Sequence
          (:then_0
            (Utilities|IsValid (Variables|Default|GetCurrentSound)
              (:Is%20Valid
                (Audio|Components|Audio|Stop (Variables|Default|GetAudio)))))
          (:then_1
            (if (== (Utilities|Array|Length (Variables|Default|GetSounds)) (Utilities|Array|Length (Variables|Default|GetAnimes)))
              (if (Utilities|Array|IsEmpty Name)
                (if (> (Utilities|Array|Length _sounds) 0)
                  (bind _output_get (Variables|Default|SetSoundIndex 0))
                  (bind _output_get_2 (Variables|Default|SetCurrentSound (Utilities|Array|Get(acopy) _sounds _output_get)))
                  (Audio|Components|Audio|SetSound _audio_2 _output_get_2)
                  (Audio|Components|Audio|Play _audio_2 0.0)
                  (Components|Animation|PlayAnimation (Variables|/Script/Engine.Character|GetMesh (Variables|Default|GetNarrator)) (Utilities|Array|Get(acopy) (Variables|Default|GetAnimes) (Variables|Default|GetSoundIndex)) false))
                (elif (and (>= _returnvalue 0) (< _returnvalue (Utilities|Array|Length (Variables|Default|GetSounds))))
                  (bind _output_get_3 (Variables|Default|SetSoundIndex _returnvalue))
                  (bind _output_get_4 (Variables|Default|SetCurrentSound (Utilities|Array|Get(acopy) (Variables|Default|GetSounds) _output_get_3)))
                  (Audio|Components|Audio|SetSound _audio _output_get_4)
                  (Audio|Components|Audio|Play _audio 0.0)
                  (Components|Animation|PlayAnimation (Variables|/Script/Engine.Character|GetMesh (Variables|Default|GetNarrator)) (Utilities|Array|Get(acopy) (Variables|Default|GetAnimes) (Variables|Default|GetSoundIndex)) false)))))
          (:then_2
            (Utilities|IsValid _ghud
              (:Is%20Valid
                (Utilities|IsValid _uw_main
                  (:Is%20Valid
                    (Utilities|IsValid _uw_combobox
                      (:Is%20Valid
                        (Default|SwitchTopic _uw_combobox Name))
                      (:Is%20Not%20Valid
                        _)))
                  (:Is%20Not%20Valid
                    _)))
              (:Is%20Not%20Valid
                _))
            (Math|Integer|IncrementInt (Variables|Default|GetSoundIndex)
              (:%20%20
                (bind _asdisplay_screen_robotic_arm (Utilities|Casting|CastToDisplayScreenRoboticArm (Variables|/Game/UI/UW_Main.UW_Main_C|GetDisplayScreen _uw_main)))
                (Components|Animation|PlayAnimation (Variables|/Game/Blueprints/Screen/DisplayScreenRoboticArm.DisplayScreenRoboticArm_C|GetRoboticArm _asdisplay_screen_robotic_arm) (.animtoplay (Variables|/Script/Engine.SkeletalMeshComponent|GetAnimationData (Variables|/Game/Blueprints/Screen/DisplayScreenRoboticArm.DisplayScreenRoboticArm_C|GetRoboticArm _asdisplay_screen_robotic_arm))) false))))
          (:then_3
            (if (Variables|/Game/GamePlay/GPlayerController.GPlayerController_C|GetMetahumenSpeekPause (CallFunction|GetGPlayerController))
              (CallFunction|OnMetahumenSpeekPause false))))))))

(fn ShowNarrator
  (params (Show :type Boolean))
  (bind _arrow (Variables|Default|GetArrow))
  (bind _narrator (Variables|Default|GetNarrator))
  (bind _returnvalue (Transformation|GetWorldTransform _arrow))
  (Utilities|IsValid _narrator
    (:Is%20Valid
      (if Show
        (Transformation|SetActorLocationAndRotation _narrator (.location _returnvalue) (.rotation _returnvalue))
        (else
          (Transformation|SetActorLocationAndRotation _narrator "0.000000,0.000000,-100.000000"))))))

(fn OtherBeginAction
  (bind _otherskelete (Variables|Default|GetOtherSkelete))
  (Utilities|IsValid _otherskelete
    (:Is%20Valid
      (Audio|Components|Audio|Play (Variables|/Script/Engine.SkeletalMeshActor|GetSkeletalMeshComponent _otherskelete) true))))

(fn OtherEndAction
  (bind _otherskelete (Variables|Default|GetOtherSkelete))
  (Utilities|IsValid _otherskelete
    (:Is%20Valid
      (Audio|Components|Audio|Stop (Variables|/Script/Engine.SkeletalMeshActor|GetSkeletalMeshComponent _otherskelete)))))

(fn OnMetahumenSpeekPause
  (params (Pause :type Boolean))
  (bind _narrator (Variables|Default|GetNarrator))
  (bind _mesh (Variables|/Script/Engine.Character|GetMesh _narrator))
  (Class|AudioComponent|SetPaused (Variables|Default|GetAudio) Pause)
  (Utilities|IsValid _narrator
    (:Is%20Valid
      (if Pause
        (Audio|Components|Audio|Stop _mesh)
        (else
          (Audio|Components|Audio|Play _mesh true))))))