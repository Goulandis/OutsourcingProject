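; PrefectPosition is a box trigger that marks a named area for the first-person character.
; Its construction script binds the box overlaps; on entry it writes PositionName to the main HUD widget and player controller and sets the widget's index to Index minus one.
; For the 智慧文旅区 (smart culture and tourism) area, entry also plays the referenced skeletal mesh's configured animation, and exit re-sets that animation without calling play.
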(event EventBeginPlay)

(event Collision|EventActorBeginOverlap
  (params (OtherActor :type Actor%20Object%20Reference)))

(event EventTick
  (params (DeltaSeconds :type Float%20%28single-precision%29)))

(fn ConstructionScript
  (bind _box (Variables|Default|GetBox))
  (Collision|BindEventtoOnComponentBeginOverlap _box (EventDispatchers|CreateEvent :!event OnBoxOverlapBegin))
  (Collision|BindEventtoOnComponentEndOverlap _box (EventDispatchers|CreateEvent :!event OnBoxOverlapEnd)))

(fn OnBoxOverlapBegin
  (params (OverlappedComponent :type Primitive%20Component%20Object%20Reference) (OtherActor :type Actor%20Object%20Reference) (OtherComp :type Primitive%20Component%20Object%20Reference) (OtherBodyIndex :type Integer) (bFromSweep :type Boolean) (SweepResult :type Hit%20Result%20Structure))
  (bind _ghud (CallFunction|GetGHUD))
  (bind _positionname (Variables|Default|GetPositionName))
  (bind _uw_main (Variables|/Game/GamePlay/GHUD.GHUD_C|GetUW_Main _ghud))
  (Utilities|Casting|CastToGFirstPersonCharacter OtherActor)
  (Utilities|FlowControl|Sequence
    (:then_0
      (Utilities|IsValid _uw_main
        (:Is%20Valid
          (Variables|/Script/UMG.TextBlock|SetText (Variables|/Game/UI/UW_Main.UW_Main_C|GetTXT_Position _uw_main) (Utilities|Text|ToText(Name) _positionname))
          (Variables|/Game/UI/UW_Main.UW_Main_C|SetIndex _uw_main (- (Variables|Default|GetIndex) 1))
          (Variables|/Game/GamePlay/GPlayerController.GPlayerController_C|SetCurrentPrefectPosition (CallFunction|GetGPlayerController) _positionname))))
    (:then_1
      (CallFunction|OtherOverlapBeginAction))))

(fn OtherOverlapBeginAction
  (bind _skeletalmesh (Variables|Default|GetSkeletalMesh))
  (bind _skeletalmeshcomponent (Variables|/Script/Engine.SkeletalMeshActor|GetSkeletalMeshComponent _skeletalmesh))
  (bind _animationdata (Variables|/Script/Engine.SkeletalMeshComponent|GetAnimationData _skeletalmeshcomponent))
  (switch name (Variables|Default|GetPositionName)
    (:智慧文旅区
      (Utilities|IsValid _skeletalmesh
        (:Is%20Valid
          (Components|Animation|PlayAnimation _skeletalmeshcomponent (.animtoplay _animationdata) (.bsavedlooping _animationdata)))))))

(fn OnBoxOverlapEnd
  (params (OverlappedComponent :type Primitive%20Component%20Object%20Reference) (OtherActor :type Actor%20Object%20Reference) (OtherComp :type Primitive%20Component%20Object%20Reference) (OtherBodyIndex :type Integer))
  (Utilities|Casting|CastToGFirstPersonCharacter OtherActor)
  (CallFunction|OtherOverlapEndAction))

(fn OtherOverlapEndAction
  (bind _skeletalmesh (Variables|Default|GetSkeletalMesh))
  (bind _skeletalmeshcomponent (Variables|/Script/Engine.SkeletalMeshActor|GetSkeletalMeshComponent _skeletalmesh))
  (switch name (Variables|Default|GetPositionName)
    (:智慧文旅区
      (Utilities|IsValid _skeletalmesh
        (:Is%20Valid
          (Components|Animation|SetAnimation _skeletalmeshcomponent (.animtoplay (Variables|/Script/Engine.SkeletalMeshComponent|GetAnimationData _skeletalmeshcomponent))))))))