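; In-world display screen that plays image slideshows or video, with paging and a UI view of the current content.
; Box overlap by the first-person character plays or pauses video and toggles HUD slideshow controls and a combo box of optional directories.
; Selected directories load at runtime as PNG textures or file media.
; Dynamic material instances feed both the screen mesh and UI.
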(event Custom|PauseMedia
  (params (Key :type String))
  (bind _mediaplayer (Variables|Default|GetMediaPlayer))
  (bind _mediasoundcomp (Variables|Default|GetMediaSoundComp))
  (if (not (Variables|/Game/GamePlay/GGameInstance.GGameInstance_C|GetInBox (CallFunction|GetGGameInstance)))
    (Utilities|IsValid _mediaplayer
      (:Is%20Valid
        (Utilities|FlowControl|Delay 2.0)
        (Sequencer|Player|Pause _mediaplayer)
        (Utilities|IsValid _mediasoundcomp
          (:Is%20Valid
            (Utilities|FlowControl|Delay 1.0)
            (Audio|Components|Audio|SetVolumeMultiplier _mediasoundcomp 1.0 :!class /Script/AudioMixer.SynthComponent)))))))

(event EventBeginPlay
  (bind _box (Variables|Default|GetBox))
  (Collision|BindEventtoOnComponentBeginOverlap _box (EventDispatchers|CreateEvent :!event OnBoxOverlapBegin))
  (Collision|BindEventtoOnComponentEndOverlap _box (EventDispatchers|CreateEvent :!event OnBoxOverlapEnd)))

(event EventTick
  (params (DeltaSeconds :type Float%20%28single-precision%29)))

(fn ConstructionScript)

(fn SetMaterial
  (params (Mat :type Material%20Instance%20Dynamic%20Object%20Reference))
  (Rendering|Material|SetMaterial (Variables|Default|GetScreen) 0 Mat))

(fn SetContent
  (params (Texs :type Array%20of%20Texture%202D%20Object%20References) (Mats :type Array%20of%20Material%20Instance%20Dynamic%20Object%20References) (MediaPlayers :type Media%20Player%20Object%20Reference) (MediaSource :type File%20Media%20Source%20Object%20Reference) (Type :type EDisplayType%20Enum :default "NewEnumerator0") (MediaTexure :type Media%20Texture%20Object%20Reference))
  (bind _mediasoundcomp (Variables|Default|GetMediaSoundComp))
  (Variables|Default|SetTexs Texs)
  (Variables|Default|SetMats Mats)
  (Variables|Default|SetMediaPlayer MediaPlayers)
  (Variables|Default|SetMediaSources MediaSource)
  (Variables|Default|SetDisplayType Type)
  (Variables|Default|SetMediaTexture MediaTexure)
  (Utilities|IsValid _mediasoundcomp
    (:Is%20Valid
      (Audio|Components|Audio|SetVolumeMultiplier _mediasoundcomp 0.0 :!class /Script/AudioMixer.SynthComponent))))

(fn OnBoxOverlapBegin
  (params (OverlappedComponent :type Primitive%20Component%20Object%20Reference) (OtherActor :type Actor%20Object%20Reference) (OtherComp :type Primitive%20Component%20Object%20Reference) (OtherBodyIndex :type Integer) (bFromSweep :type Boolean) (SweepResult :type Hit%20Result%20Structure%20%28by%20ref%29))
  (bind _ghud (CallFunction|GetGHUD))
  (bind _mediaplayer (Variables|Default|GetMediaPlayer))
  (bind _uw_main (Variables|/Game/GamePlay/GHUD.GHUD_C|GetUW_Main _ghud))
  (Utilities|Casting|CastToGFirstPersonCharacter OtherActor)
  (Variables|/Game/GamePlay/GGameInstance.GGameInstance_C|SetInBox (CallFunction|GetGGameInstance) true)
  (Variables|Default|SetInBox true)
  (if (Utilities|Array|IsEmpty (Variables|Default|GetOptionalDirs))
    _
    (else
      (CallFunction|ShowComboBox true)))
  (switch Utilities|FlowControl|Switch|SwitchonEPlayType (Variables|/Game/GamePlay/GHUD.GHUD_C|GetPlayType (CallFunction|GetGHUD))
    (:NewEnumerator0
      _)
    (:NewEnumerator2
      _))
  (switch Utilities|FlowControl|Switch|SwitchonEDisplayType (Variables|Default|GetDisplayType)
    (:NewEnumerator0
      (if (> (Utilities|Array|Length (Variables|Default|GetMats)) 1)
        (Utilities|IsValid _uw_main
          (:Is%20Valid
            (Widget|SetVisibility (Variables|/Game/UI/UW_Main.UW_Main_C|GetCanvas_PPT _uw_main) "Visible"))))
      (Variables|/Game/UI/UW_Main.UW_Main_C|SetDisplayScreen _uw_main self))
    (:NewEnumerator1
      (Utilities|IsValid _mediaplayer
        (:Is%20Valid
          (Media|MediaPlayer|Play _mediaplayer :!class /Script/MediaAssets.MediaPlayer)))))
  (Variables|/Game/GamePlay/GHUD.GHUD_C|SetPlayType (CallFunction|GetGHUD) "NewEnumerator2"))

(fn OnBoxOverlapEnd
  (params (OverlappedComponent :type Primitive%20Component%20Object%20Reference) (OtherActor :type Actor%20Object%20Reference) (OtherComp :type Primitive%20Component%20Object%20Reference) (OtherBodyIndex :type Integer))
  (bind _ghud (CallFunction|GetGHUD))
  (bind _ghud_2 (CallFunction|GetGHUD))
  (bind _ghud_3 (CallFunction|GetGHUD))
  (bind _mediaplayer (Variables|Default|GetMediaPlayer))
  (bind _uw_main (Variables|/Game/GamePlay/GHUD.GHUD_C|GetUW_Main _ghud))
  (Variables|/Game/GamePlay/GGameInstance.GGameInstance_C|SetInBox (CallFunction|GetGGameInstance) false)
  (Variables|Default|SetInBox false)
  (if (Utilities|Array|IsEmpty (Variables|Default|GetOptionalDirs))
    _
    (else
      (CallFunction|ShowComboBox false)))
  (Utilities|IsValid _ghud_3
    (:Is%20Valid
      (switch Utilities|FlowControl|Switch|SwitchonEPlayType (Variables|/Game/GamePlay/GHUD.GHUD_C|GetPlayType _ghud_3)
        (:NewEnumerator0
          _)
        (:NewEnumerator2
          _))
      (Utilities|FlowControl|Sequence
        (:then_0
          (Utilities|IsValid _ghud
            (:Is%20Valid
              (Utilities|IsValid _uw_main
                (:Is%20Valid
                  (Widget|SetVisibility (Variables|/Game/UI/UW_Main.UW_Main_C|GetCanvas_PPT _uw_main) "Hidden")
                  (Variables|/Game/UI/UW_Main.UW_Main_C|SetDisplayScreen _uw_main 0))))))
        (:then_1
          (switch Utilities|FlowControl|Switch|SwitchonEDisplayType (Variables|Default|GetDisplayType)
            (:NewEnumerator0
              _)
            (:NewEnumerator1
              (Utilities|IsValid _mediaplayer
                (:Is%20Valid
                  (Sequencer|Player|Pause _mediaplayer)))))))
      (Utilities|IsValid _ghud_2
        (:Is%20Valid
          (Variables|/Game/GamePlay/GHUD.GHUD_C|SetPlayType _ghud_2 "NewEnumerator0"))))))

(fn ShowPage
  (params (AllowPauseVideo :type Boolean) (Key :type String))
  (bind _mediaplayer (Variables|Default|GetMediaPlayer))
  (if (Utilities|Array|IsEmpty (Variables|Default|GetOptionalDirs))
    (switch Utilities|FlowControl|Switch|SwitchonEDisplayType (Variables|Default|GetDisplayType)
      (:NewEnumerator0
        (if (and (< (Variables|Default|GetPageIndex) (Utilities|Array|Length (Variables|Default|GetMats))) (>= (Variables|Default|GetPageIndex) 0))
          (CallFunction|SetMaterial (Utilities|Array|Get(acopy) (Variables|Default|GetMats) (Variables|Default|GetPageIndex)))
          (bind _returnvalue (Rendering|Material|CreateDynamicMaterialInstance "/Game/Blueprints/Screen/Materials/M_ScreenUIBase.M_ScreenUIBase" "None" "None" :!class /Script/Engine.KismetMaterialLibrary))
          (Rendering|Material|SetTextureParameterValue _returnvalue "Texture" (Utilities|Array|Get(acopy) (Variables|Default|GetTexs) (Variables|Default|GetPageIndex)))
          (Variables|Default|SetCurrentUIMat _returnvalue)))
      (:NewEnumerator1
        (bind _returnvalue_2 (Rendering|Material|CreateDynamicMaterialInstance "/Game/Blueprints/Screen/Materials/M_ScreenBase.M_ScreenBase" "None" "None" :!class /Script/Engine.KismetMaterialLibrary))
        (Rendering|Material|SetTextureParameterValue _returnvalue_2 "Texture" (Variables|Default|GetMediaTexture))
        (CallFunction|SetMaterial _returnvalue_2)
        (bind _returnvalue_3 (Rendering|Material|CreateDynamicMaterialInstance "/Game/Blueprints/Screen/Materials/M_ScreenUIBase.M_ScreenUIBase" "None" "None" :!class /Script/Engine.KismetMaterialLibrary))
        (Rendering|Material|SetTextureParameterValue _returnvalue_3 "Texture" (Variables|Default|GetMediaTexture))
        (Variables|Default|SetCurrentUIMat _returnvalue_3)
        (Utilities|IsValid _mediaplayer
          (:Is%20Valid
            (Media|MediaPlayer|OpenSource _mediaplayer (Variables|Default|GetMediaSources))
            (if AllowPauseVideo
              (CallFunction|PauseMedia))))))
    (else
      (CallFunction|InitOptionalContent AllowPauseVideo))))

(fn NextPage
  (bind _ghud (CallFunction|GetGHUD))
  (bind _uw_main (Variables|/Game/GamePlay/GHUD.GHUD_C|GetUW_Main _ghud))
  (bind _uw_contentshow (Variables|/Game/UI/UW_Main.UW_Main_C|GetUW_ContentShow _uw_main))
  (switch Utilities|FlowControl|Switch|SwitchonEDisplayType (Variables|Default|GetDisplayType)
    (:NewEnumerator0
      (bind _result (Math|Integer|IncrementInt (Variables|Default|GetPageIndex))
        (:%20%20
          (if (>= _result (Utilities|Array|Length (Variables|Default|GetMats)))
            (Variables|Default|SetPageIndex 0))
          (CallFunction|ShowPage true)
          (switch Utilities|FlowControl|Switch|SwitchonESlateVisibility (Widget|GetVisibility _uw_contentshow)
            (:Visible
              (Default|SetMat _uw_contentshow (Variables|Default|GetCurrentUIMat)))))))))

(fn LastPage
  (bind _ghud (CallFunction|GetGHUD))
  (bind _uw_main (Variables|/Game/GamePlay/GHUD.GHUD_C|GetUW_Main _ghud))
  (bind _uw_contentshow (Variables|/Game/UI/UW_Main.UW_Main_C|GetUW_ContentShow _uw_main))
  (switch Utilities|FlowControl|Switch|SwitchonEDisplayType (Variables|Default|GetDisplayType)
    (:NewEnumerator0
      (bind _result (Math|Integer|DecrementInt (Variables|Default|GetPageIndex))
        (:%20%20
          (if (< _result 0)
            (Variables|Default|SetPageIndex (- (Utilities|Array|Length (Variables|Default|GetMats)) 1)))
          (CallFunction|ShowPage true)
          (switch Utilities|FlowControl|Switch|SwitchonESlateVisibility (Widget|GetVisibility _uw_contentshow)
            (:Visible
              (Default|SetMat _uw_contentshow (Variables|Default|GetCurrentUIMat)))))))))

(fn ShowContent
  (bind _ghud (CallFunction|GetGHUD))
  (bind _self self)
  (bind _mediaplayer (Variables|Default|GetMediaPlayer))
  (bind _uw_main (Variables|/Game/GamePlay/GHUD.GHUD_C|GetUW_Main _ghud))
  (Utilities|IsValid _uw_main
    (:Is%20Valid
      (Variables|/Game/UI/UW_Main.UW_Main_C|SetDisplayScreen _uw_main _self)
      (Default|UpdateContent (Variables|/Game/UI/UW_Main.UW_Main_C|GetUW_ContentShow _uw_main) (Variables|Default|GetCurrentUIMat) _self (Variables|Default|GetUISize) (Variables|Default|GetUIPosition))
      (Default|ShowMediaTable _uw_main true)
      (switch Utilities|FlowControl|Switch|SwitchonEDisplayType (Variables|Default|GetDisplayType)
        (:NewEnumerator0
          _)
        (:NewEnumerator1
          (Utilities|IsValid _mediaplayer
            (:Is%20Valid
              (Media|MediaPlayer|Play _mediaplayer :!class /Script/MediaAssets.MediaPlayer)))))
      (Variables|/Game/GamePlay/GHUD.GHUD_C|SetPlayType (CallFunction|GetGHUD) "NewEnumerator1"))))

(fn UpdateOptionalContent
  (params (OptionalDir :type String))
  (bind _ghud (CallFunction|GetGHUD))
  (bind _ghud_2 (CallFunction|GetGHUD))
  (bind _mediaplayer (Variables|Default|GetMediaPlayer))
  (bind _optionaldirs (Variables|Default|GetOptionalDirs))
  (bind _mediaplayer_2 (Variables|Default|GetMediaPlayer))
  (bind _returnvalue (Utilities|Array|FindItem _optionaldirs OptionalDir))
  (bind _uw_main (Variables|/Game/GamePlay/GHUD.GHUD_C|GetUW_Main _ghud_2))
  (bind _uw_main_2 (Variables|/Game/GamePlay/GHUD.GHUD_C|GetUW_Main _ghud))
  (Variables|Default|SetPageIndex 0)
  (if (>= _returnvalue 0)
    (Variables|Default|SetOptionalIndex _returnvalue)
    (CallFunction|ShowPage true)
    (switch Utilities|FlowControl|Switch|SwitchonEDisplayType (Variables|Default|GetDisplayType)
      (:NewEnumerator0
        (Utilities|IsValid _uw_main_2
          (:Is%20Valid
            (Widget|SetVisibility (Variables|/Game/UI/UW_Main.UW_Main_C|GetCanvas_PPT _uw_main_2) "Visible")
            (Utilities|IsValid _mediaplayer_2
              (:Is%20Valid
                (Sequencer|Player|Pause _mediaplayer_2))))))
      (:NewEnumerator1
        (Utilities|IsValid _mediaplayer
          (:Is%20Valid
            (Media|MediaPlayer|Play _mediaplayer :!class /Script/MediaAssets.MediaPlayer)
            (Utilities|IsValid _uw_main
              (:Is%20Valid
                (Widget|SetVisibility (Variables|/Game/UI/UW_Main.UW_Main_C|GetCanvas_PPT _uw_main) "Hidden")))))))))

(fn InitOptionalContent
  (params (AllowPauseVideo :type Boolean))
  (bind _mats (Variables|Default|GetMats))
  (Utilities|Array|Clear (Variables|Default|GetTexs))
  (Utilities|Array|Clear (Variables|Default|GetMats))
  (Variables|Default|SetDisplayType "NewEnumerator2")
  (bind _returnvalue (Class|CommonFunLib|GetDirType (Variables|Default|GetOptionalDirs)))
  (bind _output_get (Variables|Default|SetDirTypeMap _returnvalue))
  (bind _keys (Utilities|Map|Keys _output_get))
  (LocalVariables|SetDir (Utilities|Array|Get(acopy) _keys (Variables|Default|GetOptionalIndex)))
  (Utilities|SwitchDirType (.Value (Utilities|Map|Find (Variables|Default|GetDirTypeMap) (Utilities|Array|Get(acopy) _keys (Variables|Default|GetOptionalIndex))))
    (:PPT
      (bind _returnvalue_2 (Class|CommonFunLib|GetAllSubdirectories (LocalVariables|GetDir)))
      (if (Utilities|Array|IsNotEmpty _returnvalue_2)
        (bind _texs (Class|CommonFunLib|LoadPNG2Texture (Utilities|Array|Get(acopy) _returnvalue_2)))
        (bind _output_get_2 (Variables|Default|SetTexs _texs))
        (for _array_element _output_get_2
          (bind _returnvalue_3 (Rendering|Material|CreateDynamicMaterialInstance "/Game/Blueprints/Screen/Materials/M_ScreenBase.M_ScreenBase" "None" "None" :!class /Script/Engine.KismetMaterialLibrary))
          (Rendering|Material|SetTextureParameterValue _returnvalue_3 "Texture" _array_element)
          (Utilities|Array|Add _mats _returnvalue_3))
        (CallFunction|SetMaterial (Utilities|Array|Get(acopy) _mats (Variables|Default|GetPageIndex)) :!label _label)
        (Variables|Default|SetDisplayType "NewEnumerator0")
        (bind _returnvalue_4 (Rendering|Material|CreateDynamicMaterialInstance "/Game/Blueprints/Screen/Materials/M_ScreenUIBase.M_ScreenUIBase" "None" "None" :!class /Script/Engine.KismetMaterialLibrary))
        (Rendering|Material|SetTextureParameterValue _returnvalue_4 "Texture" (Utilities|Array|Get(acopy) (Variables|Default|GetTexs) (Variables|Default|GetPageIndex)))
        (Variables|Default|SetCurrentUIMat _returnvalue_4)))
    (:Image
      (bind _texs_2 (Class|CommonFunLib|LoadPNG2Texture (LocalVariables|GetDir)))
      (bind _output_get_3 (Variables|Default|SetTexs _texs_2))
      (for _array_element_2 _output_get_3
        (bind _returnvalue_5 (Rendering|Material|CreateDynamicMaterialInstance "/Game/Blueprints/Screen/Materials/M_ScreenBase.M_ScreenBase" "None" "None" :!class /Script/Engine.KismetMaterialLibrary))
        (Rendering|Material|SetTextureParameterValue _returnvalue_5 "Texture" _array_element_2)
        (Utilities|Array|Add (Variables|Default|GetMats) _returnvalue_5))
      (goto _label))
    (:Video
      (bind _returnvalue_6 (Class|CommonFunLib|GetFilesfromDir (LocalVariables|GetDir)))
      (if (Utilities|Array|IsNotEmpty _returnvalue_6)
        (bind _returnvalue_7 (Game|ConstructObjectfromClass "/Script/MediaAssets.FileMediaSource"))
        (Class|FileMediaSource|SetFilePath _returnvalue_7 (Utilities|Array|Get(acopy) _returnvalue_6))
        (Variables|Default|SetMediaSources _returnvalue_7)
        (bind _returnvalue_8 (Game|ConstructObjectfromClass "/Script/MediaAssets.MediaPlayer"))
        (bind _output_get_4 (Variables|Default|SetMediaPlayer _returnvalue_8))
        (bind _returnvalue_9 (Game|ConstructObjectfromClass "/Script/MediaAssets.MediaTexture"))
        (Media|MediaSoundComponent|SetMediaPlayer _returnvalue_9 _output_get_4)
        (Class|MediaTexture|UpdateResource _returnvalue_9)
        (Variables|Default|SetMediaTexture _returnvalue_9)
        (bind _returnvalue_10 (Rendering|Material|CreateDynamicMaterialInstance "/Game/Blueprints/Screen/Materials/M_ScreenBase.M_ScreenBase" "None" "None" :!class /Script/Engine.KismetMaterialLibrary))
        (Rendering|Material|SetTextureParameterValue _returnvalue_10 "Texture" (Variables|Default|GetMediaTexture))
        (CallFunction|SetMaterial _returnvalue_10)
        (Variables|Default|SetDisplayType "NewEnumerator1")
        (bind _returnvalue_11 (Rendering|Material|CreateDynamicMaterialInstance "/Game/Blueprints/Screen/Materials/M_ScreenUIBase.M_ScreenUIBase" "None" "None" :!class /Script/Engine.KismetMaterialLibrary))
        (Rendering|Material|SetTextureParameterValue _returnvalue_11 "Texture" (Variables|Default|GetMediaTexture))
        (Variables|Default|SetCurrentUIMat _returnvalue_11)
        (Utilities|IsValid (Variables|Default|GetMediaPlayer)
          (:Is%20Valid
            (Media|MediaPlayer|OpenSource (Variables|Default|GetMediaPlayer) (Variables|Default|GetMediaSources))
            (if AllowPauseVideo
              (CallFunction|PauseMedia))))))))

(fn ShowComboBox
  (params (Show :type Boolean))
  (bind _ghud (CallFunction|GetGHUD))
  (bind _ghud_2 (CallFunction|GetGHUD))
  (bind _uw_main (Variables|/Game/GamePlay/GHUD.GHUD_C|GetUW_Main _ghud))
  (bind _uw_main_2 (Variables|/Game/GamePlay/GHUD.GHUD_C|GetUW_Main _ghud_2))
  (bind _uw_combobox (Variables|/Game/UI/UW_Main.UW_Main_C|GetUW_ComboBox _uw_main))
  (if (Utilities|Array|IsNotEmpty (Variables|Default|GetOptionalDirs))
    (if Show
      (Utilities|IsValid _ghud
        (:Is%20Valid
          (Utilities|IsValid _uw_main
            (:Is%20Valid
              (Widget|SetVisibility _uw_combobox "Visible")
              (Default|UpdateContent _uw_combobox (Variables|Default|GetOptionalDirs))
              (Variables|/Game/UI/UW_Main.UW_Main_C|SetDisplayScreen _uw_main self)))))
      (else
        (Utilities|IsValid _ghud_2
          (:Is%20Valid
            (Utilities|IsValid _ghud_2
              (:Is%20Valid
                (Utilities|IsValid _uw_main_2
                  (:Is%20Valid
                    (Widget|SetVisibility (Variables|/Game/UI/UW_Main.UW_Main_C|GetUW_ComboBox _uw_main_2) "Hidden")))))))))))