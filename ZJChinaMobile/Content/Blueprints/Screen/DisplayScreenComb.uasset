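; A child display screen that shows paged images and videos loaded at runtime from selectable DiyContents folders, with optional combined UI view via its trigger box.
; InitOptionalContent rebuilds per-page materials from disk textures or runtime-created media players, adding sound components only for Key "11".
; Page changes open video sources, swap the screen material and refresh visible UI content.
; SetMaterial also creates a matching UI material instance.
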(event EventBeginPlay
  (|CallParentFunction))

(event Collision|EventActorBeginOverlap
  (params (OtherActor :type Actor%20Object%20Reference)))

(event EventTick
  (params (DeltaSeconds :type Float%20%28single-precision%29))
  (|CallParentFunction DeltaSeconds) ; This node is disabled and will not be called.\nDrag off pins to build functionality.
)

(fn ConstructionScript
  (|CallParentFunction))

(fn GenerateOptionalDir
  (params (OptionalDir :type String))
  (bind _returnvalue (Utilities|String|ParseIntoArray OptionalDir "/"))
  (return (Utilities|String|Append (Class|KismetSystemLibrary|ConverttoAbsolutePath (Utilities|String|Append (Class|KismetSystemLibrary|GetProjectDirectory) "DiyContents")) "/" (Variables|Default|GetKey) "/" (Utilities|Array|Get(acopy) _returnvalue (Utilities|Array|LastIndex _returnvalue)))))

(fn UpdateOptionalContent
  (params (OptionalDir :type String))
  (bind _ghud (CallFunction|GetGHUD))
  (bind _ghud_2 (CallFunction|GetGHUD))
  (bind _result (CallFunction|GenerateOptionalDir OptionalDir))
  (bind _mediaplayer (Variables|Default|GetMediaPlayer))
  (bind _optionaldirs (Variables|Default|GetOptionalDirs))
  (bind _mediaplayer_2 (Variables|Default|GetMediaPlayer))
  (bind _returnvalue (Utilities|Array|FindItem _optionaldirs _result))
  (bind _uw_main (Variables|/Game/GamePlay/GHUD.GHUD_C|GetUW_Main _ghud_2))
  (bind _uw_main_2 (Variables|/Game/GamePlay/GHUD.GHUD_C|GetUW_Main _ghud))
  (Variables|Default|SetPageIndex 0)
  (if (>= _returnvalue 0)
    (Variables|Default|SetOptionalIndex _returnvalue)
    (Utilities|FlowControl|Sequence
      (:then_0
        (switch Utilities|FlowControl|Switch|SwitchonEDisplayType (Variables|Default|GetDisplayType)
          (:NewEnumerator0
            (Utilities|IsValid _uw_main_2
              (:Is%20Valid
                (Widget|SetVisibility (Variables|/Game/UI/UW_Main.UW_Main_C|GetCanvas_PPT _uw_main_2) "Visible")
                (Utilities|IsValid _mediaplayer_2
                  (:Is%20Valid
                    (Sequencer|Player|Pause _mediaplayer_2))))))
          (:NewEnumerator1
            (Utilities|IsValid _mediaplayer
              (:Is%20Valid
                (Media|MediaPlayer|Play _mediaplayer :!class /Script/MediaAssets.MediaPlayer)
                (Utilities|IsValid _uw_main
                  (:Is%20Valid
                    (Widget|SetVisibility (Variables|/Game/UI/UW_Main.UW_Main_C|GetCanvas_PPT _uw_main) "Hidden"))))))))
      (:then_1
        (CallFunction|ShowPage true)))))

(fn InitOptionalContent
  (params (AllowPauseVideo :type Boolean))
  (bind _trrigerbox (Variables|Default|GetTrrigerBox))
  (bind _mats (Variables|Default|GetMats))
  (bind _trrigerbox_2 (Variables|Default|GetTrrigerBox))
  (bind _keymediaplayers (Variables|Default|GetKeyMediaPlayers))
  (bind _keymediasources (Variables|Default|GetKeyMediaSources))
  (bind _optionaldirs (Variables|Default|GetOptionalDirs))
  (bind _mats_2 (Variables|Default|GetMats))
  (bind _ketmediasoundcomps (Variables|Default|GetKetMediaSoundComps))
  (bind _pageindex (Variables|Default|GetPageIndex))
  (bind _pageindex_2 (Variables|Default|GetPageIndex))
  (bind _pageindex_3 (Variables|Default|GetPageIndex))
  (bind (_value _returnvalue) (Utilities|Map|Find _keymediaplayers _pageindex_2))
  (bind _value_2 (Utilities|Map|Find _keymediasources _pageindex_2))
  (bind _keys (Utilities|Map|Keys _ketmediasoundcomps))
  (for _array_element _keys
    (Components|DestroyComponent (.Value (Utilities|Map|Find _ketmediasoundcomps _array_element))))
  (Utilities|Map|Clear _ketmediasoundcomps)
  (Utilities|Map|Clear (Variables|Default|GetKeyMediaSources))
  (Utilities|Map|Clear (Variables|Default|GetKeyMediaPlayers))
  (Utilities|Map|Clear (Variables|Default|GetKeyMediaTextures))
  (Utilities|Array|Clear (Variables|Default|GetMats))
  (Variables|Default|SetDisplayType "NewEnumerator2")
  (if (Utilities|Array|IsNotEmpty _optionaldirs)
    (bind _returnvalue_2 (Class|CommonFunLib|GetAllFilesfromDir (Utilities|Array|Get(acopy) _optionaldirs (Variables|Default|GetOptionalIndex))))
    (bind _keys_2 (Utilities|Map|Keys _returnvalue_2))
    (for (_array_element_2 _array_index) _keys_2
      (LocalVariables|SetCurrentFile _array_element_2)
      (LocalVariables|SetCurrentIndex _array_index)
      (switch string (.Value (Utilities|Map|Find _returnvalue_2 _array_element_2))
        (:Image
          (bind _returnvalue_3 (Class|CommonFunLib|LoadPNG2TexturefromFile (LocalVariables|GetCurrentFile)))
          (bind _returnvalue_4 (Rendering|Material|CreateDynamicMaterialInstance "/Game/Blueprints/Screen/Materials/M_ScreenBase.M_ScreenBase" "None" "None" :!class /Script/Engine.KismetMaterialLibrary))
          (Rendering|Material|SetTextureParameterValue _returnvalue_4 "Texture" _returnvalue_3)
          (Utilities|Array|Add (Variables|Default|GetMats) _returnvalue_4))
        (:Video
          (bind _returnvalue_5 (Game|ConstructObjectfromClass "/Script/MediaAssets.FileMediaSource"))
          (Class|FileMediaSource|SetFilePath _returnvalue_5 (LocalVariables|GetCurrentFile))
          (Utilities|Map|Add (Variables|Default|GetKeyMediaSources) (LocalVariables|GetCurrentIndex) _returnvalue_5)
          (bind _returnvalue_6 (Game|ConstructObjectfromClass "/Script/MediaAssets.MediaPlayer"))
          (bind _returnvalue_7 (Game|ConstructObjectfromClass "/Script/MediaAssets.MediaTexture"))
          (Media|MediaSoundComponent|SetMediaPlayer _returnvalue_7 _returnvalue_6)
          (Class|MediaTexture|UpdateResource _returnvalue_7)
          (Utilities|Map|Add (Variables|Default|GetKeyMediaTextures) (LocalVariables|GetCurrentIndex) _returnvalue_7)
          (Utilities|Map|Add (Variables|Default|GetKeyMediaPlayers) (LocalVariables|GetCurrentIndex) _returnvalue_6)
          (bind _returnvalue_8 (Rendering|Material|CreateDynamicMaterialInstance "/Game/Blueprints/Screen/Materials/M_ScreenBase.M_ScreenBase" "None" "None" :!class /Script/Engine.KismetMaterialLibrary))
          (Rendering|Material|SetTextureParameterValue _returnvalue_8 "Texture" _returnvalue_7)
          (Utilities|Array|Add (Variables|Default|GetMats) _returnvalue_8)
          (if (Utilities|Enum|Equal(Enum) (Variables|Default|GetKey) "11")
            (bind _returnvalue_9 (Game|AddComponentbyClass "/Script/MediaAssets.MediaSoundComponent" false))
            (Transformation|AttachComponentToComponent _returnvalue_9 (Variables|Default|GetDefaultSceneRoot) "None" "KeepRelative" "KeepRelative" "KeepRelative" true)
            (Audio|Components|Audio|SetVolumeMultiplier _returnvalue_9 1.0 :!class /Script/AudioMixer.SynthComponent)
            (Media|MediaSoundComponent|SetMediaPlayer _returnvalue_9 _returnvalue_6)
            (Utilities|Map|Add (Variables|Default|GetKetMediaSoundComps) (LocalVariables|GetCurrentIndex) _returnvalue_9)))))
    (if _returnvalue
      (if (> (Utilities|Array|Length _mats) _pageindex)
        (Variables|Default|SetDisplayType "NewEnumerator1")
        (CallFunction|SetMaterial (Utilities|Array|Get(acopy) _mats _pageindex))
        (Variables|Default|SetMediaPlayer _value)
        (Variables|Default|SetMediaSources _value_2)
        (Media|MediaPlayer|OpenSource _value _value_2)
        (CallFunction|PauseMedia)
        (Utilities|IsValid _trrigerbox
          (:Is%20Valid
            (Default|ShowPPTCanvas _trrigerbox false))))
      (elif (> (Utilities|Array|Length _mats_2) _pageindex_3)
        (Variables|Default|SetDisplayType "NewEnumerator0")
        (CallFunction|SetMaterial (Utilities|Array|Get(acopy) _mats_2 _pageindex_3))
        (if (Variables|/Game/GamePlay/GGameInstance.GGameInstance_C|GetInBox (CallFunction|GetGGameInstance))
          (Utilities|IsValid _trrigerbox_2
            (:Is%20Valid
              (Default|ShowPPTCanvas _trrigerbox_2 true))))))))

(fn NextPage
  (bind _ghud (CallFunction|GetGHUD))
  (bind _trrigerbox (Variables|Default|GetTrrigerBox))
  (bind _uw_main (Variables|/Game/GamePlay/GHUD.GHUD_C|GetUW_Main _ghud))
  (bind _uw_contentshow (Variables|/Game/UI/UW_Main.UW_Main_C|GetUW_ContentShow _uw_main))
  (bind _result (Math|Integer|IncrementInt (Variables|Default|GetPageIndex))
    (:%20%20
      (if (< _result (Utilities|Array|Length (Variables|Default|GetMats)))
        _
        (else
          (Variables|Default|SetPageIndex (Utilities|Array|LastIndex (Variables|Default|GetMats)))))
      (Utilities|CurrentMatType
        (:Video
          (Variables|Default|SetDisplayType "NewEnumerator1")
          (if (.ReturnValue (Utilities|Map|Find (Variables|Default|GetKeyMediaPlayers) (Variables|Default|GetPageIndex)))
            (Variables|Default|SetMediaPlayer (.Value (Utilities|Map|Find (Variables|Default|GetKeyMediaPlayers) (Variables|Default|GetPageIndex))))
            (Media|MediaPlayer|OpenSource (.Value (Utilities|Map|Find (Variables|Default|GetKeyMediaPlayers) (Variables|Default|GetPageIndex))) (.Value (Utilities|Map|Find (Variables|Default|GetKeyMediaSources) (Variables|Default|GetPageIndex))))
            (CallFunction|SetMaterial (Utilities|Array|Get(acopy) (Variables|Default|GetMats) (Variables|Default|GetPageIndex)) :!label _label)
            (switch Utilities|FlowControl|Switch|SwitchonESlateVisibility (Widget|GetVisibility _uw_contentshow)
              (:Visible
                (if (Variables|Default|GetAllowUIComb)
                  (Utilities|IsValid _trrigerbox
                    (:Is%20Valid
                      (Default|ShowContentComb _trrigerbox)))
                  (elif (== self (Variables|/Game/UI/UW_Main.UW_Main_C|GetDisplayScreen _uw_main))
                    (Default|SetMat _uw_contentshow (Variables|Default|GetCurrentUIMat))))))))
        (:Imge
          (Variables|Default|SetDisplayType "NewEnumerator0")
          (goto _label))))))

(fn LastPage
  (bind _ghud (CallFunction|GetGHUD))
  (bind _trrigerbox (Variables|Default|GetTrrigerBox))
  (bind _uw_main (Variables|/Game/GamePlay/GHUD.GHUD_C|GetUW_Main _ghud))
  (bind _uw_contentshow (Variables|/Game/UI/UW_Main.UW_Main_C|GetUW_ContentShow _uw_main))
  (bind _result (Math|Integer|DecrementInt (Variables|Default|GetPageIndex))
    (:%20%20
      (if (>= _result 0)
        _
        (else
          (Variables|Default|SetPageIndex 0)))
      (Utilities|CurrentMatType
        (:Video
          (Variables|Default|SetDisplayType "NewEnumerator1")
          (if (and (.ReturnValue (Utilities|Map|Find (Variables|Default|GetKeyMediaPlayers) (Variables|Default|GetPageIndex))) (.ReturnValue (Utilities|Map|Find (Variables|Default|GetKeyMediaSources) (Variables|Default|GetPageIndex))))
            (Variables|Default|SetMediaPlayer (.Value (Utilities|Map|Find (Variables|Default|GetKeyMediaPlayers) (Variables|Default|GetPageIndex))))
            (Media|MediaPlayer|OpenSource (.Value (Utilities|Map|Find (Variables|Default|GetKeyMediaPlayers) (Variables|Default|GetPageIndex))) (.Value (Utilities|Map|Find (Variables|Default|GetKeyMediaSources) (Variables|Default|GetPageIndex))))
            (CallFunction|SetMaterial (Utilities|Array|Get(acopy) (Variables|Default|GetMats) (Variables|Default|GetPageIndex)) :!label _label)
            (switch Utilities|FlowControl|Switch|SwitchonESlateVisibility (Widget|GetVisibility _uw_contentshow)
              (:Visible
                (if (Variables|Default|GetAllowUIComb)
                  (Utilities|IsValid _trrigerbox
                    (:Is%20Valid
                      (Default|ShowContentComb _trrigerbox)))
                  (elif (== self (Variables|/Game/UI/UW_Main.UW_Main_C|GetDisplayScreen _uw_main))
                    (Default|SetMat _uw_contentshow (Variables|Default|GetCurrentUIMat))))))))
        (:Imge
          (Variables|Default|SetDisplayType "NewEnumerator0")
          (goto _label))))))

(fn SetMaterial
  (params (Mat :type Material%20Instance%20Dynamic%20Object%20Reference))
  (Rendering|Material|SetMaterial (Variables|Default|GetScreen) 0 Mat)
  (switch Utilities|FlowControl|Switch|SwitchonEDisplayType (Variables|Default|GetDisplayType)
    (:NewEnumerator0
      (bind _returnvalue (Rendering|Material|CreateDynamicMaterialInstance "/Game/Blueprints/Screen/Materials/M_ScreenUIBase.M_ScreenUIBase" "None" "None" :!class /Script/Engine.KismetMaterialLibrary))
      (bind _returnvalue_2 (Rendering|Material|GetTextureParameterValue Mat "Texture" :!class /Script/Engine.MaterialInstanceDynamic))
      (Rendering|Material|SetTextureParameterValue _returnvalue "Texture" _returnvalue_2)
      (Variables|Default|SetCurrentUIMat _returnvalue))
    (:NewEnumerator1
      (bind _returnvalue_3 (Rendering|Material|CreateDynamicMaterialInstance "/Game/Blueprints/Screen/Materials/M_ScreenUIBase.M_ScreenUIBase" "None" "None" :!class /Script/Engine.KismetMaterialLibrary))
      (Rendering|Material|SetTextureParameterValue _returnvalue_3 "Texture" (.Value (Utilities|Map|Find (Variables|Default|GetKeyMediaTextures) (Variables|Default|GetPageIndex))))
      (Variables|Default|SetCurrentUIMat _returnvalue_3))))

(fn ShowContent
  (bind _trrigerbox (Variables|Default|GetTrrigerBox))
  (if (Variables|Default|GetAllowUIComb)
    (if (!= (Utilities|Array|LastIndex (Variables|Default|GetOptionalDirs)) (Variables|Default|GetOptionalIndex))
      (Utilities|IsValid _trrigerbox
        (:Is%20Valid
          (Default|ShowContentComb _trrigerbox)))
      (else
        (|CallParentFunction :!label _label)))
    (else
      (goto _label))))