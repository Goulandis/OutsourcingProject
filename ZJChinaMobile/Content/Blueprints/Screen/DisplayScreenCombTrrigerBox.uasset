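; Trigger box that controls a group of combined display screens as the first-person player enters or leaves it.
; Overlap toggles the combo box and PPT canvas, resets screen content on entry and pauses media on exit.
; HUD events fan out content changes and page switching to every linked screen.
; For the 智慧文旅区 area, ShowContentComb presents a screen pair side by side in the main widget, playing any video.
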(event EventBeginPlay
  (bind _ghud (CallFunction|GetGHUD))
  (EventDispatchers|BindEventtoOnChangedScreenContentbyCombTrriger _ghud (EventDispatchers|CreateEvent :!event OnChangedScreenContentbyCombTrriger))
  (EventDispatchers|BindEventtoOnSwitchPPTbyCombTrriger _ghud (EventDispatchers|CreateEvent :!event OnSwitchPPTbyCombTrriger))
  (for _array_element (Variables|Default|GetDisplayScreenCombs)
    (Variables|/Game/Blueprints/Screen/DisplayScreenComb.DisplayScreenComb_C|SetTrrigerBox _array_element self)))

(fn ConstructionScript
  (bind _box (Variables|Default|GetBox))
  (Collision|BindEventtoOnComponentBeginOverlap _box (EventDispatchers|CreateEvent :!event OnBoxOverlapBegin))
  (Collision|BindEventtoOnComponentEndOverlap _box (EventDispatchers|CreateEvent :!event OnBoxOverlapBoxEnd)))

(fn OnBoxOverlapBegin
  (params (OverlappedComponent :type Primitive%20Component%20Object%20Reference) (OtherActor :type Actor%20Object%20Reference) (OtherComp :type Primitive%20Component%20Object%20Reference) (OtherBodyIndex :type Integer) (bFromSweep :type Boolean) (SweepResult :type Hit%20Result%20Structure))
  (bind _displayscreencombs (Variables|Default|GetDisplayScreenCombs))
  (Utilities|Casting|CastToGFirstPersonCharacter OtherActor)
  (Variables|/Game/GamePlay/GGameInstance.GGameInstance_C|SetInBox (CallFunction|GetGGameInstance) true)
  (if (>= (Utilities|Array|Length _displayscreencombs) 0)
    (Default|ShowComboBox (Utilities|Array|Get(acopy) _displayscreencombs) true)
    (CallFunction|ShowPPTCanvas true)
    (for _array_element (Variables|Default|GetDisplayScreenCombs)
      (Variables|/Game/Blueprints/Screen/DisplayScreen.DisplayScreen_C|SetOptionalIndex _array_element 0)
      (Default|InitOptionalContent _array_element false))))

(fn OnBoxOverlapBoxEnd
  (params (OverlappedComponent :type Primitive%20Component%20Object%20Reference) (OtherActor :type Actor%20Object%20Reference) (OtherComp :type Primitive%20Component%20Object%20Reference) (OtherBodyIndex :type Integer))
  (bind _displayscreencombs (Variables|Default|GetDisplayScreenCombs))
  (Utilities|Casting|CastToGFirstPersonCharacter OtherActor)
  (Variables|/Game/GamePlay/GGameInstance.GGameInstance_C|SetInBox (CallFunction|GetGGameInstance) false)
  (if (>= (Utilities|Array|Length _displayscreencombs) 0)
    (Default|ShowComboBox (Utilities|Array|Get(acopy) _displayscreencombs) false)
    (CallFunction|ShowPPTCanvas false)
    (for _array_element (Variables|Default|GetDisplayScreenCombs)
      (Utilities|IsValid (Variables|/Game/Blueprints/Screen/DisplayScreen.DisplayScreen_C|GetMediaPlayer _array_element)
        (:Is%20Valid
          (Sequencer|Player|Pause (Variables|/Game/Blueprints/Screen/DisplayScreen.DisplayScreen_C|GetMediaPlayer _array_element)))))))

(fn OnChangedScreenContentbyCombTrriger
  (params (OptionalDir :type String))
  (bind _ghud (CallFunction|GetGHUD))
  (bind _uw_main (Variables|/Game/GamePlay/GHUD.GHUD_C|GetUW_Main _ghud))
  (bind _uw_contentshow (Variables|/Game/UI/UW_Main.UW_Main_C|GetUW_ContentShow _uw_main))
  (for _array_element (Variables|Default|GetDisplayScreenCombs)
    (Default|UpdateOptionalContent _array_element OptionalDir)
    (switch name (Variables|/Game/GamePlay/GPlayerController.GPlayerController_C|GetCurrentPrefectPosition (CallFunction|GetGPlayerController))
      (:智慧文旅区
        (switch Utilities|FlowControl|Switch|SwitchonESlateVisibility (Widget|GetVisibility _uw_contentshow)
          (:Visible
            (Widget|SetVisibility _uw_contentshow "Hidden")
            (Widget|SetVisibility (Variables|/Game/UI/UW_Main.UW_Main_C|GetBackgroundBlur _uw_main) "Hidden")
            (Widget|SetVisibility (Variables|/Game/UI/UW_ContentShow.UW_ContentShow_C|GetIMG_Content_L _uw_contentshow) "Hidden")
            (Widget|SetVisibility (Variables|/Game/UI/UW_ContentShow.UW_ContentShow_C|GetIMG_Content_R _uw_contentshow) "Hidden")
            (Default|ControllerPlayer (CallFunction|GetGPlayerController) true)))))))

(fn ShowPPTCanvas
  (params (Show :type Boolean))
  (bind _ghud (CallFunction|GetGHUD))
  (bind _ghud_2 (CallFunction|GetGHUD))
  (bind _ghud_3 (CallFunction|GetGHUD))
  (bind _uw_main (Variables|/Game/GamePlay/GHUD.GHUD_C|GetUW_Main _ghud))
  (bind _uw_main_2 (Variables|/Game/GamePlay/GHUD.GHUD_C|GetUW_Main _ghud_3))
  (bind _uw_main_3 (Variables|/Game/GamePlay/GHUD.GHUD_C|GetUW_Main _ghud_2))
  (if Show
    (bind _array_element (Utilities|Array|ForEachLoopwithBreak (Variables|Default|GetDisplayScreenCombs) :!label _label)
      (:LoopBody
        (if (> (Utilities|Array|Length (Variables|/Game/Blueprints/Screen/DisplayScreen.DisplayScreen_C|GetMats _array_element)) 1)
          (LocalVariables|SetIsShowPPTCanvas true)
          (LocalVariables|SetDisplayScreenCombsSelf _array_element)
          (goto _label Break)))
      (:Completed
        (if (LocalVariables|GetIsShowPPTCanvas)
          (Utilities|IsValid (LocalVariables|GetDisplayScreenCombsSelf)
            (:Is%20Valid
              (switch Utilities|FlowControl|Switch|SwitchonEDisplayType (Variables|/Game/Blueprints/Screen/DisplayScreen.DisplayScreen_C|GetDisplayType (LocalVariables|GetDisplayScreenCombsSelf))
                (:NewEnumerator0
                  (Utilities|IsValid _ghud_2
                    (:Is%20Valid
                      (Utilities|IsValid _uw_main_3
                        (:Is%20Valid
                          (Widget|SetVisibility (Variables|/Game/UI/UW_Main.UW_Main_C|GetCanvas_PPT _uw_main_3) "Visible")
                          (Utilities|IsValid (Variables|/Game/Blueprints/Screen/DisplayScreen.DisplayScreen_C|GetMediaPlayer (LocalVariables|GetDisplayScreenCombsSelf))
                            (:Is%20Valid
                              (Sequencer|Player|Pause (Variables|/Game/Blueprints/Screen/DisplayScreen.DisplayScreen_C|GetMediaPlayer (LocalVariables|GetDisplayScreenCombsSelf))))))))))
                (:NewEnumerator1
                  (Utilities|IsValid (Variables|/Game/Blueprints/Screen/DisplayScreen.DisplayScreen_C|GetMediaPlayer (LocalVariables|GetDisplayScreenCombsSelf))
                    (:Is%20Valid
                      (Utilities|IsValid _ghud
                        (:Is%20Valid
                          (Media|MediaPlayer|Play (Variables|/Game/Blueprints/Screen/DisplayScreen.DisplayScreen_C|GetMediaPlayer (LocalVariables|GetDisplayScreenCombsSelf)) :!class /Script/MediaAssets.MediaPlayer)
                          (Utilities|IsValid _uw_main
                            (:Is%20Valid
                              (Widget|SetVisibility (Variables|/Game/UI/UW_Main.UW_Main_C|GetCanvas_PPT _uw_main) "Hidden"))))))))))))))
    (else
      (Utilities|IsValid _ghud_3
        (:Is%20Valid
          (Utilities|IsValid _uw_main_2
            (:Is%20Valid
              (Widget|SetVisibility (Variables|/Game/UI/UW_Main.UW_Main_C|GetCanvas_PPT _uw_main_2) "Hidden"))))))))

(fn OnSwitchPPTbyCombTrriger
  (params (Type :type String))
  (switch string Type
    (:Next
      (for _array_element (Variables|Default|GetDisplayScreenCombs)
        (Default|NextPage _array_element)))
    (:Last
      (for _array_element_2 (Variables|Default|GetDisplayScreenCombs)
        (Default|LastPage _array_element_2)))))

(fn ShowContentComb
  (bind _ghud (CallFunction|GetGHUD))
  (bind _displayscreencombs (Variables|Default|GetDisplayScreenCombs))
  (bind _output (Utilities|Array|Get(acopy) _displayscreencombs))
  (bind _output_2 (Utilities|Array|Get(acopy) _displayscreencombs 1))
  (bind _uw_main (Variables|/Game/GamePlay/GHUD.GHUD_C|GetUW_Main _ghud))
  (bind _mediaplayer (Variables|/Game/Blueprints/Screen/DisplayScreen.DisplayScreen_C|GetMediaPlayer _output))
  (bind _mediaplayer_2 (Variables|/Game/Blueprints/Screen/DisplayScreen.DisplayScreen_C|GetMediaPlayer _output_2))
  (switch name (Variables|/Game/GamePlay/GPlayerController.GPlayerController_C|GetCurrentPrefectPosition (CallFunction|GetGPlayerController))
    (:智慧文旅区
      (if (== (Utilities|Array|Length (Variables|Default|GetDisplayScreenCombs)) 2)
        (Utilities|IsValid _uw_main
          (:Is%20Valid
            (Variables|/Game/UI/UW_Main.UW_Main_C|SetDisplayScreen _uw_main _output)
            (Default|UpdateContentComb (Variables|/Game/UI/UW_Main.UW_Main_C|GetUW_ContentShow _uw_main) (Variables|/Game/Blueprints/Screen/DisplayScreen.DisplayScreen_C|GetCurrentUIMat _output) (Variables|/Game/Blueprints/Screen/DisplayScreen.DisplayScreen_C|GetCurrentUIMat _output_2) _output "(X=1920.000000,Y=1248.000000)" "(X=-1920.000000,Y=-516.000000)" "(X=1920.000000,Y=1248.000000)" "(X=0.000000,Y=-516.000000)")
            (Default|ShowMediaTable _uw_main true)
            (Utilities|FlowControl|Sequence
              (:then_0
                (switch Utilities|FlowControl|Switch|SwitchonEDisplayType (Variables|/Game/Blueprints/Screen/DisplayScreen.DisplayScreen_C|GetDisplayType _output)
                  (:NewEnumerator0
                    _)
                  (:NewEnumerator1
                    (Utilities|IsValid _mediaplayer
                      (:Is%20Valid
                        (Media|MediaPlayer|Play _mediaplayer :!class /Script/MediaAssets.MediaPlayer)))))
                (Variables|/Game/GamePlay/GHUD.GHUD_C|SetPlayType (CallFunction|GetGHUD) "NewEnumerator1"))
              (:then_1
                (switch Utilities|FlowControl|Switch|SwitchonEDisplayType (Variables|/Game/Blueprints/Screen/DisplayScreen.DisplayScreen_C|GetDisplayType _output_2)
                  (:NewEnumerator0
                    _)
                  (:NewEnumerator1
                    (Utilities|IsValid _mediaplayer_2
                      (:Is%20Valid
                        (Media|MediaPlayer|Play _mediaplayer_2 :!class /Script/MediaAssets.MediaPlayer)))))
                (Variables|/Game/GamePlay/GHUD.GHUD_C|SetPlayType (CallFunction|GetGHUD) "NewEnumerator1")))))))))