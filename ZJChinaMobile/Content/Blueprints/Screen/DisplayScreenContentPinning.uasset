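; Display screen that pages through images and videos loaded at runtime from a left or right DiyContents folder, chosen by its Position.
; Init turns each file into a dynamic screen material, with a media source, player and texture per video.
; A leading video opens under a near-muted sound component, then PauseMedia pauses it after a delay and restores volume.
; NextPage and LastPage swap materials and open that page's video.
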(event Custom|PauseMedia
  (params (Index :type Integer))
  (bind _keymediaplayers (Variables|Default|GetKeyMediaPlayers))
  (bind _mediasoundcomp (Variables|Default|GetMediaSoundComp))
  (bind (_value _returnvalue) (Utilities|Map|Find _keymediaplayers Index))
  (if _returnvalue
    (Utilities|FlowControl|Delay 2.0)
    (Sequencer|Player|Pause _value)
    (Utilities|IsValid _mediasoundcomp
      (:Is%20Valid
        (Utilities|FlowControl|Delay 1.0)
        (Audio|Components|Audio|SetVolumeMultiplier _mediasoundcomp 1.0 :!class /Script/AudioMixer.SynthComponent)))))

(event EventBeginPlay
  (CallFunction|Init))

(event EventTick
  (params (DeltaSeconds :type Float%20%28single-precision%29)))

(fn ConstructionScript)

(fn Init
  (bind _mats (Variables|Default|GetMats))
  (bind _keymediaplayers (Variables|Default|GetKeyMediaPlayers))
  (bind (_value _returnvalue) (Utilities|Map|Find _keymediaplayers 0))
  (switch string (Variables|Default|GetPosition)
    (:Left
      (LocalVariables|SetDir (Class|KismetSystemLibrary|ConverttoAbsolutePath (Utilities|String|Append (Class|KismetSystemLibrary|GetProjectDirectory) "DiyContents/Content11/MediaLeft"))))
    (:Right
      (LocalVariables|SetDir (Class|KismetSystemLibrary|ConverttoAbsolutePath (Utilities|String|Append (Class|KismetSystemLibrary|GetProjectDirectory) "DiyContents/Content11/MediaRight")))))
  (bind _returnvalue_2 (Class|CommonFunLib|GetAllFilesfromDir (LocalVariables|GetDir)))
  (bind _keys (Utilities|Map|Keys _returnvalue_2))
  (for (_array_element _array_index) _keys
    (LocalVariables|SetCurrentFile _array_element)
    (LocalVariables|SetCurrentIndex _array_index)
    (switch string (.Value (Utilities|Map|Find _returnvalue_2 _array_element))
      (:Image
        (bind _returnvalue_3 (Class|CommonFunLib|LoadPNG2TexturefromFile (LocalVariables|GetCurrentFile)))
        (bind _returnvalue_4 (Rendering|Material|CreateDynamicMaterialInstance "/Game/Blueprints/Screen/Materials/M_ScreenBase.M_ScreenBase" "None" "None" :!class /Script/Engine.KismetMaterialLibrary))
        (Rendering|Material|SetTextureParameterValue _returnvalue_4 "Texture" _returnvalue_3)
        (Utilities|Array|Add (Variables|Default|GetMats) _returnvalue_4))
      (:Video
        (bind _returnvalue_5 (Game|ConstructObjectfromClass "/Script/MediaAssets.FileMediaSource"))
        (Class|FileMediaSource|SetFilePath _returnvalue_5 (LocalVariables|GetCurrentFile))
        (Utilities|Map|Add (Variables|Default|GetKeyMediaSources) (LocalVariables|GetCurrentIndex) _returnvalue_5)
        (bind _returnvalue_6 (Game|ConstructObjectfromClass "/Script/MediaAssets.MediaPlayer"))
        (bind _returnvalue_7 (Game|ConstructObjectfromClass "/Script/MediaAssets.MediaTexture"))
        (Media|MediaSoundComponent|SetMediaPlayer _returnvalue_7 _returnvalue_6)
        (Class|MediaTexture|UpdateResource _returnvalue_7)
        (Utilities|Map|Add (Variables|Default|GetKeyMediaPlayers) (LocalVariables|GetCurrentIndex) _returnvalue_6)
        (bind _returnvalue_8 (Rendering|Material|CreateDynamicMaterialInstance "/Game/Blueprints/Screen/Materials/M_ScreenBase.M_ScreenBase" "None" "None" :!class /Script/Engine.KismetMaterialLibrary))
        (Rendering|Material|SetTextureParameterValue _returnvalue_8 "Texture" _returnvalue_7)
        (Utilities|Array|Add (Variables|Default|GetMats) _returnvalue_8)
        (Utilities|IsValid (Variables|Default|GetMediaSoundComp)
          (:Is%20Not%20Valid
            (bind _returnvalue_9 (Game|AddComponentbyClass "/Script/MediaAssets.MediaSoundComponent" false))
            (Transformation|AttachComponentToComponent _returnvalue_9 (Variables|Default|GetDefaultSceneRoot) "None" "KeepRelative" "KeepRelative" "KeepRelative" true)
            (bind _output_get (Variables|Default|SetMediaSoundComp _returnvalue_9))
            (Audio|Components|Audio|SetVolumeMultiplier _output_get 0.001 :!class /Script/AudioMixer.SynthComponent))))))
  (if (> (Utilities|Array|Length _mats) 0)
    (Rendering|Material|SetMaterial (Variables|Default|GetScreen) 0 (Utilities|Array|Get(acopy) _mats))
    (Variables|Default|SetDisplayType "NewEnumerator0")
    (if _returnvalue
      (Variables|Default|SetCurrentMediaPlayer _value)
      (Media|MediaPlayer|OpenSource _value (.Value (Utilities|Map|Find (Variables|Default|GetKeyMediaSources) 0)))
      (Variables|Default|SetDisplayType "NewEnumerator1")
      (CallFunction|PauseMedia))))

(fn NextPage
  (bind _result (Math|Integer|IncrementInt (Variables|Default|GetPageIndex))
    (:%20%20
      (if (< _result (- (Utilities|Array|Length (Variables|Default|GetMats)) 1))
        _
        (else
          (Variables|Default|SetPageIndex 0)))
      (Rendering|Material|SetMaterial (Variables|Default|GetScreen) 0 (Utilities|Array|Get(acopy) (Variables|Default|GetMats) (Variables|Default|GetPageIndex)))
      (Variables|Default|SetDisplayType "NewEnumerator0")
      (if (.ReturnValue (Utilities|Map|Find (Variables|Default|GetKeyMediaPlayers) (Variables|Default|GetPageIndex)))
        (Variables|Default|SetCurrentMediaPlayer (.Value (Utilities|Map|Find (Variables|Default|GetKeyMediaPlayers) (Variables|Default|GetPageIndex))))
        (Media|MediaPlayer|OpenSource (.Value (Utilities|Map|Find (Variables|Default|GetKeyMediaPlayers) (Variables|Default|GetPageIndex))) (.Value (Utilities|Map|Find (Variables|Default|GetKeyMediaSources) (Variables|Default|GetPageIndex))))
        (Variables|Default|SetDisplayType "NewEnumerator1")
        (else
          (Variables|Default|SetCurrentMediaPlayer 0))))))

(fn LastPage
  (bind _result (Math|Integer|DecrementInt (Variables|Default|GetPageIndex))
    (:%20%20
      (if (>= _result 0)
        _
        (else
          (Variables|Default|SetPageIndex 0)))
      (Rendering|Material|SetMaterial (Variables|Default|GetScreen) 0 (Utilities|Array|Get(acopy) (Variables|Default|GetMats) (Variables|Default|GetPageIndex)))
      (Variables|Default|SetDisplayType "NewEnumerator0")
      (if (.ReturnValue (Utilities|Map|Find (Variables|Default|GetKeyMediaPlayers) (Variables|Default|GetPageIndex)))
        (Variables|Default|SetCurrentMediaPlayer (.Value (Utilities|Map|Find (Variables|Default|GetKeyMediaPlayers) (Variables|Default|GetPageIndex))))
        (Media|MediaPlayer|OpenSource (.Value (Utilities|Map|Find (Variables|Default|GetKeyMediaPlayers) (Variables|Default|GetPageIndex))) (.Value (Utilities|Map|Find (Variables|Default|GetKeyMediaSources) (Variables|Default|GetPageIndex))))
        (Variables|Default|SetDisplayType "NewEnumerator1")
        (else
          (Variables|Default|SetCurrentMediaPlayer 0))))))

(fn ShowComboBox)