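; Trigger box for display screens that flags in the game instance whether the first-person player is inside.
; Entering only prints each linked screen's material count; leaving hides the HUD's PPT canvas and pauses the screens' media players.
; HUD events for content changes and page switching are bound on BeginPlay, but their handlers are empty.
; The logic for paging, content updates and image-versus-video display is left disconnected.
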(event EventBeginPlay
  (bind _ghud (CallFunction|GetGHUD))
  (EventDispatchers|BindEventtoOnChangedScreenContentbyCombTrriger _ghud (EventDispatchers|CreateEvent :!event OnChangedScreenContentbyCombTrriger))
  (EventDispatchers|BindEventtoOnSwitchPPTbyCombTrriger _ghud (EventDispatchers|CreateEvent :!event OnSwitchPPTbyCombTrriger)))

(fn ConstructionScript
  (bind _box (Variables|Default|GetBox))
  (Collision|BindEventtoOnComponentBeginOverlap _box (EventDispatchers|CreateEvent :!event OnBoxOverlapBegin))
  (Collision|BindEventtoOnComponentEndOverlap _box (EventDispatchers|CreateEvent :!event OnBoxOverlapBoxEnd)))

(fn OnBoxOverlapBegin
  (params (OverlappedComponent :type Primitive%20Component%20Object%20Reference) (OtherActor :type Actor%20Object%20Reference) (OtherComp :type Primitive%20Component%20Object%20Reference) (OtherBodyIndex :type Integer) (bFromSweep :type Boolean) (SweepResult :type Hit%20Result%20Structure))
  (Utilities|Casting|CastToGFirstPersonCharacter OtherActor)
  (Variables|/Game/GamePlay/GGameInstance.GGameInstance_C|SetInBox (CallFunction|GetGGameInstance) true)
  (CallFunction|ShowPPTCanvas true))

(fn OnBoxOverlapBoxEnd
  (params (OverlappedComponent :type Primitive%20Component%20Object%20Reference) (OtherActor :type Actor%20Object%20Reference) (OtherComp :type Primitive%20Component%20Object%20Reference) (OtherBodyIndex :type Integer))
  (Utilities|Casting|CastToGFirstPersonCharacter OtherActor)
  (Variables|/Game/GamePlay/GGameInstance.GGameInstance_C|SetInBox (CallFunction|GetGGameInstance) false)
  (CallFunction|ShowPPTCanvas false))

(fn OnChangedScreenContentbyCombTrriger
  (params (OptionalDir :type String)))

(fn ShowPPTCanvas
  (params (Show :type Boolean))
  (bind _ghud (CallFunction|GetGHUD))
  (bind _uw_main (Variables|/Game/GamePlay/GHUD.GHUD_C|GetUW_Main _ghud))
  (if Show
    (bind _array_element (Utilities|Array|ForEachLoopwithBreak (Variables|Default|GetDisplayScreenCombs))
      (:LoopBody
        (Development|PrintString (Utilities|String|ToString(Integer) (Utilities|Array|Length (Variables|/Game/Blueprints/Screen/DisplayScreenContentPinning.DisplayScreenContentPinning_C|GetMats _array_element))))))
    (else
      (Utilities|FlowControl|Sequence
        (:then_0
          (Utilities|IsValid _ghud
            (:Is%20Valid
              (Utilities|IsValid _uw_main
                (:Is%20Valid
                  (Widget|SetVisibility (Variables|/Game/UI/UW_Main.UW_Main_C|GetCanvas_PPT _uw_main) "Hidden"))))))
        (:then_1
          (for _array_element_2 (Variables|Default|GetDisplayScreenCombs)
            (Utilities|IsValid (Variables|/Game/Blueprints/Screen/DisplayScreenContentPinning.DisplayScreenContentPinning_C|GetCurrentMediaPlayer _array_element_2)
              (:Is%20Valid
                (Sequencer|Player|Pause (Variables|/Game/Blueprints/Screen/DisplayScreenContentPinning.DisplayScreenContentPinning_C|GetCurrentMediaPlayer _array_element_2))))))))))

(fn OnSwitchPPTbyCombTrriger
  (params (Type :type String)))