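; An interactive display screen actor that shows image or video content and drives related canvases on the main HUD widget.
; ShowContent registers the screen on that widget and shows it, unless a DisplayScreenInteractive is already registered.
; ShowScreen toggles the screen and cancel canvas, reveals the PPT canvas for images, and plays or pauses the media player for video.
; The construction script starts the screen hidden.
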(event EventBeginPlay
  (|CallParentFunction) ; This node is disabled and will not be called.\nDrag off pins to build functionality.
)

(event Collision|EventActorBeginOverlap
  (params (OtherActor :type Actor%20Object%20Reference)))

(event EventTick
  (params (DeltaSeconds :type Float%20%28single-precision%29))
  (|CallParentFunction DeltaSeconds) ; This node is disabled and will not be called.\nDrag off pins to build functionality.
)

(fn ConstructionScript
  (|CallParentFunction)
  (CallFunction|ShowScreen false))

(fn ShowScreen
  (params (Show :type Boolean))
  (bind _ghud (CallFunction|GetGHUD))
  (bind _ghud_2 (CallFunction|GetGHUD))
  (bind _mediaplayer (Variables|Default|GetMediaPlayer))
  (bind _mediaplayer_2 (Variables|Default|GetMediaPlayer))
  (bind _uw_main (Variables|/Game/GamePlay/GHUD.GHUD_C|GetUW_Main _ghud))
  (bind _uw_main_2 (Variables|/Game/GamePlay/GHUD.GHUD_C|GetUW_Main _ghud_2))
  (bind _canvas_cancle (Variables|/Game/UI/UW_Main.UW_Main_C|GetCanvas_Cancle _uw_main_2))
  (Development|SetHiddeninGame (Variables|Default|GetScreen) (not Show) false)
  (Utilities|IsValid _uw_main_2
    (:Is%20Valid
      (Utilities|IsValid _canvas_cancle
        (:Is%20Valid
          (if Show
            (Widget|SetVisibility _canvas_cancle "Visible")
            (switch Utilities|FlowControl|Switch|SwitchonEDisplayType (Variables|Default|GetDisplayType)
              (:NewEnumerator0
                (Utilities|IsValid _uw_main
                  (:Is%20Valid
                    (Widget|SetVisibility (Variables|/Game/UI/UW_Main.UW_Main_C|GetCanvas_PPT _uw_main) "Visible"))))
              (:NewEnumerator1
                (Utilities|IsValid _mediaplayer_2
                  (:Is%20Valid
                    (Media|MediaPlayer|Play _mediaplayer_2 :!class /Script/MediaAssets.MediaPlayer)))))
            (else
              (Widget|SetVisibility _canvas_cancle "Hidden")
              (switch Utilities|FlowControl|Switch|SwitchonEDisplayType (Variables|Default|GetDisplayType)
                (:NewEnumerator1
                  (Utilities|IsValid _mediaplayer
                    (:Is%20Valid
                      (Sequencer|Player|Pause _mediaplayer))))))))))))

(fn ShowContent
  (bind _ghud (CallFunction|GetGHUD))
  (bind _uw_main (Variables|/Game/GamePlay/GHUD.GHUD_C|GetUW_Main _ghud))
  (Utilities|IsValid _uw_main
    (:Is%20Valid
      (Utilities|Casting|CastToDisplayScreenInteractive (Variables|/Game/UI/UW_Main.UW_Main_C|GetDisplayScreen _uw_main)
        (:CastFailed
          (Variables|/Game/UI/UW_Main.UW_Main_C|SetDisplayScreen _uw_main self)
          (CallFunction|ShowScreen true))))))