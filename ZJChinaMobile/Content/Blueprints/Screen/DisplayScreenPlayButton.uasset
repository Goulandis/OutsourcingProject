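; Play/pause button actor for a display screen, toggling its media playback when clicked.
; OnMouseClicked checks the linked DisplayScreen's MediaPlayer and calls Pause or Play on that screen.
; Its own Play and Pause functions swap the plane's material between play and pause versions, and Show toggles visibility.
; BeginPlay creates a dynamic play-button material with a texture but never assigns it to the plane.
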(event EventBeginPlay
  (bind _returnvalue (Rendering|Material|CreateDynamicMaterialInstance "/Game/Blueprints/Screen/Materials/M_DisplayScreenPlayButton.M_DisplayScreenPlayButton" "None" "None" :!class /Script/Engine.KismetMaterialLibrary))
  (Rendering|Material|SetTextureParameterValue _returnvalue "Texture" "/Game/UI/Textures/播放.播放"))

(fn ConstructionScript)

(fn Play
  (Rendering|Material|SetMaterial (Variables|Default|GetPlane) 0 "/Game/Blueprints/Screen/Materials/M_DisplayScreenPlayButton.M_DisplayScreenPlayButton"))

(fn Pause
  (Rendering|Material|SetMaterial (Variables|Default|GetPlane) 0 "/Game/Blueprints/Screen/Materials/M_DisplayScreenPauseButton.M_DisplayScreenPauseButton"))

(fn OnMouseClicked
  (bind _displayscreen (Variables|Default|GetDisplayScreen))
  (Utilities|IsValid _displayscreen
    (:Is%20Valid
      (if (Audio|Components|Audio|IsPlaying (Variables|/Game/Blueprints/Screen/DisplayScreen.DisplayScreen_C|GetMediaPlayer _displayscreen))
        (Default|Pause _displayscreen)
        (else
          (Default|Play _displayscreen))))))

(fn Show
  (params (Show :type Boolean))
  (Rendering|SetActorHiddenInGame (not Show)))