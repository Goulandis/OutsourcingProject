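; Display screen actor for a robotic arm whose keyed material slots show image pages or videos.
; Content is either preset per key or loaded from project DiyContents folders at runtime, building dynamic materials, media players and sound components.
; A box overlap by the first-person character animates the arm and, for optional content, toggles a combo box and media playback.
; Selecting a folder refreshes the screens and, if visible, the three-panel HUD view.
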(event EventBeginPlay
  (|CallParentFunction) ; This node is disabled and will not be called.\nDrag off pins to build functionality.
)

(event Collision|EventActorBeginOverlap
  (params (OtherActor :type Actor%20Object%20Reference)))

(event EventTick
  (params (DeltaSeconds :type Float%20%28single-precision%29))
  (|CallParentFunction DeltaSeconds) ; This node is disabled and will not be called.\nDrag off pins to build functionality.
)

(event EventPauseMedia
  (params (Key :type String))
  (bind _keysoundcompsmap (Variables|Default|GetKeySoundCompsMap))
  (bind _keymediaplayersmap (Variables|Default|GetKeyMediaPlayersMap))
  (bind _value (Utilities|Map|Find _keymediaplayersmap Key))
  (bind _value_2 (Utilities|Map|Find _keysoundcompsmap Key))
  (Utilities|IsValid _value
    (:Is%20Valid
      (Utilities|FlowControl|Delay 2.0)
      (Sequencer|Player|Pause _value)
      (Utilities|IsValid _value_2
        (:Is%20Valid
          (Utilities|FlowControl|Delay 1.0)
          (Audio|Components|Audio|SetVolumeMultiplier _value_2 1.0 :!class /Script/AudioMixer.SynthComponent))))))

(fn ConstructionScript
  (|CallParentFunction))

(fn ShowPage
  (params (AllowPauseVideo :type Boolean) (Key :type String))
  (if (Utilities|Array|IsEmpty (Variables|Default|GetOptionalDirs))
    (for _array_element (Variables|Default|GetTextsAndMatsForKey)
      (switch Utilities|FlowControl|Switch|SwitchonEDisplayType (.DisplayType (Utilities|Struct|BreakSDisplayTexsAndMats _array_element))
        (:NewEnumerator0
          (if (and (< (Variables|Default|GetPageIndex) (Utilities|Array|Length (.Mats (Utilities|Struct|BreakSDisplayTexsAndMats _array_element)))) (>= (Variables|Default|GetPageIndex) 0))
            (Rendering|Material|SetMaterial (Variables|Default|GetRoboticArm) (.Value (Utilities|Map|Find (Variables|Default|GetKeyForMatIndex) (.Key (Utilities|Struct|BreakSDisplayTexsAndMats _array_element)))) (Utilities|Array|Get(acopy) (.Mats (Utilities|Struct|BreakSDisplayTexsAndMats _array_element)) (Variables|Default|GetPageIndex)))))
        (:NewEnumerator1
          (bind _returnvalue (Rendering|Material|CreateDynamicMaterialInstance 0 "None" "None" :!class /Script/Engine.KismetMaterialLibrary))
          (Rendering|Material|SetTextureParameterValue _returnvalue "Texture" (.MediaTexture (Utilities|Struct|BreakSDisplayTexsAndMats _array_element)))
          (Rendering|Material|SetMaterial (Variables|Default|GetRoboticArm) (.Value (Utilities|Map|Find (Variables|Default|GetKeyForMatIndex) (.Key (Utilities|Struct|BreakSDisplayTexsAndMats _array_element)))) _returnvalue)
          (Utilities|IsValid (.MediaPlayer (Utilities|Struct|BreakSDisplayTexsAndMats _array_element))
            (:Is%20Valid
              (Media|MediaPlayer|OpenSource (.MediaPlayer (Utilities|Struct|BreakSDisplayTexsAndMats _array_element)) (.MediaSource (Utilities|Struct|BreakSDisplayTexsAndMats _array_element)))
              (Media|MediaPlayer|Play (.MediaPlayer (Utilities|Struct|BreakSDisplayTexsAndMats _array_element)) :!class /Script/MediaAssets.MediaPlayer))))))
    (else
      (CallFunction|InitOptionalContent AllowPauseVideo))))

(fn SetTexsandMatsbyKey
  (params (Key :type String) (Texs :type Array%20of%20Texture%202D%20Object%20References) (DisplayType :type EDisplayType%20Enum :default "NewEnumerator0"))
  (switch Utilities|FlowControl|Switch|SwitchonEDisplayType DisplayType
    (:NewEnumerator0
      (Utilities|Array|Clear (LocalVariables|GetMats))
      (for (_array_element _array_index) (Variables|Default|GetTextsAndMatsForKey)
        (if (Utilities|Enum|Equal(Enum) Key (.Key (Utilities|Struct|BreakSDisplayTexsAndMats _array_element)))
          (for _array_element_2 Texs
            (bind _returnvalue (Rendering|Material|CreateDynamicMaterialInstance 0 "None" "None" :!class /Script/Engine.KismetMaterialLibrary))
            (Rendering|Material|SetTextureParameterValue _returnvalue "Texture" _array_element_2)
            (Utilities|Array|Add (LocalVariables|GetMats) _returnvalue))
          (Utilities|Array|SetArrayElem (Variables|Default|GetTextsAndMatsForKey) _array_index (Utilities|Struct|MakeSDisplayTexsAndMats (.Key (Utilities|Struct|BreakSDisplayTexsAndMats _array_element)) Texs (LocalVariables|GetMats) "NewEnumerator0" 0 0 0))
          (return))))))

(fn SetMediaContentbyKey
  (params (MediaSource :type File%20Media%20Source%20Object%20Reference) (MediaPlayer :type Media%20Player%20Object%20Reference) (MediaTexture :type Media%20Texture%20Object%20Reference) (Key :type String))
  (bind _textsandmatsforkey (Variables|Default|GetTextsAndMatsForKey))
  (bind (_array_element _array_index) (Utilities|Array|ForEachLoopwithBreak _textsandmatsforkey :!label _label)
    (:LoopBody
      (if (Utilities|Enum|Equal(Enum) Key (.Key (Utilities|Struct|BreakSDisplayTexsAndMats _array_element)))
        (Utilities|Array|SetArrayElem _textsandmatsforkey _array_index (Utilities|Struct|MakeSDisplayTexsAndMats (.Key (Utilities|Struct|BreakSDisplayTexsAndMats _array_element)) (.Texs (Utilities|Struct|BreakSDisplayTexsAndMats _array_element)) (.Mats (Utilities|Struct|BreakSDisplayTexsAndMats _array_element)) "NewEnumerator1" MediaSource MediaPlayer MediaTexture))
        (goto _label Break)))))

(fn OnBoxOverlapBegin
  (params (OverlappedComponent :type Primitive%20Component%20Object%20Reference) (OtherActor :type Actor%20Object%20Reference) (OtherComp :type Primitive%20Component%20Object%20Reference) (OtherBodyIndex :type Integer) (bFromSweep :type Boolean) (SweepResult :type Hit%20Result%20Structure%20%28by%20ref%29))
  (bind _keymediaplayersmap (Variables|Default|GetKeyMediaPlayersMap))
  (Utilities|Casting|CastToGFirstPersonCharacter OtherActor)
  (Variables|/Game/GamePlay/GGameInstance.GGameInstance_C|SetInBox (CallFunction|GetGGameInstance) true)
  (Variables|Default|SetInBox true)
  (Audio|Components|Audio|Play (Variables|Default|GetRoboticArm) true)
  (if (Utilities|Array|IsEmpty (Variables|Default|GetOptionalDirs))
    (return)
    (else
      (CallFunction|ShowComboBox true)
      (bind _keys (Utilities|Map|Keys _keymediaplayersmap))
      (for _array_element _keys
        (Media|MediaPlayer|Play (.Value (Utilities|Map|Find _keymediaplayersmap _array_element)) :!class /Script/MediaAssets.MediaPlayer))
      (return))))

(fn OnBoxOverlapEnd
  (params (OverlappedComponent :type Primitive%20Component%20Object%20Reference) (OtherActor :type Actor%20Object%20Reference) (OtherComp :type Primitive%20Component%20Object%20Reference) (OtherBodyIndex :type Integer))
  (bind _roboticarm (Variables|Default|GetRoboticArm))
  (bind _keymediaplayersmap (Variables|Default|GetKeyMediaPlayersMap))
  (Utilities|Casting|CastToGFirstPersonCharacter OtherActor)
  (Variables|/Game/GamePlay/GGameInstance.GGameInstance_C|SetInBox (CallFunction|GetGGameInstance) false)
  (Variables|Default|SetInBox false)
  (Components|Animation|SetAnimation _roboticarm (.animtoplay (Variables|/Script/Engine.SkeletalMeshComponent|GetAnimationData _roboticarm)))
  (if (Utilities|Array|IsEmpty (Variables|Default|GetOptionalDirs))
    (return)
    (else
      (CallFunction|ShowComboBox false)
      (bind _keys (Utilities|Map|Keys _keymediaplayersmap))
      (for _array_element _keys
        (Sequencer|Player|Pause (.Value (Utilities|Map|Find _keymediaplayersmap _array_element)))
        (return)))))

(fn InitOptionalContent
  (params (AllowPauseVideo :type Boolean))
  (bind _mats (Variables|Default|GetMats))
  (CallFunction|ClearKeyMap)
  (Variables|Default|SetDisplayType "NewEnumerator2")
  (for _array_element (Variables|Default|GetKeys)
    (CallFunction|GenerateOptionalDir _array_element)
    (LocalVariables|SetCurerntKey _array_element)
    (Utilities|Array|Clear (Variables|Default|GetTexs))
    (Utilities|Array|Clear (Variables|Default|GetMats))
    (bind _returnvalue (Class|CommonFunLib|GetDirType (Variables|Default|GetOptionalDirs)))
    (bind _output_get (Variables|Default|SetDirTypeMap _returnvalue))
    (bind _keys (Utilities|Map|Keys _output_get))
    (LocalVariables|SetDir (Utilities|Array|Get(acopy) _keys (Variables|Default|GetOptionalIndex)))
    (Utilities|SwitchDirType (.Value (Utilities|Map|Find (Variables|Default|GetDirTypeMap) (Utilities|Array|Get(acopy) _keys (Variables|Default|GetOptionalIndex))))
      (:PPT
        (bind _returnvalue_2 (Class|CommonFunLib|GetAllSubdirectories (LocalVariables|GetDir)))
        (if (Utilities|Array|IsNotEmpty _returnvalue_2)
          (bind _texs (Class|CommonFunLib|LoadPNG2Texture (Utilities|Array|Get(acopy) _returnvalue_2)))
          (bind _output_get_2 (Variables|Default|SetTexs _texs))
          (Utilities|Map|Add (Variables|Default|GetKeyTexsMap) (LocalVariables|GetCurerntKey) (Utilities|Struct|MakeSKeyTex _output_get_2))
          (for _array_element_2 _output_get_2
            (bind _returnvalue_3 (Rendering|Material|CreateDynamicMaterialInstance "/Game/Blueprints/Screen/Materials/M_ScreenBase_SkeletalMat.M_ScreenBase_SkeletalMat" "None" "None" :!class /Script/Engine.KismetMaterialLibrary))
            (Rendering|Material|SetTextureParameterValue _returnvalue_3 "Texture" _array_element_2)
            (Utilities|Array|Add (Variables|Default|GetMats) _returnvalue_3))
          (Utilities|Map|Add (Variables|Default|GetKeyMatsMap) (LocalVariables|GetCurerntKey) (Utilities|Struct|MakeSKeyMat (Variables|Default|GetMats)))))
      (:Image
        (bind _texs_2 (Class|CommonFunLib|LoadPNG2Texture (LocalVariables|GetDir)))
        (bind _output_get_3 (Variables|Default|SetTexs _texs_2))
        (Utilities|Map|Add (Variables|Default|GetKeyTexsMap) (LocalVariables|GetCurerntKey) (Utilities|Struct|MakeSKeyTex _output_get_3))
        (for _array_element_3 _output_get_3
          (bind _returnvalue_4 (Rendering|Material|CreateDynamicMaterialInstance "/Game/Blueprints/Screen/Materials/M_ScreenBase_SkeletalMat.M_ScreenBase_SkeletalMat" "None" "None" :!class /Script/Engine.KismetMaterialLibrary))
          (Rendering|Material|SetTextureParameterValue _returnvalue_4 "Texture" _array_element_3)
          (Utilities|Array|Add (Variables|Default|GetMats) _returnvalue_4))
        (Utilities|Map|Add (Variables|Default|GetKeyMatsMap) (LocalVariables|GetCurerntKey) (Utilities|Struct|MakeSKeyMat (Variables|Default|GetMats))))
      (:Video
        (bind _returnvalue_5 (Class|CommonFunLib|GetFilesfromDir (LocalVariables|GetDir)))
        (if (Utilities|Array|IsNotEmpty _returnvalue_5)
          (bind _returnvalue_6 (Game|ConstructObjectfromClass "/Script/MediaAssets.FileMediaSource"))
          (Class|FileMediaSource|SetFilePath _returnvalue_6 (Utilities|Array|Get(acopy) _returnvalue_5))
          (Utilities|Map|Add (Variables|Default|GetKeyMediaSourcesMap) (LocalVariables|GetCurerntKey) _returnvalue_6)
          (bind _returnvalue_7 (Game|ConstructObjectfromClass "/Script/MediaAssets.MediaPlayer"))
          (Utilities|Map|Add (Variables|Default|GetKeyMediaPlayersMap) (LocalVariables|GetCurerntKey) _returnvalue_7)
          (bind _returnvalue_8 (Game|ConstructObjectfromClass "/Script/MediaAssets.MediaTexture"))
          (Media|MediaSoundComponent|SetMediaPlayer _returnvalue_8 _returnvalue_7)
          (Class|MediaTexture|UpdateResource _returnvalue_8)
          (Utilities|Map|Add (Variables|Default|GetKeyMediaTexturesMap) (LocalVariables|GetCurerntKey) _returnvalue_8)
          (bind _returnvalue_9 (Game|AddComponentbyClass "/Script/MediaAssets.MediaSoundComponent" false))
          (Utilities|Map|Add (Variables|Default|GetKeySoundCompsMap) (LocalVariables|GetCurerntKey) _returnvalue_9)
          (Transformation|AttachComponentToComponent _returnvalue_9 (Variables|Default|GetDefaultSceneRoot) "None" "KeepRelative" "KeepRelative" "KeepRelative" true)
          (Media|MediaSoundComponent|SetMediaPlayer _returnvalue_9 (.Value (Utilities|Map|Find (Variables|Default|GetKeyMediaPlayersMap) (LocalVariables|GetCurerntKey))))
          (Audio|Components|Audio|SetVolumeMultiplier _returnvalue_9 0.0 :!class /Script/AudioMixer.SynthComponent)
          (bind _returnvalue_10 (Rendering|Material|CreateDynamicMaterialInstance 0 "None" "None" :!class /Script/Engine.KismetMaterialLibrary))
          (Rendering|Material|SetTextureParameterValue _returnvalue_10 "Texture" (.Value (Utilities|Map|Find (Variables|Default|GetKeyMediaTexturesMap) (LocalVariables|GetCurerntKey))))
          (Utilities|Array|Add _mats _returnvalue_10)
          (Utilities|Map|Add (Variables|Default|GetKeyMatsMap) (LocalVariables|GetCurerntKey) (Utilities|Struct|MakeSKeyMat _mats))
          (Variables|Default|SetDisplayType "NewEnumerator1")
          (Utilities|IsValid (.Value (Utilities|Map|Find (Variables|Default|GetKeyMediaPlayersMap) (LocalVariables|GetCurerntKey)))
            (:Is%20Valid
              (Media|MediaPlayer|OpenSource (.Value (Utilities|Map|Find (Variables|Default|GetKeyMediaPlayersMap) (LocalVariables|GetCurerntKey))) (.Value (Utilities|Map|Find (Variables|Default|GetKeyMediaSourcesMap) (LocalVariables|GetCurerntKey))))
              (if (not (Variables|Default|GetInBox))
                (if AllowPauseVideo
                  (CallFunction|PauseMedia (LocalVariables|GetCurerntKey))))))))))
  (for _array_element_4 (Variables|Default|GetKeys)
    (Rendering|Material|SetMaterial (Variables|Default|GetRoboticArm) (.Value (Utilities|Map|Find (Variables|Default|GetKeyForMatIndex) _array_element_4)) (Utilities|Array|Get(acopy) (.mats (.Value (Utilities|Map|Find (Variables|Default|GetKeyMatsMap) _array_element_4))) (Variables|Default|GetPageIndex)))
    (Variables|Default|SetDisplayType "NewEnumerator0")))

(fn GenerateOptionalDir
  (params (Key :type String))
  (for _array_element (Variables|Default|GetOptionalDirs)
    (Utilities|Array|Add (LocalVariables|GetOptionalDirsSelf) (Utilities|String|Append (Class|KismetSystemLibrary|ConverttoAbsolutePath (Utilities|String|Append (Class|KismetSystemLibrary|GetProjectDirectory) "DiyContents")) "/" Key "/" (Utilities|Array|Get(acopy) (Utilities|String|ParseIntoArray _array_element "/") (Utilities|Array|LastIndex (Utilities|String|ParseIntoArray _array_element "/"))))))
  (Variables|Default|SetOptionalDirs (LocalVariables|GetOptionalDirsSelf)))

(fn ClearKeyMap
  (bind _keysoundcompsmap (Variables|Default|GetKeySoundCompsMap))
  (Utilities|Map|Clear (Variables|Default|GetCurrentKey))
  (Utilities|Map|Clear (Variables|Default|GetKeyMatsMap))
  (Utilities|Map|Clear (Variables|Default|GetKeyMediaSourcesMap))
  (Utilities|Map|Clear (Variables|Default|GetKeyMediaPlayersMap))
  (Utilities|Map|Clear (Variables|Default|GetKeyMediaTexturesMap))
  (Utilities|Map|Clear (Variables|Default|GetKeyTexsMap))
  (bind _keys (Utilities|Map|Keys _keysoundcompsmap))
  (for _array_element _keys
    (Components|DestroyComponent (.Value (Utilities|Map|Find _keysoundcompsmap _array_element))))
  (Utilities|Map|Clear (Variables|Default|GetKeySoundCompsMap)))

(fn UpdateOptionalContent
  (params (OptionalDir :type String))
  (bind _optionaldirs (Variables|Default|GetOptionalDirs))
  (bind _returnvalue (Utilities|Array|FindItem _optionaldirs OptionalDir))
  (Variables|Default|SetPageIndex 0)
  (if (>= _returnvalue 0)
    (Variables|Default|SetOptionalIndex _returnvalue)
    (CallFunction|ShowPage true)
    (switch Utilities|FlowControl|Switch|SwitchonESlateVisibility (Widget|GetVisibility (Variables|/Game/UI/UW_Main.UW_Main_C|GetUW_ContentShow (Variables|/Game/GamePlay/GHUD.GHUD_C|GetUW_Main (CallFunction|GetGHUD))))
      (:Visible
        (CallFunction|ShowContent)))))

(fn ShowContent
  (bind _ghud (CallFunction|GetGHUD))
  (bind _self self)
  (bind _mediaplayer (Variables|Default|GetMediaPlayer))
  (bind _uw_main (Variables|/Game/GamePlay/GHUD.GHUD_C|GetUW_Main _ghud))
  (Utilities|IsValid _uw_main
    (:Is%20Valid
      (Variables|/Game/UI/UW_Main.UW_Main_C|SetDisplayScreen _uw_main _self)
      (Default|UpdateContentRoboticArm (Variables|/Game/UI/UW_Main.UW_Main_C|GetUW_ContentShow _uw_main) (CallFunction|GenarateUIMatbyKey "3") (CallFunction|GenarateUIMatbyKey "4") (CallFunction|GenarateUIMatbyKey "5") _self "(X=976.000000,Y=1736.000000)" "(X=-1456.000000,Y=-816.000000)" "(X=976.000000,Y=1736.000000)" "(X=-480.000000,Y=-816.000000)" "(X=976.000000,Y=1736.000000)" "(X=496.000000,Y=-816.000000)")
      (Default|ShowMediaTable _uw_main true)
      (switch Utilities|FlowControl|Switch|SwitchonEDisplayType (Variables|Default|GetDisplayType)
        (:NewEnumerator0
          _)
        (:NewEnumerator1
          (Utilities|IsValid _mediaplayer
            (:Is%20Valid
              (Media|MediaPlayer|Play _mediaplayer :!class /Script/MediaAssets.MediaPlayer)))))
      (Variables|/Game/GamePlay/GHUD.GHUD_C|SetPlayType (CallFunction|GetGHUD) "NewEnumerator1"))))

(fn GenarateUIMatbyKey
  (params (Key :type String))
  (bind _keytexsmap (Variables|Default|GetKeyTexsMap))
  (bind (_value _returnvalue) (Utilities|Map|Find _keytexsmap Key))
  (if _returnvalue
    (bind _returnvalue_2 (Rendering|Material|CreateDynamicMaterialInstance "/Game/Blueprints/Screen/Materials/M_ScreenUIBase.M_ScreenUIBase" "None" "None" :!class /Script/Engine.KismetMaterialLibrary))
    (Rendering|Material|SetTextureParameterValue _returnvalue_2 "Texture" (Utilities|Array|Get(acopy) (.texs _value) (Variables|Default|GetPageIndex)))
    (return _returnvalue_2)))