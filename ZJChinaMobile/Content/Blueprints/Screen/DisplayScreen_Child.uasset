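; DisplayScreen_Child is a child screen actor that shows a local video file on its material when play begins.
; After the parent BeginPlay, it builds a file media source, media player and media texture at runtime instead of using media assets.
; The texture feeds a dynamic instance of M_MediaBase applied to the screen, then the player opens the source.
; The video path is a hard-coded absolute drive path.
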(event EventBeginPlay
  (|CallParentFunction)
  (bind _returnvalue (Game|ConstructObjectfromClass "/Script/MediaAssets.FileMediaSource"))
  (Variables|/Script/MediaAssets.FileMediaSource|SetFilePath _returnvalue "E:\\Goulandis\\ZJChinaMobile\\ZJChinaMobile\\DiyContents\\3\\Video1.mp4")
  (bind _returnvalue_2 (Game|ConstructObjectfromClass "/Script/MediaAssets.MediaPlayer"))
  (bind _returnvalue_3 (Game|ConstructObjectfromClass "/Script/MediaAssets.MediaTexture"))
  (Media|MediaSoundComponent|SetMediaPlayer _returnvalue_3 _returnvalue_2)
  (Class|MediaTexture|UpdateResource _returnvalue_3)
  (bind _returnvalue_4 (Rendering|Material|CreateDynamicMaterialInstance "/Game/Blueprints/Screen/Materials/M_MediaBase.M_MediaBase" "None" "None" :!class /Script/Engine.KismetMaterialLibrary))
  (Rendering|Material|SetTextureParameterValue _returnvalue_4 "MediaTexture" _returnvalue_3)
  (CallFunction|SetMaterial _returnvalue_4)
  (Media|MediaPlayer|OpenSource _returnvalue_2 _returnvalue))

(event Collision|EventActorBeginOverlap
  (params (OtherActor :type Actor%20Object%20Reference)))

(event EventTick
  (params (DeltaSeconds :type Float%20%28single-precision%29))
  (|CallParentFunction DeltaSeconds) ; 此节点被禁用，将不会被调用。\n从引脚连出引线来编译功能。
)

(fn ConstructionScript
  (|CallParentFunction))